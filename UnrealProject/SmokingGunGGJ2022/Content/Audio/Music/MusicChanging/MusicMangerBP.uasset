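; Music manager Blueprint that plays the game's music and switches tracks when ChangeMusicFromTo is called, per its comments from MusicChangingVolBP.
; On BeginPlay it creates and starts every TrackList sound muted, stores the references, then fades in the first.
; Switching uses a timeline to set crossfade volumes scaled by MusicVolume, so tracks change without restarting.
; CurrentPlayTrack becomes the new song on the fade's first update, not at its end.
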(event `self.ReceiveBeginPlay`
  ;[1 1 1 1 12] Creates all the music tracks from an array, sets their volume to 0, and plays them.
  (for _array_element (`self.TrackList`)
    (bind _returnvalue (`GameplayStatics.CreateSound2D` _array_element 1.0 1.0 0.0 null))
    (`KismetArrayLibrary.Array_Add` (`self.MusicReferences`) _returnvalue)
    (`AudioComponent.SetVolumeMultiplier` _returnvalue 0.0)
    (`AudioComponent.Play` _returnvalue 0.0)
    (set `self.CurrentPlayTrack` 0))
  ;[1 1 1 1 12] After all the music tracks are created, this sections fades in the first one on index 0.
  (bind (_direction _volumecontrolup) (`Timeline|MusicFadeInStart` :!via `PlayFromStart`)
    (:`Update`
      (`AudioComponent.SetVolumeMultiplier` (`|GetArrayItem` (`self.MusicReferences`)) (* (`self.MusicVolume`) _volumecontrolup)))))

(event `Change Music From To`
  (params (SongToPlay :type Integer))
  (bind _musicvolume (`self.MusicVolume`))
  (bind _musicreferences (`self.MusicReferences`))
  ;[1 1 1 1 12] This section crossfades between music tracks. The track to turn on and the track to turn off are determined by the MusicChangingVolBP. The overall music volume is adjustable with the MusicVolume float which is public.
  (bind (_direction _volumecontrolup _volumecontroldown) (`Timeline|MusicSelectorFade` :!via `PlayFromStart`)
    (:`Update`
      (`AudioComponent.SetVolumeMultiplier` (`|GetArrayItem` _musicreferences (`self.CurrentPlayTrack`)) (* _musicvolume _volumecontroldown))
      (`AudioComponent.SetVolumeMultiplier` (`|GetArrayItem` _musicreferences SongToPlay) (* _musicvolume _volumecontrolup))
      (set `self.CurrentPlayTrack` SongToPlay))))

(fn `UserConstructionScript`)