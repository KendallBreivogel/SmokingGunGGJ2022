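; Trigger volume Blueprint that changes the level's music when the player pawn overlaps its box.
; On BeginPlay it caches the first MusicMangerBP found in the level, assuming only one exists.
; Each player overlap flips a flag and calls ChangeMusicFromTo on the manager, alternating between the first-overlap and second-overlap tracks so that re-entering restores the original music.
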(event `self.ReceiveBeginPlay`
  ;[1 1 1 1 12] Gets and stores a reference to the MusicMangerBP. There should only be 1 MusicMangerBP per level so it will be index 0.
  (bind _outactors (`GameplayStatics.GetAllActorsOfClass` "/Game/Audio/Music/MusicChanging/MusicMangerBP.MusicMangerBP_C"))
  (set `self.MusicMangerRef` (`|GetArrayItem` _outactors)))

(event `self.Box.OnComponentBeginOverlap`
  (params (OverlappedComponent :type "PrimitiveComponent Object Reference") (OtherActor :type "Actor Object Reference") (OtherComp :type "PrimitiveComponent Object Reference") (OtherBodyIndex :type Integer) (bFromSweep :type Boolean) (SweepResult :type "HitResult Structure (by ref)"))
  (bind _musicmangerref (`self.MusicMangerRef`))
  ;[1 1 1 1 12] Detect when the player pawn overlaps with the trigger box
  (if (== OtherActor (`GameplayStatics.GetPlayerPawn` 0))
    ;[1 1 1 1 12] Sends a message to the MusicMangerBP saying which track to turn on and which track to turn off. Reverses the tracks to play and stop after a player overlaps with the trigger box so that the music goes back to its original state when the player overlaps with the box again.
    (if (`self.MusicAlreadyChanged`)
      (`/Game/Audio/Music/MusicChanging/MusicMangerBP.Change Music From To` _musicmangerref (`self.MusicToPlayOn2ndOverlap`))
      (else
        (`/Game/Audio/Music/MusicChanging/MusicMangerBP.Change Music From To` _musicmangerref (`self.MusicToPlayOnOverlap`))))
    (set `self.MusicAlreadyChanged` (not (`self.MusicAlreadyChanged`)))))

(fn `UserConstructionScript`)