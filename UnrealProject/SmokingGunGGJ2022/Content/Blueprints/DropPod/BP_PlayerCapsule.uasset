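; Player drop pod that plays an arrival sequence on BeginPlay when UseDropPod is set, otherwise hides itself.
; A temporary pawn attached to the capsule takes possession while alarms, camera shake and timeline-driven flashing light and red tint play.
; The Drop timeline moves the capsule, fades audio and animates the black sphere's opacity.
; On landing it explodes, blows off the physics door and hands control to FirstPersonCharacter.
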(event `self.ReceiveBeginPlay`
  (`self.DropPlayer`))

(event `DropPlayer`
  (bind _returnvalue (`self.K2_GetActorLocation`))
  (bind _returnvalue_2 (`GameplayStatics.GetPlayerController` 0))
  (bind _actualpawn (`self.ActualPawn`))
  (bind _door (`self.Door`))
  (if (`self.UseDropPod`)
    (`|ExecutionSequence`
      (:`then_0`
        ;[1 1 1] Fade in Alarms + drop sound
        (`AudioComponent.FadeIn` (`self.WAV_DropPod`) 5.0 1.0 0.0 "Linear")
        (`AudioComponent.FadeIn` (`self.WAV_Alarm`) 5.0 1.0 0.0 "Linear"))
      (:`then_1`
        ;[1 1 1] Begin flashing lights + animating scene tint
        (bind _returnvalue_3 (`KismetMaterialLibrary.CreateDynamicMaterialInstance` "/Game/Blueprints/DropPod/Assets/M_FlashingLight_Master.M_FlashingLight_Master"))
        (bind _output_get (set `self.LightMat` _returnvalue_3))
        (`PrimitiveComponent.SetMaterial` (`self.SM_Capsule`) 4 _output_get)
        (bind _returnvalue_4 (`KismetMaterialLibrary.CreateDynamicMaterialInstance` "/Game/Blueprints/DropPod/Assets/M_TotalBlack.M_TotalBlack"))
        (bind _output_get_2 (set `self.BlackMat` _returnvalue_4))
        (`PrimitiveComponent.SetMaterial` (`self.SM_InvertedSphere`) 0 _output_get_2)
        (`TimelineComponent.SetPlayRate` (`self.LightFlash`) 1.0)
        (`|ExecutionSequence`
          (:`then_0`
            (bind (_direction _intensity) (`Timeline|LightFlash`)
              (:`Update`
                (`LightComponent.SetIntensity` (`self.PointLight`) (* _intensity 5000.0))
                (`MaterialInstanceDynamic.SetScalarParameterValue` (`self.LightMat`) "Intensity" _intensity))))
          (:`then_1`
            (bind (_direction_2 _intensity_2) (`Timeline|SceneTint` :!label _label)
              (:`Update`
                (set `PostProcessVolume.Settings` (make `PostProcessSettings` :`SceneColorTint` (make `LinearColor` (* (+ _intensity_2 0.25) 15.0) 1.0 1.0 1.0)) (`self.PP`)))))))
      (:`then_2`
        ;[1 1 1] Attatch the player to the Drop Pod, then begin the camera shake animation
        (bind _returnvalue_5 (`|SpawnActorFromClass` "/Game/Blueprints/DropPod/BP_StartingPawn.BP_StartingPawn_C" (`KismetMathLibrary.MakeTransform` (`self.K2_GetActorLocation`) (struct :`Yaw` 180.0)) "Undefined" "OverrideRootScale" null null))
        (`Controller.Possess` _returnvalue_2 _returnvalue_5)
        (set `self.TempPawn` _returnvalue_5)
        (`self.K2_AttachToComponent` _returnvalue_5 (`self.SM_Capsule`) "None" "KeepWorld" "KeepWorld" "KeepWorld" true)
        (`PlayerController.ClientStartCameraShake` :`self` _returnvalue_2 :`Shake` "/Game/UI/DropShake.DropShake_C")
        (bind _outactors (`GameplayStatics.GetAllActorsOfClass` "/Game/ExtraContent/FirstPersonBP/Blueprints/FirstPersonCharacter.FirstPersonCharacter_C"))
        (set `self.ActualPawn` (`|GetArrayItem` _outactors)))
      (:`then_3`
        ;[1 1 1] Begin dropping the pod from a height = fallHeight. Begin fading out spacesphere
        (bind (_direction_3 _drop _sphereopacity) (`Timeline|Drop`)
          (:`Update`
            (`SceneComponent.K2_SetRelativeLocation` (`self.SM_Capsule`) (`KismetMathLibrary.MakeVector` 0.0 0.0 (* _drop (`self.FallHeight`))) false false)
            (`MaterialInstanceDynamic.SetScalarParameterValue` (`self.BlackMat`) "Opacity" _sphereopacity)
            (`AudioComponent.SetVolumeMultiplier` (`self.WAV_DropPod`) (- 1.0 _drop))
            (`AudioComponent.SetVolumeMultiplier` (`self.WAV_Alarm`) (- 1.0 _drop)))
          (:`Finished`
            (`GameplayStatics.SpawnEmitterAtLocation` "/Game/Blueprints/DropPod/Assets/P_Explosion.P_Explosion" _returnvalue (struct) (12.0 12.0 12.0))
            (`|ExecutionSequence`
              (:`then_0`
                (goto _label :!via `Stop`))
              (:`then_1`
                (`AudioComponent.Stop` (`self.WAV_DropPod`))
                (`AudioComponent.FadeOut` (`self.WAV_Alarm`) 0.2 0.0 "Linear")
                (`GameplayStatics.PlaySoundAtLocation` "/Game/Audio/Explosion02.Explosion02" _returnvalue (struct) 1.5 0.8 0.0 null null null)
                (set `PostProcessVolume.bEnabled` false (`self.PP`))
                (`ActorComponent.SetActive` (`self.P_Fire_Capsule`) false false)
                (`KismetSystemLibrary.Delay` 2.0)
                (`PrimitiveComponent.SetSimulatePhysics` _door true)
                (`PrimitiveComponent.AddForce` _door (* (`SceneComponent.GetRightVector` _door) 3000000.0) "None" false)
                (`GameplayStatics.PlaySoundAtLocation` "/Game/Audio/WAV_Metal_Hit.WAV_Metal_Hit" (`self.K2_GetActorLocation`) (struct) 1.0 0.5 0.0 null null null)
                (`self.K2_SetActorTransform` _actualpawn (`self.GetTransform` (`GameplayStatics.GetPlayerPawn` 0)) false false)
                (`Controller.Possess` (`GameplayStatics.GetPlayerController` 0) _actualpawn)
                (`|ExecutionSequence`
                  (:`then_0`
                    (`KismetSystemLibrary.Delay` 9.0)
                    (`PrimitiveComponent.SetSimulatePhysics` (`self.Door`) false))
                  (:`then_1`
                    (`KismetSystemLibrary.Delay` 2.0)
                    (`self.K2_DestroyActor` (`self.TempPawn`))
                    (`KismetSystemLibrary.Delay` 3.0)))))))))
    (else
      (`self.SetActorHiddenInGame` true))))

(event `self.Door.OnComponentHit`
  (params (HitComponent :type "PrimitiveComponent Object Reference") (OtherActor :type "Actor Object Reference") (OtherComp :type "PrimitiveComponent Object Reference") (NormalImpulse :type "Vector Structure") (Hit :type "HitResult Structure (by ref)"))
  (if (> (`KismetMathLibrary.VSize` NormalImpulse) 30000.0)
    (`GameplayStatics.PlaySoundAtLocation` "/Game/Audio/WAV_Metal_Hit.WAV_Metal_Hit" (`SceneComponent.K2_GetComponentLocation` (`self.Door`)) (struct) 0.7 1.0 0.0 "/Game/Audio/BasicAtt.BasicAtt" null null)))

(fn `UserConstructionScript`)