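; BP_ChickenMonster is a chicken monster enemy, derived from a parent monster class, with a pounce attack and a light-triggered enrage.
; Pounce halts AI movement and briefly enables two sphere hitboxes that damage overlapped actors.
; When detected light exceeds a threshold, a one-time enrage timeline shifts emissive material from blue to orange and raises idle speed.
; Both actions set a Blackboard interrupt flag while they play.
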(event `self.ReceiveBeginPlay`
  (`parent.ReceiveBeginPlay`)
  (`self.WakeUp`))

(event `self.ReceiveTick`
  (params (DeltaSeconds :type "Float (single-precision)"))
  (`parent.ReceiveTick` DeltaSeconds))

(event `self.DeathEffects`
  (`parent.DeathEffects`))

(event `self.DeathCleanup`
  (`self.K2_DestroyActor`))

(event `Enrage`
  (bind _returnvalue (`AIBlueprintHelperLibrary.GetBlackboard` (`AIBlueprintHelperLibrary.GetAIController` self)))
  (if (not (`self.Enraged`))
    (set `self.PlayingEnrageAnim` true)
    (`BlackboardComponent.SetValueAsBool` _returnvalue "AnimationInterrupt" true)
    (set `self.Enraged` true)
    (bind (_direction _bloodalpha) (`Timeline|ChangeBloodColor` :!via `PlayFromStart`)
      (:`Update`
        (for _array_element (`self.Material`)
          (`MaterialInstanceDynamic.SetVectorParameterValue` _array_element "EmissiveColor" (`KismetMathLibrary.LinearColorLerp` (struct :`G` 0.715694 :`B` 1.0 :`A` 1.0) (struct :`R` 1.0 :`G` 0.404153 :`A` 1.0) _bloodalpha))
          (`MaterialInstanceDynamic.SetScalarParameterValue` _array_element "Brightness" (`KismetMathLibrary.Lerp` 0.01 0.05 _bloodalpha))
          (set `self.IdleSpeed` (`KismetMathLibrary.Lerp` 100.0 800.0 _bloodalpha))))
      (:`Finished`
        (`BlackboardComponent.SetValueAsBool` _returnvalue "AnimationInterrupt" false)
        (set `self.PlayingEnrageAnim` false)))))

(event `self.WakeUp`
  (`parent.WakeUp`)
  (set `CharacterMovementComponent.GravityScale` 1.0 (`self.CharacterMovement`)))

(event `self.Pounce`
  (params (Location :type "Vector Structure"))
  (bind _returnvalue (`AIBlueprintHelperLibrary.GetAIController` self))
  (bind _returnvalue_2 (`AIBlueprintHelperLibrary.GetBlackboard` (`AIBlueprintHelperLibrary.GetAIController` self)))
  (`PrimitiveComponent.SetCollisionEnabled` (`self.Sphere`) "QueryOnly")
  (`PrimitiveComponent.SetCollisionEnabled` (`self.Sphere1`) "QueryOnly")
  (set `self.State` "NewEnumerator4")
  (set `self.canPounce` false)
  (`Controller.StopMovement` _returnvalue)
  (`BlackboardComponent.SetValueAsBool` (`AIBlueprintHelperLibrary.GetBlackboard` _returnvalue) "AnimationInterrupt" true)
  (`KismetSystemLibrary.Delay` 1.05)
  (set `self.State` "NewEnumerator1")
  (set `self.canPounce` true)
  (`BlackboardComponent.SetValueAsBool` _returnvalue_2 "Pouncing" false)
  (`PrimitiveComponent.SetCollisionEnabled` (`self.Sphere`) "NoCollision")
  (`PrimitiveComponent.SetCollisionEnabled` (`self.Sphere1`) "NoCollision")
  (`BlackboardComponent.SetValueAsBool` _returnvalue_2 "AnimationInterrupt" false))

(event `self.ResetCanPounce`
  (`parent.ResetCanPounce`))

(event `self.Sphere.OnComponentBeginOverlap`
  (params (OverlappedComponent :type "PrimitiveComponent Object Reference") (OtherActor :type "Actor Object Reference") (OtherComp :type "PrimitiveComponent Object Reference") (OtherBodyIndex :type Integer) (bFromSweep :type Boolean) (SweepResult :type "HitResult Structure (by ref)"))
  (`self.DamageActor` OtherActor))

(event `self.Sphere1.OnComponentBeginOverlap`
  (params (OverlappedComponent :type "PrimitiveComponent Object Reference") (OtherActor :type "Actor Object Reference") (OtherComp :type "PrimitiveComponent Object Reference") (OtherBodyIndex :type Integer) (bFromSweep :type Boolean) (SweepResult :type "HitResult Structure (by ref)"))
  (`self.DamageActor` OtherActor))

(fn `UpdateLighting`
  (`parent.UpdateLighting`)
  (if (> (`/Game/Blueprints/LightDetection/SceneComp_LightDetector.LightLevel` (`self.SceneComp_LightDetector`)) (`self.LightEffectTriggerValue`))
    (`self.Enrage`)))

(fn `UpdateSpeed`
  (params (NewSpeed :type "Float (double-precision)"))
  (bind _returnvalue_x (`KismetMathLibrary.BreakVector` (`self.GetActorScale3D`)))
  (`parent.UpdateSpeed` NewSpeed)
  (set `self.WalkAnimSpeed` (/ (/ NewSpeed 78.0) _returnvalue_x)))

(fn `UserConstructionScript`
  (bind _returnvalue (`KismetMaterialLibrary.CreateDynamicMaterialInstance` "/Game/Blueprints/Monsters/ChickenMonster/Mesh/MI_ChickenMonster.MI_ChickenMonster"))
  (`KismetArrayLibrary.Array_Add` (`self.Material`) _returnvalue)
  (`PrimitiveComponent.SetMaterial` (`self.Mesh`) 0 _returnvalue))