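; Test monster that shows its light-related state through text displays for inspecting illumination and weakness.
; On BeginPlay it labels itself as light or dark sensitive based on IsLightSensitive.
; Every tick, after the parent's tick, it writes the illumination probe reading and the current WeaknessScalar to their text displays.
; It only displays these values and does not calculate them in this Blueprint.
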(event `self.ReceiveBeginPlay`
  (`parent.ReceiveBeginPlay`)
  (`self.SetLightSensitivityText`))

(event `self.ReceiveTick`
  (params (DeltaSeconds :type "Float (single-precision)"))
  (`parent.ReceiveTick` DeltaSeconds)
  (`self.SetIlluminationText`)
  (`self.SetWeaknessScalarText`))

(fn `SetIlluminationText`
  (`TextRenderComponent.K2_SetText` (`self.LitCoefficient`) (`KismetTextLibrary.Conv_DoubleToText` (`/Game/IlluminationDetection/Blueprints/IlluminationComponents/BP_IlluminationProbe.ProbeIllumination` (`self.BP_IlluminationProbe`)) "HalfToEven")))

(fn `SetLightSensitivityText`
  (if (`self.bIsLightSensitive`)
    (`TextRenderComponent.K2_SetText` (`self.LightSensitivity`) "Light Sensitivity")
    (else
      (`TextRenderComponent.K2_SetText` (`self.LightSensitivity`) "Dark Sensitivity"))))

(fn `SetWeaknessScalarText`
  (`TextRenderComponent.K2_SetText` (`self.WeaknessScalarText`) (`KismetTextLibrary.Conv_DoubleToText` (`self.WeaknessScalar`) "HalfToEven")))

(fn `UserConstructionScript`)