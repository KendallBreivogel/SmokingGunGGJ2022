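; BP_Wurm is a giant worm monster that travels along a spline, carving a tunnel through voxel terrain.
; BeginPath runs a timeline over Time, bending Front and Back spline meshes along the path while a sphere and tunneling sound follow the head.
; The head removes voxels from a lazily found overlapping world and triggers rock debris bursts with sound at EmitRockDistances fractions.
; The construction script previews those burst points with debug spheres.
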(event `BeginPath`
  (bind _spline (`self.Spline`))
  (bind _wurmlength (`self.WurmLength`))
  (bind _voxelworld (`self.VoxelWorld`))
  (bind _returnvalue (`SplineComponent.GetSplineLength` _spline))
  (`AudioComponent.FadeIn` (`self.WAV_WurmTunneling`) 1.0 1.0 0.0 "Linear")
  (`TimelineComponent.SetPlayRate` (`self.MoveAlongSpline`) (/ 1.0 (`self.Time`)))
  (bind (_direction _dist) (`Timeline|MoveAlongSpline` :!via `PlayFromStart`)
    (:`Update`
      (bind _returnvalue_2 (`KismetMathLibrary.FClamp` _dist))
      (bind _returnvalue_3 (* _returnvalue _returnvalue_2))
      (bind _returnvalue_4 (`KismetMathLibrary.FClamp` (- _returnvalue_3 _wurmlength) 0.0 _returnvalue))
      (bind _returnvalue_5 (`KismetMathLibrary.FClamp` (- _returnvalue_3 (/ _wurmlength 2.0)) 0.0 _returnvalue))
      (`SplineMeshComponent.SetStartAndEnd` (`self.Back`) (`SplineComponent.GetLocationAtDistanceAlongSpline` _spline _returnvalue_4 "Local") (`SplineComponent.GetTangentAtDistanceAlongSpline` _spline _returnvalue_4 "Local") (`SplineComponent.GetLocationAtDistanceAlongSpline` _spline _returnvalue_5 "Local") (`SplineComponent.GetTangentAtDistanceAlongSpline` _spline _returnvalue_5 "Local") true)
      (bind _returnvalue_6 (+ _returnvalue_5 (`self.Offset`)))
      (bind _returnvalue_7 (`SplineComponent.GetLocationAtDistanceAlongSpline` _spline _returnvalue_3 "Local"))
      (`SplineMeshComponent.SetStartAndEnd` (`self.Front`) (`SplineComponent.GetLocationAtDistanceAlongSpline` _spline _returnvalue_6 "Local") (`SplineComponent.GetTangentAtDistanceAlongSpline` _spline _returnvalue_6 "Local") _returnvalue_7 (`SplineComponent.GetTangentAtDistanceAlongSpline` _spline _returnvalue_3 "Local") true)
      (bind _returnvalue_8 (`KismetMathLibrary.TransformLocation` (`self.GetTransform`) _returnvalue_7))
      (`SceneComponent.K2_SetWorldLocation` (`self.Sphere`) _returnvalue_8 false false)
      (`SceneComponent.K2_SetWorldLocation` (`self.WAV_WurmTunneling`) _returnvalue_8 false false)
      (`|ExecutionSequence`
        (:`then_0`
          (if (> (`KismetArrayLibrary.Array_Length` (`self.EmitRockDistances`)) (`self.CurrentEmitInt`))
            (if (> _returnvalue_2 (`|GetArrayItem` (`self.EmitRockDistances`) (`self.CurrentEmitInt`)))
              (`/Engine/EditorBlueprintResources/StandardMacros.IncrementInt` (`self.CurrentEmitInt`)
                (:`  `
                  (`GameplayStatics.SpawnEmitterAtLocation` "/Game/Blueprints/Monsters/Wurm/Assets/PS_RockDebris.PS_RockDebris" _returnvalue_8)
                  (`GameplayStatics.PlaySoundAtLocation` "/Game/Audio/Monsters/Wurm/WAV_WurmBurst.WAV_WurmBurst" _returnvalue_8 (struct) 1.0 1.0 0.0 "/Game/Audio/BasicAtt.BasicAtt" null null))))))
        (:`then_1`
          (if (`KismetSystemLibrary.IsValid` _voxelworld)
            (if (`VoxelWorld.IsCreated` _voxelworld)
              (`VoxelSphereTools.RemoveSphere` _voxelworld _returnvalue_8 (`self.DestroyRadius`)))
            (else
              (bind _returnvalue_9 (`VoxelBlueprintLibrary.GetAllVoxelWorldsOverlappingActor` null))
              (bind _output (`|GetArrayItem` _returnvalue_9))
              (if (`KismetSystemLibrary.IsValid` _output)
                (set `self.VoxelWorld` _output)))))))
    (:`Finished`
      (`AudioComponent.FadeOut` (`self.WAV_WurmTunneling`) 5.0 0.0 "Linear"))))

(fn `UserConstructionScript`
  (bind _spline (`self.Spline`))
  (for _array_element (`self.EmitRockDistances`)
    (`KismetSystemLibrary.DrawDebugSphere` (`SplineComponent.GetLocationAtDistanceAlongSpline` _spline (* _array_element (`SplineComponent.GetSplineLength` _spline)) "World") 500.0 4 (struct :`R` 1.0 :`G` 1.0 :`B` 1.0 :`A` 1.0) 1.0)))