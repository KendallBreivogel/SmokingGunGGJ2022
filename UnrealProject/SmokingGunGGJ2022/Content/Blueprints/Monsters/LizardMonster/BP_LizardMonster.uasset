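; Lizard monster enemy that reacts to light, extending a parent class that supplies pouncing, death effects and state.
; Any light wakes it from one state, then after a delay it restores gravity and a timeline levels its pitch and roll.
; Otherwise, outside one excluded state, light above a threshold sets the blackboard flee flag and disables its damage sphere.
; It also creates dynamic body and eye materials and scales walk animation to speed and actor size.
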(event `self.ReceiveBeginPlay`
  (`parent.ReceiveBeginPlay`))

(event `self.ReceiveTick`
  (params (DeltaSeconds :type "Float (single-precision)"))
  (`parent.ReceiveTick` DeltaSeconds))

(event `self.DeathEffects`
  (`parent.DeathEffects`))

(event `self.DeathCleanup`
  (`self.K2_DestroyActor`))

(event `self.Pounce`
  (params (Location :type "Vector Structure"))
  (`parent.Pounce` Location))

(event `self.WakeUp`
  (bind (_returnvalue_roll _returnvalue_pitch _returnvalue_yaw) (`KismetMathLibrary.BreakRotator` (`self.K2_GetActorRotation`)))
  (`parent.WakeUp`)
  (`KismetSystemLibrary.Delay` 2.0)
  (set `CharacterMovementComponent.GravityScale` 1.0 (`self.CharacterMovement`))
  (bind (_direction _alpha) (`Timeline|CorrectRotation` :!via `PlayFromStart`)
    (:`Update`
      (`self.K2_SetActorRotation` (`KismetMathLibrary.MakeRotator` (`KismetMathLibrary.Lerp` _returnvalue_roll 0.0 _alpha) (`KismetMathLibrary.Lerp` _returnvalue_pitch 0.0 _alpha) _returnvalue_yaw)))))

(event `self.Sphere.OnComponentBeginOverlap`
  (params (OverlappedComponent :type "PrimitiveComponent Object Reference") (OtherActor :type "Actor Object Reference") (OtherComp :type "PrimitiveComponent Object Reference") (OtherBodyIndex :type Integer) (bFromSweep :type Boolean) (SweepResult :type "HitResult Structure (by ref)"))
  (`self.DamageActor` OtherActor))

(fn `UpdateLighting`
  (bind _state (`self.State`))
  (bind _lightlevel (`/Game/Blueprints/LightDetection/SceneComp_LightDetector.LightLevel` (`self.SceneComp_LightDetector`)))
  (bind _returnvalue (> _lightlevel (`self.LightEffectTriggerValue`)))
  (`parent.UpdateLighting`)
  (if (and (> _lightlevel 0.0) (`|EnumEquality` _state "NewEnumerator5"))
    (`self.WakeUp`)
    (elif (not (`|EnumEquality` _state "NewEnumerator6"))
      (`BlackboardComponent.SetValueAsBool` (`AIBlueprintHelperLibrary.GetBlackboard` (`AIBlueprintHelperLibrary.GetAIController` self)) "IsFleeing" _returnvalue)
      (`PrimitiveComponent.SetCollisionEnabled` (`self.Sphere`) (select `bool` _returnvalue :`false` "QueryOnly" :`true` "NoCollision" :!type "ECollisionEnabled Enum")))))

(fn `UpdateSpeed`
  (params (NewSpeed :type "Float (double-precision)"))
  (bind _returnvalue_x (`KismetMathLibrary.BreakVector` (`self.GetActorScale3D`)))
  (`parent.UpdateSpeed` NewSpeed)
  (set `self.WalkAnimSpeed` (/ (/ NewSpeed 78.0) _returnvalue_x)))

(fn `UserConstructionScript`
  (bind _returnvalue (`KismetMaterialLibrary.CreateDynamicMaterialInstance` "/Game/Blueprints/Monsters/LizardMonster/Mesh/MI_lizardMonster.MI_LizardMonster"))
  (`KismetArrayLibrary.Array_Add` (`self.Material`) _returnvalue)
  (`PrimitiveComponent.SetMaterial` (`self.Mesh`) 1 _returnvalue)
  (bind _returnvalue_2 (`KismetMaterialLibrary.CreateDynamicMaterialInstance` "/Game/Blueprints/Monsters/LizardMonster/Mesh/M_Eyes.M_Eyes"))
  (`KismetArrayLibrary.Array_Add` (`self.Material`) _returnvalue_2)
  (`PrimitiveComponent.SetMaterial` (`self.Mesh`) 0 _returnvalue_2))