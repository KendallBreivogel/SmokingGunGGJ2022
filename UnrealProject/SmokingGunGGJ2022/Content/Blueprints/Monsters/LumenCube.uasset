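; LumenCube is a monster Blueprint that derives a weakness value from how lit it is and displays it as text.
; Each tick it reads ProbeIllumination from BPIlluminationProbe and sets WeaknessScalar to that value if light sensitive, or one minus it if dark sensitive.
; Text elements show the sensitivity type, set on BeginPlay, plus the live illumination and weakness values, refreshed every tick.
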(event `self.ReceiveBeginPlay`
  (`parent.ReceiveBeginPlay`)
  (`self.SetLightSensitivityText`))

(event `self.ReceiveTick`
  (params (DeltaSeconds :type "Float (single-precision)"))
  (`self.SetWeaknessScalar`)
  (`self.SetIlluminationText`)
  (`self.SetWeaknessScalarText`))

(fn `SetIlluminationText`
  (`TextRenderComponent.K2_SetText` (`self.LitCoefficient`) (`KismetTextLibrary.Conv_DoubleToText` (`/Game/IlluminationDetection/Blueprints/IlluminationComponents/BP_IlluminationProbe.ProbeIllumination` (`self.BP_IlluminationProbe`)) "HalfToEven")))

(fn `SetLightSensitivityText`
  (if (`self.bIsLightSensitive`)
    (`TextRenderComponent.K2_SetText` (`self.LightSensitivity`) "Light Sensitivity")
    (else
      (`TextRenderComponent.K2_SetText` (`self.LightSensitivity`) "Dark Sensitivity"))))

(fn `SetWeaknessScalar`
  (bind _bp_illuminationprobe (`self.BP_IlluminationProbe`))
  (if (`self.bIsLightSensitive`)
    (set `self.WeaknessScalar` (`/Game/IlluminationDetection/Blueprints/IlluminationComponents/BP_IlluminationProbe.ProbeIllumination` _bp_illuminationprobe))
    (else
      (set `self.WeaknessScalar` (- 1.0 (`/Game/IlluminationDetection/Blueprints/IlluminationComponents/BP_IlluminationProbe.ProbeIllumination` _bp_illuminationprobe))))))

(fn `SetWeaknessScalarText`
  (`TextRenderComponent.K2_SetText` (`self.WeaknessScalarText`) (`KismetTextLibrary.Conv_DoubleToText` (`self.WeaknessScalar`) "HalfToEven")))

(fn `UserConstructionScript`)