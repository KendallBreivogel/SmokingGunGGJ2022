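; Monster actor that takes damage from first-person projectile hits and destroys itself when Health runs out, printing debug messages along the way.
; Each tick it derives WeaknessScalar from an illumination probe component, using the light level directly if light-sensitive, otherwise its inverse.
; The scalar does not affect damage here, and the probe's update event only reaches an empty UpdateLighting stub.
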(event `self.ReceiveBeginPlay`
  (add `/Game/IlluminationDetection/Blueprints/IlluminationComponents/BP_IlluminationProbe.ProbeIlluminationUpdated` (`self.BP_IlluminationProbe`) (delegate `LightingChanged`)))

(event `LightingChanged`
  (`self.UpdateLighting`))

(event `self.ReceiveTick`
  (params (DeltaSeconds :type "Float (single-precision)"))
  (`self.SetWeaknessScalar`))

(event `self.ReceiveAnyDamage`
  (params (Damage :type "Float (single-precision)") (DamageType :type "DamageType Object Reference") (InstigatedBy :type "Controller Object Reference") (DamageCauser :type "Actor Object Reference"))
  (`KismetSystemLibrary.PrintString` (`KismetStringLibrary.Concat_StrStr` (`KismetSystemLibrary.GetDisplayName` self) ": Was Damaged"))
  (bind _output_get (set `self.Health` (- (`self.Health`) Damage)))
  (`KismetSystemLibrary.PrintString` (`KismetStringLibrary.Concat_StrStr` "Health: " (`KismetStringLibrary.Conv_DoubleToString` _output_get)))
  (if (<= (`self.Health`) 0.0)
    (`self.PlayerDied`)))

(event `self.ReceiveHit`
  (params (MyComp :type "PrimitiveComponent Object Reference") (Other :type "Actor Object Reference") (OtherComp :type "PrimitiveComponent Object Reference") (bSelfMoved :type Boolean) (HitLocation :type "Vector Structure") (HitNormal :type "Vector Structure") (NormalImpulse :type "Vector Structure") (Hit :type "HitResult Structure (by ref)"))
  (if (== (`GameplayStatics.GetObjectClass` Other) "/Game/ExtraContent/FirstPersonBP/Blueprints/FirstPersonProjectile.FirstPersonProjectile_C")
    (`GameplayStatics.ApplyDamage` self 10.0 null Other)))

(event `self.ReceiveDestroyed`
  (`KismetSystemLibrary.PrintString` "Destroyed"))

(fn `PlayerDied`
  (`self.K2_DestroyActor`))

(fn `PlayerRecievesDamage`)

(fn `SetWeaknessScalar`
  (if (`self.bIsLightSensitive`)
    (set `self.WeaknessScalar` (`/Game/IlluminationDetection/Blueprints/IlluminationComponents/BP_IlluminationProbe.ProbeIllumination` (`self.BP_IlluminationProbe`)))
    (else
      (set `self.WeaknessScalar` (- 1.0 (`/Game/IlluminationDetection/Blueprints/IlluminationComponents/BP_IlluminationProbe.ProbeIllumination` (`self.BP_IlluminationProbe`)))))))

(fn `UpdateLighting`)

(fn `UserConstructionScript`)