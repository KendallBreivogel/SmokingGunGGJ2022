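; Spawner actor that generates light detection volumes for the point and spot lights in the level.
; GenerateOverlaps gathers both light types, skipping any with attached actors or the ExcludeFromCalculations tag, and passes each to CreateVolume.
; CreateVolume spawns a BP_LightVolume_Sphere sized to the light's attenuation radius and attaches it, using spheres even for spot lights.
; The Volumes array is cleared, but the loop that would refill it is unconnected.
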(event `GenerateOverlaps`
  (`KismetArrayLibrary.Array_Clear` (`self.Volumes`))
  (bind _outactors (`GameplayStatics.GetAllActorsOfClass` "/Script/Engine.PointLight"))
  (for _array_element _outactors
    (if (and (not (> (`KismetArrayLibrary.Array_Length` (`self.GetAttachedActors` _array_element true)) 0)) (not (`KismetArrayLibrary.Array_Contains` (`Actor.Tags` _array_element) "ExcludeFromCalculations")))
      (`self.CreateVolume` _array_element)))
  (bind _outactors_2 (`GameplayStatics.GetAllActorsOfClass` "/Script/Engine.SpotLight"))
  (for _array_element_2 _outactors_2
    (if (and (not (> (`KismetArrayLibrary.Array_Length` (`self.GetAttachedActors` _array_element_2 true)) 0)) (not (`KismetArrayLibrary.Array_Contains` (`Actor.Tags` _array_element_2) "ExcludeFromCalculations")))
      (`self.CreateVolume` _array_element_2))))

(fn `CreateVolume`
  (params (Light :type "Actor Object Reference"))
  (bind _returnvalue (`self.K2_GetActorLocation` Light))
  (bind _aspoint_light (cast `PointLight` Light)
    (:`then`
      (bind _returnvalue_2 (`|SpawnActorFromClass` "/Game/Blueprints/LightDetection/BP_LightVolume_Sphere.BP_LightVolume_Sphere_C" (`KismetMathLibrary.MakeTransform` _returnvalue) "Undefined" "OverrideRootScale" null _aspoint_light (`LocalLightComponent.AttenuationRadius` (`PointLight.PointLightComponent` _aspoint_light)) null))
      (`self.K2_AttachToActor` _returnvalue_2 _aspoint_light "None" "SnapToTarget" "KeepWorld" "KeepWorld" true))
    (:`CastFailed`
      (bind _asspot_light (cast `SpotLight` Light))
      (bind _returnvalue_3 (`|SpawnActorFromClass` "/Game/Blueprints/LightDetection/BP_LightVolume_Sphere.BP_LightVolume_Sphere_C" (`KismetMathLibrary.MakeTransform` _returnvalue) "Undefined" "OverrideRootScale" null _asspot_light (`LocalLightComponent.AttenuationRadius` (`SpotLight.SpotLightComponent` _asspot_light)) null))
      (`self.K2_AttachToActor` _returnvalue_3 _asspot_light "None" "SnapToTarget" "KeepWorld" "KeepWorld" true))))

(fn `UserConstructionScript`)