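; Scene component that measures the light level at its position, ignoring its owner in occlusion checks.
; It sums contributions from registered LightVolumes, pruning out-of-range ones, and adds scaled intensity from each DirectionalLight whose visibility trace is unblocked.
; GetTotalLightLevelAtLocation samples another point by temporarily moving the component.
; GetStrongestLightInVicinity finds the brightest volume, excluding directional lights, and GatherLightLevel prints the total.
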(event `self.ReceiveBeginPlay`
  (`KismetArrayLibrary.Array_Add` (`self.ActorsToIgnore`) (`self.GetOwner`)))

(event `GatherLightLevel`
  (bind _lightlevel (`self.GetTotalLightLevel`))
  (`KismetSystemLibrary.PrintString` (`KismetStringLibrary.Conv_DoubleToString` _lightlevel)))

(event `self.ReceiveTick`
  (params (DeltaSeconds :type "Float (single-precision)")))

(fn `GetStrongestLightInVicinity`
  (returns (LightLevel :type "Float (double-precision)") (StrongestLightVolume :type "/Game/Blueprints/LightDetection/BP_LightVolume Object Reference"))
  (locals (LocalLightLevel :type "Float (double-precision)") (HighestLightLevel :type "Float (double-precision)") (VolumeToReturn :type "/Game/Blueprints/LightDetection/BP_LightVolume Object Reference"))
  (set `local.LocalLightLevel` 0.0)
  (`KismetArrayLibrary.Array_Clear` (`self.LightVolumesToRemove`))
  (for _array_element (`self.LightVolumes`)
    (if (`KismetSystemLibrary.IsValid` _array_element)
      (bind (_lightcontribution _outofrange) (`/Game/Blueprints/LightDetection/BP_LightVolume.GetLightContribution` _array_element (`self.K2_GetComponentLocation`) (`self.ActorsToIgnore`)))
      (if _outofrange
        (`KismetArrayLibrary.Array_Add` (`self.LightVolumesToRemove`) _array_element)
        (elif (> _lightcontribution (`local.HighestLightLevel`))
          (set `local.HighestLightLevel` _lightcontribution)
          (set `local.VolumeToReturn` _array_element)))))
  (for _array_element_2 (`self.LightVolumesToRemove`)
    (`KismetArrayLibrary.Array_RemoveItem` (`self.LightVolumes`) _array_element_2))
  (return (`local.HighestLightLevel`) (`local.VolumeToReturn`)))

(fn `GetTotalLightLevel`
  (returns (LightLevel :type "Float (double-precision)"))
  (locals (LocalLightLevel :type "Float (double-precision)"))
  (set `local.LocalLightLevel` 0.0)
  (`KismetArrayLibrary.Array_Clear` (`self.LightVolumesToRemove`))
  (for _array_element (`self.LightVolumes`)
    (if (`KismetSystemLibrary.IsValid` _array_element)
      (bind (_lightcontribution _outofrange) (`/Game/Blueprints/LightDetection/BP_LightVolume.GetLightContribution` _array_element (`self.K2_GetComponentLocation`) (`self.ActorsToIgnore`)))
      (if _outofrange
        (`KismetArrayLibrary.Array_Add` (`self.LightVolumesToRemove`) _array_element)
        (else
          (set `local.LocalLightLevel` (+ (`local.LocalLightLevel`) _lightcontribution))))))
  (for _array_element_2 (`self.LightVolumesToRemove`)
    (`KismetArrayLibrary.Array_RemoveItem` (`self.LightVolumes`) _array_element_2))
  (bind _outactors (`GameplayStatics.GetAllActorsOfClass` "/Script/Engine.DirectionalLight"))
  (for _array_element_3 _outactors
    (bind (_outhit _returnvalue) (`KismetSystemLibrary.LineTraceSingle` (`self.K2_GetComponentLocation`) (* (* (`Actor.GetActorForwardVector` _array_element_3) -1.0) 30000.0) "TraceTypeQuery1" false (`self.ActorsToIgnore`)))
    (if (not _returnvalue)
      (set `local.LocalLightLevel` (+ (`local.LocalLightLevel`) (* (`LightComponentBase.Intensity` (`Light.LightComponent` _array_element_3)) 100.0)))))
  (bind _output_get (set `self.LightLevel` (`local.LocalLightLevel`)))
  (return _output_get))

(fn `GetTotalLightLevelAtLocation`
  (params (Location :type "Vector Structure"))
  (returns (LightLevel :type "Float (double-precision)"))
  (locals (LocalLightLevel :type "Float (double-precision)") (OriginalLocation :type "Vector Structure"))
  (set `local.OriginalLocation` (`self.RelativeLocation`))
  (`self.K2_SetWorldLocation` Location)
  (set `local.LocalLightLevel` 0.0)
  (`KismetArrayLibrary.Array_Clear` (`self.LightVolumesToRemove`))
  (for _array_element (`self.LightVolumes`)
    (if (`KismetSystemLibrary.IsValid` _array_element)
      (bind (_lightcontribution _outofrange) (`/Game/Blueprints/LightDetection/BP_LightVolume.GetLightContribution` _array_element (`self.K2_GetComponentLocation`) (`self.ActorsToIgnore`)))
      (if _outofrange
        (`KismetArrayLibrary.Array_Add` (`self.LightVolumesToRemove`) _array_element)
        (else
          (set `local.LocalLightLevel` (+ (`local.LocalLightLevel`) _lightcontribution))))))
  (for _array_element_2 (`self.LightVolumesToRemove`)
    (`KismetArrayLibrary.Array_RemoveItem` (`self.LightVolumes`) _array_element_2))
  (bind _outactors (`GameplayStatics.GetAllActorsOfClass` "/Script/Engine.DirectionalLight"))
  (for _array_element_3 _outactors
    (bind (_outhit _returnvalue) (`KismetSystemLibrary.LineTraceSingle` (`self.K2_GetComponentLocation`) (* (* (`Actor.GetActorForwardVector` _array_element_3) -1.0) 30000.0) "TraceTypeQuery1" false (`self.ActorsToIgnore`)))
    (if (not _returnvalue)
      (set `local.LocalLightLevel` (+ (`local.LocalLightLevel`) (* (`LightComponentBase.Intensity` (`Light.LightComponent` _array_element_3)) 100.0)))))
  (bind _output_get (set `self.LightLevel` (`local.LocalLightLevel`)))
  (`self.K2_SetRelativeLocation` (`local.OriginalLocation`))
  (return _output_get))