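; Spotlight light volume for the light detection system that reports how much its light component lights a given location.
; GetLightContribution runs a Visibility trace from the actor and returns zero when blocked.
; Otherwise it gates intensity by the outer cone angle, applies linear falloff over the attenuation radius and a multiplier, then clamps the result.
; OutOfRange is set when the unfloored value drops well below zero, so only for in-cone points beyond the radius.
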(fn `GetLightContribution`
  (params (Location :type "Vector Structure") (ActorsToIgnore :type "Array of Actor Object Reference (by ref)"))
  (returns (LightContribution :type "Float (double-precision)") (OutOfRange :type Boolean))
  (bind _lightcomponent (`self.LightComponent`))
  (bind _attenuationradius (`LocalLightComponent.AttenuationRadius` _lightcomponent))
  (bind _returnvalue (`KismetMathLibrary.Normal` (- (`self.K2_GetActorLocation`) (`local.Location`))))
  (bind _returnvalue_2 (`KismetMathLibrary.Normal` (* (`SceneComponent.GetForwardVector` (`self.LightComponent`)) -1.0)))
  (bind (_returnvalue_x _returnvalue_y _returnvalue_z) (`KismetMathLibrary.BreakVector` (`KismetMathLibrary.Cross_VectorVector` _returnvalue_2 _returnvalue)))
  (bind _returnvalue_3 (* (`LightComponentBase.Intensity` _lightcomponent) (`KismetMathLibrary.SelectFloat` 1.0 0.0 (<= (`KismetMathLibrary.Abs` (* (`KismetMathLibrary.DegAcos` (`KismetMathLibrary.Dot_VectorVector` _returnvalue_2 _returnvalue)) (`KismetMathLibrary.SelectFloat` 1.0 -1.0 (> _returnvalue_z 0.0)))) (`SpotLightComponent.OuterConeAngle` _lightcomponent)))))
  (bind _returnvalue_4 (`KismetMathLibrary.FClamp` (* (* _returnvalue_3 (- 1.0 (/ (`KismetMathLibrary.Vector_Distance` Location (`self.K2_GetActorLocation`)) (`KismetMathLibrary.FClamp` _attenuationradius 0.001 _attenuationradius)))) (`self.ContributionMulitplier`)) -100.0 _returnvalue_3))
  (bind (_outhit _returnvalue_5) (`KismetSystemLibrary.LineTraceSingle` (`self.K2_GetActorLocation`) (`local.Location`) "TraceTypeQuery1" false (`local.ActorsToIgnore`)))
  (if _returnvalue_5
    (return 0.0 false)
    (else
      (return (`KismetMathLibrary.FClamp` _returnvalue_4 0.0 _returnvalue_3) (< _returnvalue_4 -50.0)))))

(fn `UserConstructionScript`
  (`parent.UserConstructionScript`))