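; Trigger volume that switches ambiance when the first-person character enters it.
; On construction it matches a linked level streaming volume's location, rotation and bounds, or falls back to a small default box.
; At BeginPlay it collapses the box and restores it after a short delay, so overlaps register afresh.
; On overlap, if NewAmbiance is set, it passes its Ambiance to the first BP_VibeManager found.
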(event `self.ReceiveBeginPlay`
  (bind _box (`self.Box`))
  (bind _output_get (set `self.BoxEntents` (`BoxComponent.BoxExtent` _box)))
  (`BoxComponent.SetBoxExtent` _box (0.0 0.0 0.0) true)
  (`KismetSystemLibrary.Delay` 1.0)
  (`BoxComponent.SetBoxExtent` _box _output_get true))

(event `self.Box.OnComponentBeginOverlap`
  (params (OverlappedComponent :type "PrimitiveComponent Object Reference") (OtherActor :type "Actor Object Reference") (OtherComp :type "PrimitiveComponent Object Reference") (OtherBodyIndex :type Integer) (bFromSweep :type Boolean) (SweepResult :type "HitResult Structure (by ref)"))
  (`KismetSystemLibrary.PrintString` "New Vibes!")
  (cast `/Game/ExtraContent/FirstPersonBP/Blueprints/FirstPersonCharacter` OtherActor)
  (bind _outactors (`GameplayStatics.GetAllActorsOfClass` "/Game/Blueprints/Volumes/BP_VibeManager.BP_VibeManager_C"))
  (if (`self.NewAmbiance`)
    (`/Game/Blueprints/Volumes/BP_VibeManager.NewAmbiance` (`|GetArrayItem` _outactors) (`self.Ambiance`))))

(fn `UserConstructionScript`
  (bind _levelstreamvol (`self.LevelStreamVol`))
  (bind _box (`self.Box`))
  (if (`KismetSystemLibrary.IsValid` _levelstreamvol)
    (`self.K2_SetActorLocation` (`self.K2_GetActorLocation` _levelstreamvol))
    (`BoxComponent.SetBoxExtent` _box (`.BoxExtent` (`KismetSystemLibrary.GetComponentBounds` (`Brush.BrushComponent` _levelstreamvol))) true)
    (`self.K2_SetActorRotation` (`self.K2_GetActorRotation` _levelstreamvol))
    (else
      (`BoxComponent.SetBoxExtent` _box (32.0 32.0 32.0) true))))