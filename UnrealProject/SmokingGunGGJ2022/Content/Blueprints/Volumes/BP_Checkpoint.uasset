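; Checkpoint trigger volume that autosaves when the first-person character enters a room numbered higher than the current one.
; On overlap it raises CurrentRoomNum on BP_SaveLoadManager, then writes a new SaveSlot1 object to the "Autosave" slot.
; The save holds room number, world-space spawn location and MultiTool modes and scans, but no spawn rotation.
; The construction script sizes the box and places a sphere at the spawn location and rotation.
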(event `self.Box.OnComponentBeginOverlap`
  (params (OverlappedComponent :type "PrimitiveComponent Object Reference") (OtherActor :type "Actor Object Reference") (OtherComp :type "PrimitiveComponent Object Reference") (OtherBodyIndex :type Integer) (bFromSweep :type Boolean) (SweepResult :type "HitResult Structure (by ref)"))
  (bind _asfirst_person_character (cast `/Game/ExtraContent/FirstPersonBP/Blueprints/FirstPersonCharacter` OtherActor))
  (bind _outactors (`GameplayStatics.GetAllActorsOfClass` "/Game/Blueprints/BP_SaveLoadManager.BP_SaveLoadManager_C"))
  (bind _output (`|GetArrayItem` _outactors))
  (if (< (`/Game/Blueprints/BP_SaveLoadManager.CurrentRoomNum` _output) (`self.RoomNum`))
    (set `/Game/Blueprints/BP_SaveLoadManager.CurrentRoomNum` (`self.RoomNum`) _output)
    (bind _returnvalue (`GameplayStatics.CreateSaveGameObject` "/Game/Blueprints/SaveSlot1.SaveSlot1_C"))
    (set `/Game/Blueprints/SaveSlot1.SpawnLocation` (`KismetMathLibrary.TransformLocation` (`self.GetTransform`) (`self.SpawnLocation`)) _returnvalue)
    (bind _multitool (`/Game/ExtraContent/FirstPersonBP/Blueprints/FirstPersonCharacter.MultiTool` _asfirst_person_character))
    (set `/Game/Blueprints/SaveSlot1.CollectedTools` (`/Game/Blueprints/Tools/BP_MultiTool.AvailableModes` _multitool) _returnvalue)
    (set `/Game/Blueprints/SaveSlot1.RoomNum` (`self.RoomNum`) _returnvalue)
    (set `/Game/Blueprints/SaveSlot1.Scanned` (`/Game/Blueprints/Tools/BP_MultiTool.Scanned` _multitool) _returnvalue)
    (`GameplayStatics.SaveGameToSlot` _returnvalue "Autosave")))

(fn `UserConstructionScript`
  (bind _sphere (`self.Sphere`))
  (`SceneComponent.K2_SetRelativeLocation` _sphere (`self.SpawnLocation`) false false)
  (`SceneComponent.K2_SetRelativeRotation` _sphere (`self.SpawnRotation`) false false)
  (`BoxComponent.SetBoxExtent` (`self.Box`) (`self.Extents`) true))