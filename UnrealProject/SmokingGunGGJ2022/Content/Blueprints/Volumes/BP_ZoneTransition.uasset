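; BP_ZoneTransition is a trigger volume that tells the BP_VibeManager which zone the player has entered.
; When the player pawn overlaps its Box, it finds the first BP_VibeManager in the level and compares that manager's CurrentZone to its own ZoneName.
; On a change, it updates CurrentZone and, if its NewAmbiance flag is set, passes its Ambiance to the manager's NewAmbiance call.
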(event `self.Box.OnComponentBeginOverlap`
  (params (OverlappedComponent :type "PrimitiveComponent Object Reference") (OtherActor :type "Actor Object Reference") (OtherComp :type "PrimitiveComponent Object Reference") (OtherBodyIndex :type Integer) (bFromSweep :type Boolean) (SweepResult :type "HitResult Structure (by ref)"))
  (bind _zonename (`self.ZoneName`))
  (if (== OtherActor (`GameplayStatics.GetPlayerPawn` 0))
    (bind _outactors (`GameplayStatics.GetAllActorsOfClass` "/Game/Blueprints/Volumes/BP_VibeManager.BP_VibeManager_C"))
    (bind _output (`|GetArrayItem` _outactors))
    (if (not (`KismetStringLibrary.EqualEqual_StrStr` (`/Game/Blueprints/Volumes/BP_VibeManager.CurrentZone` _output) _zonename))
      (set `/Game/Blueprints/Volumes/BP_VibeManager.CurrentZone` _zonename _output)
      (`|ExecutionSequence`
        (:`then_0`
          (if (`self.NewAmbiance`)
            (`/Game/Blueprints/Volumes/BP_VibeManager.NewAmbiance` _output (`self.Ambiance`))))))))

(fn `UserConstructionScript`)