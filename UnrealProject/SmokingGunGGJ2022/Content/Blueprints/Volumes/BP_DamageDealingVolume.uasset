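; BP_DamageDealingVolume is a box volume that repeatedly damages the FirstPersonCharacter while it stays inside.
; Begin overlap stores the character and starts a fast looping timer that applies Damage on each tick of the timer; end overlap clears it.
; On BeginPlay the box shrinks to zero extent, then is set to a fixed size after a short delay, updating overlaps both times.
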(event `self.ReceiveBeginPlay`
  (bind _box (`self.Box`))
  (`BoxComponent.SetBoxExtent` _box (0.0 0.0 0.0) true)
  (`KismetSystemLibrary.Delay` 1.0)
  (`BoxComponent.SetBoxExtent` _box (32.0 32.0 32.0) true))

(event `self.Box.OnComponentBeginOverlap`
  (params (OverlappedComponent :type "PrimitiveComponent Object Reference") (OtherActor :type "Actor Object Reference") (OtherComp :type "PrimitiveComponent Object Reference") (OtherBodyIndex :type Integer) (bFromSweep :type Boolean) (SweepResult :type "HitResult Structure (by ref)"))
  (bind _asfirst_person_character (cast `/Game/ExtraContent/FirstPersonBP/Blueprints/FirstPersonCharacter` OtherActor))
  (set `self.Player` _asfirst_person_character)
  (bind _returnvalue (`KismetSystemLibrary.K2_SetTimerDelegate` (delegate `DealDamage`) 0.03 true))
  (set `self.DamageTimer` _returnvalue))

(event `self.Box.OnComponentEndOverlap`
  (params (OverlappedComponent :type "PrimitiveComponent Object Reference") (OtherActor :type "Actor Object Reference") (OtherComp :type "PrimitiveComponent Object Reference") (OtherBodyIndex :type Integer))
  (cast `/Game/ExtraContent/FirstPersonBP/Blueprints/FirstPersonCharacter` OtherActor)
  (`KismetSystemLibrary.K2_ClearAndInvalidateTimerHandle` (`self.DamageTimer`)))

(event `DealDamage`
  (`GameplayStatics.ApplyDamage` (`self.Player`) (`self.Damage`)))

(fn `UserConstructionScript`)