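; BP_LargeLevelCanister is a pickup actor that unlocks a mode on the player's MultiTool.
; BeginPlay caches the FirstPersonCharacter player as PlayerRef.
; When the player hits it, it prints the player's name, adds its EnumToolMode to the tool's AvailableModes, calls InitCannisters and destroys itself.
; It triggers on physical hit, as the overlap event is unused.
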(event `self.ReceiveBeginPlay`
  (bind _asfirst_person_character (cast `/Game/ExtraContent/FirstPersonBP/Blueprints/FirstPersonCharacter` (`GameplayStatics.GetPlayerCharacter` 0)))
  (set `self.PlayerRef` _asfirst_person_character))

(event `self.ReceiveHit`
  (params (MyComp :type "PrimitiveComponent Object Reference") (Other :type "Actor Object Reference") (OtherComp :type "PrimitiveComponent Object Reference") (bSelfMoved :type Boolean) (HitLocation :type "Vector Structure") (HitNormal :type "Vector Structure") (NormalImpulse :type "Vector Structure") (Hit :type "HitResult Structure (by ref)"))
  (bind _playerref (`self.PlayerRef`))
  (bind _multitool (`/Game/ExtraContent/FirstPersonBP/Blueprints/FirstPersonCharacter.MultiTool` (`self.PlayerRef`)))
  (if (== Other _playerref)
    (`KismetSystemLibrary.PrintString` (`KismetSystemLibrary.GetDisplayName` _playerref))
    (`KismetArrayLibrary.Array_Add` (`/Game/Blueprints/Tools/BP_MultiTool.AvailableModes` _multitool) (`self.EnumToolMode`))
    (`/Game/Blueprints/Tools/BP_MultiTool.InitCannisters` _multitool)
    (`self.K2_DestroyActor`)))

(fn `UserConstructionScript`)