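; Player multi-tool with scanner, laser and plasma flare fire modes, a selectable but unimplemented Foliage Clone mode, and a flickering flashlight.
; ScrollEquipped skips unavailable modes and animates canister position and color.
; The timer-driven laser aims by camera trace, then traces from the tool to damage targets or show reflection off reflective monsters.
; Laser and flare drain a shared battery shown as canister fill; scans print matching names for Scannable-tagged actors.
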(event `self.ReceiveBeginPlay`
  (`self.ScrollEquipped` false)
  (`self.InitCannisters`))

(event `BeginFiring`
  (if (> (`self.Battery`) 0.0)
    (switch `/Game/Blueprints/Tools/Enum_ToolModes` (`self.Mode`)
      (:`NewEnumerator3`
        (`self.Scan`))
      (:`NewEnumerator0`
        (`self.StartLaser`))
      (:`NewEnumerator2`
        (`self.FireFlare`)))))

(event `StopFiring`
  (`self.StopLaser`))

(event `FireFlare`
  (bind (_returnvalue_location _returnvalue_rotation) (`KismetMathLibrary.BreakTransform` (`SceneComponent.K2_GetComponentToWorld` (`self.FireLocation`))))
  (if (and (> (`self.Battery`) 0.0) (`self.CanFireFlare`))
    (set `self.CanFireFlare` false)
    (`|SpawnActorFromClass` "/Game/Blueprints/Tools/BP_PlasmaFlare.BP_PlasmaFlare_C" (`KismetMathLibrary.MakeTransform` _returnvalue_location _returnvalue_rotation) "Undefined" "OverrideRootScale" null null)
    (`/Game/ExtraContent/FirstPersonBP/Blueprints/FirstPersonCharacter.FireKickback` (`self.Player`))
    (`GameplayStatics.PlaySound2D` "/Game/ExtraContent/FirstPerson/Audio/FirstPersonTemplateWeaponFire02.FirstPersonTemplateWeaponFire02" 0.4 1.0 0.0 null null)
    (`/Game/Blueprints/BL_Senses.ActorNoise` (`GameplayStatics.GetPlayerPawn` 0) 3.0)
    (`self.DrainBattery` 0.25)
    (`KismetSystemLibrary.Delay` (`self.FlareCooldownTime`))
    (set `self.CanFireFlare` true)))

(event `StartLaser`
  (bind _returnvalue (`KismetSystemLibrary.K2_SetTimerDelegate` (delegate `Laser`) 0.03 true))
  (set `self.LaserTimer` _returnvalue)
  (`SceneComponent.SetHiddenInGame` (`self.FBX_LaserPlane`) false false)
  (`ActorComponent.SetActive` (`self.P_Sparks_Laser`) true false)
  (`LocalLightComponent.SetAttenuationRadius` (`self.PointLight`) 100.0)
  (`AudioComponent.Play` (`self.WAV_Laser_Engage`) 0.0)
  (`AudioComponent.FadeIn` (`self.WAV_Laser_Loop`) 0.5 1.0 0.0 "Linear"))

(event `Laser`
  (bind _returnvalue (`GameplayStatics.GetPlayerCameraManager` 0))
  (bind _pointlight (`self.PointLight`))
  (bind _fbx_laserplane (`self.FBX_LaserPlane`))
  (bind _fbx_laserplane_refleced (`self.FBX_LaserPlane_Refleced`))
  (bind _fbx_laserplane_2 (`self.FBX_LaserPlane`))
  (bind _returnvalue_2 (`SceneComponent.K2_GetComponentLocation` _fbx_laserplane))
  (bind _returnvalue_3 (`PlayerCameraManager.GetCameraLocation` _returnvalue))
  (bind (_outhit _returnvalue_4) (`KismetSystemLibrary.LineTraceSingle` :`Start` _returnvalue_3 :`End` (+ _returnvalue_3 (* (`self.GetActorForwardVector` _returnvalue) 5000.0)) :`TraceChannel` "TraceTypeQuery1" :`DrawTime` 0.1))
  (if _returnvalue_4
    (`SceneComponent.K2_SetWorldRotation` _fbx_laserplane_2 (`KismetMathLibrary.FindLookAtRotation` (`SceneComponent.K2_GetComponentLocation` _fbx_laserplane_2) (`.Location` (`GameplayStatics.BreakHitResult` _outhit))) false false))
  (bind (_outhit_2 _returnvalue_5) (`KismetSystemLibrary.LineTraceSingle` _returnvalue_2 (+ _returnvalue_2 (* (`SceneComponent.GetForwardVector` _fbx_laserplane) 5000.0)) "TraceTypeQuery1" false (`|MakeArray` (`self.Player`) :!type "Actor Object Reference") "None" true (struct :`R` 1.0 :`A` 1.0) (struct :`G` 1.0 :`A` 1.0) 0.1))
  (if _returnvalue_5
    (bind (_bblockinghit _binitialoverlap _time _distance _location _impactpoint _normal _impactnormal _physmat _hitactor) (`GameplayStatics.BreakHitResult` _outhit_2))
    (bind _asbp_monster (cast `/Game/Blueprints/Monsters/BP_Monster` _hitactor)
      (:`then`
        (bind _reflectlaser (`/Game/Blueprints/Monsters/BP_Monster.ReflectLaser` _asbp_monster))
        (`SceneComponent.SetHiddenInGame` _fbx_laserplane_refleced (not _reflectlaser) false)
        (if _reflectlaser
          (`SceneComponent.K2_SetWorldLocation` _fbx_laserplane_refleced _location false false)
          (`SceneComponent.K2_SetWorldRotation` _fbx_laserplane_refleced (`KismetMathLibrary.Conv_VectorToRotator` _normal) false false)
          (else
            (`GameplayStatics.ApplyDamage` _hitactor (`self.LaserDamage`) :!label _label))))
      (:`CastFailed`
        (`SceneComponent.SetHiddenInGame` _fbx_laserplane_refleced true false)
        (goto _label)))
    (`SceneComponent.SetRelativeScale3D` (`self.FBX_LaserPlane`) (`KismetMathLibrary.MakeVector` _distance 0.1 0.1))
    (`SceneComponent.K2_SetWorldLocation` (`self.P_Sparks_Laser`) _location false false)
    (`SceneComponent.K2_SetWorldLocation` _pointlight (+ _location (* _normal 25.0)) false false)
    (`LocalLightComponent.SetAttenuationRadius` _pointlight (`KismetMathLibrary.RandomFloatInRange` 0.0 100.0))
    (`/Game/Blueprints/BL_Senses.ActorNoise` (`GameplayStatics.GetPlayerPawn` 0) 1.0)
    (`self.DrainBattery` 0.001)))

(event `StopLaser`
  (`KismetSystemLibrary.K2_ClearAndInvalidateTimerHandle` (`self.LaserTimer`))
  (`SceneComponent.SetHiddenInGame` (`self.FBX_LaserPlane`) true false)
  (`SceneComponent.SetHiddenInGame` (`self.FBX_LaserPlane_Refleced`) true false)
  (`ActorComponent.SetActive` (`self.P_Sparks_Laser`) false false)
  (`LocalLightComponent.SetAttenuationRadius` (`self.PointLight`) 0.0)
  (`AudioComponent.FadeOut` (`self.WAV_Laser_Loop`) 0.1 0.0 "Linear")
  (`AudioComponent.FadeOut` (`self.WAV_Laser_Engage`) 0.1 0.0 "Linear"))

(event `ToggleFlashlight`
  (bind _spotlight (`self.SpotLight`))
  (bind _flashlightlightvol (`self.FlashlightLightVol`))
  (`GameplayStatics.PlaySound2D` "/Game/Blueprints/Character/Audio/WAV_Click.WAV_Click" 1.0 1.0 0.0 null null)
  (if (> (`self.Battery`) 0.0)
    (bind _output_get (set `self.FlashlightOn` (not (`self.FlashlightOn`))))
    (if _output_get
      (`LocalLightComponent.SetAttenuationRadius` _spotlight 6000.0)
      (`/Game/Blueprints/LightDetection/BP_LightVolume.Set New Radius` _flashlightlightvol 2000.0)
      (bind _returnvalue (`KismetSystemLibrary.K2_SetTimerDelegate` (delegate `FlashlightBatteryDrain`) 1.0 true))
      (set `self.FlashlightTimer` _returnvalue)
      (else
        (`LocalLightComponent.SetAttenuationRadius` _spotlight 0.0 :!label _label_2)
        (`/Game/Blueprints/LightDetection/BP_LightVolume.Set New Radius` _flashlightlightvol 0.0)
        (`KismetSystemLibrary.K2_ClearAndInvalidateTimerHandle` (`self.FlashlightTimer`))))))

(event `KillFlashlight`
  (set `self.FlashlightOn` false)
  (goto _label_2))

(event `FlashlightBatteryDrain`
  (`self.DrainBattery` 0.0)
  (if (== (`KismetMathLibrary.RandomIntegerInRange` 0 55) 0)
    (`self.FlashlightFlicker`)))

(event `FlashlightFlicker`
  (bind (_direction _power) (`Timeline|Flicker`)
    (:`Update`
      (`LocalLightComponent.SetAttenuationRadius` (`self.SpotLight`) (* _power 6000.0))
      (`/Game/Blueprints/LightDetection/BP_LightVolume.Set New Radius` (`self.FlashlightLightVol`) (* _power 2000.0)))))

(event `DrainBattery`
  (params (Drain :type "Float (double-precision)"))
  (bind _output_get (set `self.Battery` (`KismetMathLibrary.FClamp` (- (`self.Battery`) Drain))))
  (`MaterialInstanceDynamic.SetScalarParameterValue` (`self.MainCannisterMat`) "Fill" _output_get)
  (if (== _output_get 0.0)
    (`self.StopFiring`)
    (`self.KillFlashlight`)))

(event `ScrollEquipped`
  (params (Dir :type Boolean) (Skip :type Boolean))
  (bind _mode (`self.Mode`))
  (bind _previousmodecan (`self.PreviousModeCan`))
  (bind _currentmodecan (`self.CurrentModeCan`))
  (bind _asmaterial_instance_dynamic (cast `MaterialInstanceDynamic` (`PrimitiveComponent.GetMaterial` _currentmodecan 1) :!pure true))
  (bind _asmaterial_instance_dynamic_2 (cast `MaterialInstanceDynamic` (`PrimitiveComponent.GetMaterial` _previousmodecan 1) :!pure true))
  (if (`self.isSwitchingMode`)
    (`|ExecutionSequence`
      (:`then_0`
        (`MaterialInstanceDynamic.SetScalarParameterValue` (cast `MaterialInstanceDynamic` (`PrimitiveComponent.GetMaterial` (`self.PreviousModeCan`) 1) :!pure true) "Brightness" 0.0))
      (:`then_1`
        (if (not Skip) :!label _label_3
          (set `self.PreviousModeCan` (select `/Game/Blueprints/Tools/Enum_ToolModes` _mode :`NewEnumerator3` (`self.ScannerCan`) :`NewEnumerator0` (`self.LaserCan`) :`NewEnumerator2` (`self.FlareCan`) :`NewEnumerator1` (`self.CloneCan`))))
        (bind _output_get (set `self.Mode` (select `bool` Dir :`false` (select `/Game/Blueprints/Tools/Enum_ToolModes` _mode :`NewEnumerator3` "NewEnumerator0" :`NewEnumerator0` "NewEnumerator2" :`NewEnumerator2` "NewEnumerator1" :`NewEnumerator1` "NewEnumerator3" :!type "/Game/Blueprints/Tools/Enum_ToolModes Enum") :`true` (select `/Game/Blueprints/Tools/Enum_ToolModes` _mode :`NewEnumerator3` "NewEnumerator1" :`NewEnumerator0` "NewEnumerator3" :`NewEnumerator2` "NewEnumerator0" :`NewEnumerator1` "NewEnumerator2" :!type "/Game/Blueprints/Tools/Enum_ToolModes Enum"))))
        (if (`KismetArrayLibrary.Array_Contains` (`self.AvailableModes`) _output_get)
          (set `self.CurrentModeCan` (select `/Game/Blueprints/Tools/Enum_ToolModes` (`self.Mode`) :`NewEnumerator3` (`self.ScannerCan`) :`NewEnumerator0` (`self.LaserCan`) :`NewEnumerator2` (`self.FlareCan`) :`NewEnumerator1` (`self.CloneCan`)))
          (set `self.isSwitchingMode` true)
          (bind (_direction _jut) (`Timeline|SwitchCan` :!via `PlayFromStart`)
            (:`Update`
              (bind _returnvalue (- 1.0 _jut))
              (`SceneComponent.K2_SetRelativeLocation` _previousmodecan (`KismetMathLibrary.MakeVector` (* _returnvalue 2.0)) false false)
              (`SceneComponent.K2_SetRelativeLocation` _currentmodecan (`KismetMathLibrary.MakeVector` (* _jut 2.0)) false false)
              (`MaterialInstanceDynamic.SetScalarParameterValue` _asmaterial_instance_dynamic_2 "Brightness" _returnvalue)
              (`MaterialInstanceDynamic.SetScalarParameterValue` _asmaterial_instance_dynamic "Brightness" _jut)
              (bind _returnvalue_2 (`MaterialInstanceDynamic.K2_GetVectorParameterValue` _asmaterial_instance_dynamic_2 "Color"))
              (bind _returnvalue_3 (`MaterialInstanceDynamic.K2_GetVectorParameterValue` _asmaterial_instance_dynamic "Color"))
              (`MaterialInstanceDynamic.SetVectorParameterValue` (`self.MainCannisterMat`) "Color" (`KismetMathLibrary.LinearColorLerp` _returnvalue_2 _returnvalue_3 _jut)))
            (:`Finished`
              (set `self.isSwitchingMode` false)))
          (else
            (`self.ScrollEquipped` Dir true)))))
    (else
      (goto _label_3))))

(event `Scan`
  (bind _scanobject (`self.scanObject`))
  (bind _returnvalue (`SceneComponent.K2_GetComponentLocation` (`self.SM_ScanPlanes`)))
  (if (not (`self.isScanning`))
    (set `self.isScanning` true)
    (set `self.scanObject` null)
    (`SceneComponent.SetHiddenInGame` (`self.SM_ScanPlanes`) false false)
    (bind (_direction _movement) (`Timeline|ScanAnim` :!via `PlayFromStart`)
      (:`Update`
        (`SceneComponent.K2_SetRelativeRotation` (`self.SM_ScanPlanes`) (`KismetMathLibrary.MakeRotator` (+ (* _movement 25.0) 90.0)) false false)
        (bind (_outhit _returnvalue_2) (`KismetSystemLibrary.LineTraceSingle` _returnvalue (+ _returnvalue (* (`self.GetActorForwardVector` self) 5000.0)) "TraceTypeQuery1"))
        (if _returnvalue_2
          (bind (_bblockinghit _binitialoverlap _time _distance _location _impactpoint _normal _impactnormal _physmat _hitactor) (`GameplayStatics.BreakHitResult` _outhit))
          (`SceneComponent.SetWorldScale3D` (`self.SM_ScanPlanes`) (`KismetMathLibrary.MakeVector` 2.0 (/ (+ _distance 1000.0) 100.0) 5.0))
          (if (not (`KismetSystemLibrary.IsValid` (`self.scanObject`)))
            (if (`self.ActorHasTag` _hitactor "Scannable")
              (set `self.scanObject` _hitactor)))))
      (:`Finished`
        (set `self.isScanning` false)
        (`SceneComponent.SetHiddenInGame` (`self.SM_ScanPlanes`) true false)
        (if (`KismetSystemLibrary.IsValid` _scanobject)
          (`self.GetScanInfo` _scanobject))))))

(fn `GetScanInfo`
  (params (ScannedActor :type "Actor Object Reference"))
  (for _array_element (`self.scanInfo`)
    (bind (_actor _name) (break `/Game/Blueprints/Tools/Struct_ScanInfo` _array_element))
    (if (== _actor (`GameplayStatics.GetObjectClass` ScannedActor))
      (`KismetSystemLibrary.PrintString` _name true true (struct :`G` 0.66 :`B` 1.0 :`A` 1.0) 10.0))))

(fn `InitCannisters`
  (for _array_element (`self.AvailableModes`)
    (`SceneComponent.SetHiddenInGame` (select `/Game/Blueprints/Tools/Enum_ToolModes` _array_element :`NewEnumerator3` (`self.ScannerCanRoot`) :`NewEnumerator0` (`self.LaserCanRoot`) :`NewEnumerator2` (`self.FlareCanRoot`) :`NewEnumerator1` (`self.CloneCanRoot`)) false true)))

(fn `UserConstructionScript`
  (bind _returnvalue (`KismetMaterialLibrary.CreateDynamicMaterialInstance` "/Game/Blueprints/Tools/Mesh/M_Cannister.M_Cannister"))
  (bind _output_get (set `self.MainCannisterMat` _returnvalue))
  (`PrimitiveComponent.SetMaterial` (`self.SM_MultiTool`) 1 _output_get)
  (bind _returnvalue_2 (`KismetMaterialLibrary.CreateDynamicMaterialInstance` "/Game/Blueprints/Tools/Mesh/M_Cannister_Simple.M_Cannister_Simple"))
  (bind _output_get_2 (set `self.LaserCanMat` _returnvalue_2))
  (`PrimitiveComponent.SetMaterial` (`self.LaserCan`) 1 _output_get_2)
  (`MaterialInstanceDynamic.SetVectorParameterValue` _output_get_2 "Color" (struct :`R` 1.0 :`G` 0.47932 :`A` 1.0))
  (bind _returnvalue_3 (`KismetMaterialLibrary.CreateDynamicMaterialInstance` "/Game/Blueprints/Tools/Mesh/M_Cannister_Simple.M_Cannister_Simple"))
  (bind _output_get_3 (set `self.FlareCanMat` _returnvalue_3))
  (`PrimitiveComponent.SetMaterial` (`self.FlareCan`) 1 _output_get_3)
  (`MaterialInstanceDynamic.SetVectorParameterValue` _output_get_3 "Color" (struct :`R` 1.0 :`A` 1.0))
  (bind _returnvalue_4 (`KismetMaterialLibrary.CreateDynamicMaterialInstance` "/Game/Blueprints/Tools/Mesh/M_Cannister_Simple.M_Cannister_Simple"))
  (bind _output_get_4 (set `self.CloneCanMat` _returnvalue_4))
  (`PrimitiveComponent.SetMaterial` (`self.CloneCan`) 1 _output_get_4)
  (`MaterialInstanceDynamic.SetVectorParameterValue` _output_get_4 "Color" (struct :`G` 1.0 :`B` 0.984843 :`A` 1.0))
  (bind _returnvalue_5 (`KismetMaterialLibrary.CreateDynamicMaterialInstance` "/Game/Blueprints/Tools/Mesh/M_Cannister_Simple.M_Cannister_Simple"))
  (bind _output_get_5 (set `self.EXTRATOOLCanMat` _returnvalue_5))
  (`PrimitiveComponent.SetMaterial` (`self.ScannerCan`) 1 _output_get_5)
  (`MaterialInstanceDynamic.SetVectorParameterValue` _output_get_5 "Color" (struct :`G` 1.0 :`B` 0.013883 :`A` 1.0)))