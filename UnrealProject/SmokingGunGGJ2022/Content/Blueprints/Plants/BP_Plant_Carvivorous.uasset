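; Carnivorous plant that sleeps in low light and lashes its tongue at nearby pawns when lit.
; The inherited UpdateLighting compares probe illumination to a threshold, driving a timeline that closes or reopens the jaws and tongue.
; Pawns entering AttackSphere become the target: looping timers yaw the tongue toward them, while Attack re-arms itself until the target leaves or the plant sleeps.
; Attacks are animation-only, with no damage applied here.
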(event `self.ReceiveBeginPlay`)

(event `Close`
  (set `self.Asleep` true)
  (`SkeletalMeshComponent.PlayAnimation` (`self.SM_Carnivorous_Tongue`) "/Game/Environment/Plants/Carnivorous/Anim_Carnivorous_Tongue_Retract.Anim_Carnivorous_Tongue_Retract" false)
  (bind (_direction _float) (`Timeline|Close_Anim` :!via `PlayFromStart` :!label _label)
    (:`Update`
      (`SceneComponent.K2_SetRelativeRotation` (`self.JawSmall`) (`KismetMathLibrary.MakeRotator` 0.0 (* _float -20.0) 180.0) false false)
      (`SceneComponent.K2_SetRelativeRotation` (`self.JawBig`) (`KismetMathLibrary.MakeRotator` 0.0 (* _float -10.0)) false false)
      (`SceneComponent.SetHiddenInGame` (`self.SM_Carnivorous_Tongue`) (select `ETimelineDirection` _direction :`Forward` true) false))))

(event `Open`
  (bind _sm_carnivorous_tongue (`self.SM_Carnivorous_Tongue`))
  (set `self.Asleep` false)
  (`SceneComponent.SetHiddenInGame` _sm_carnivorous_tongue false false)
  (`SkeletalMeshComponent.PlayAnimation` _sm_carnivorous_tongue "/Game/Environment/Plants/Carnivorous/Anim_Carnivorous_Tongue_Unfurl.Anim_Carnivorous_Tongue_Unfurl" false)
  (goto _label :!via `ReverseFromEnd`))

(event `TrackTarget`
  (bind _sm_carnivorous_tongue (`self.SM_Carnivorous_Tongue`))
  (bind (_returnvalue_roll _returnvalue_pitch) (`KismetMathLibrary.BreakRotator` (`SceneComponent.K2_GetComponentRotation` _sm_carnivorous_tongue)))
  (bind (_returnvalue_roll_2 _returnvalue_pitch_2 _returnvalue_yaw) (`KismetMathLibrary.BreakRotator` (`KismetMathLibrary.FindLookAtRotation` (`SceneComponent.K2_GetComponentLocation` _sm_carnivorous_tongue) (`self.K2_GetActorLocation` (`self.Target`)))))
  (`SceneComponent.K2_SetWorldRotation` _sm_carnivorous_tongue (`KismetMathLibrary.MakeRotator` _returnvalue_roll _returnvalue_pitch (+ _returnvalue_yaw -90.0)) false false))

(event `Attack`
  (if (and (`KismetSystemLibrary.IsValid` (`self.Target`)) (not (`self.Asleep`)))
    (`SkeletalMeshComponent.PlayAnimation` (`self.SM_Carnivorous_Tongue`) "/Game/Environment/Plants/Carnivorous/Anim_Carnivorous_Tongue_Attack.Anim_Carnivorous_Tongue_Attack" false)
    (bind _returnvalue (`KismetSystemLibrary.K2_SetTimerDelegate` (delegate `Attack`) 2.5))
    (set `self.AttackTimer` _returnvalue)
    (else
      (`SkeletalMeshComponent.PlayAnimation` (`self.SM_Carnivorous_Tongue`) "/Game/Environment/Plants/Carnivorous/SM_Carnivorous_Tongue_Idle_Armature_Attack.SM_Carnivorous_Tongue_Idle_Armature_Attack" true))))

(event `self.AttackSphere.OnComponentBeginOverlap`
  (params (OverlappedComponent :type "PrimitiveComponent Object Reference") (OtherActor :type "Actor Object Reference") (OtherComp :type "PrimitiveComponent Object Reference") (OtherBodyIndex :type Integer) (bFromSweep :type Boolean) (SweepResult :type "HitResult Structure (by ref)"))
  (bind _aspawn (cast `Pawn` OtherActor))
  (set `self.Target` _aspawn)
  (bind _returnvalue (`KismetSystemLibrary.K2_SetTimerDelegate` (delegate `TrackTarget`) 0.03 true))
  (set `self.TrackingTimer` _returnvalue)
  (`self.Attack`))

(event `self.AttackSphere.OnComponentEndOverlap`
  (params (OverlappedComponent :type "PrimitiveComponent Object Reference") (OtherActor :type "Actor Object Reference") (OtherComp :type "PrimitiveComponent Object Reference") (OtherBodyIndex :type Integer))
  (if (== OtherActor (`self.Target`))
    (set `self.Target` null)
    (`KismetSystemLibrary.K2_ClearAndInvalidateTimerHandle` (`self.TrackingTimer`))))

(fn `UpdateLighting`
  (`parent.UpdateLighting`)
  (if (< (`/Game/IlluminationDetection/Blueprints/IlluminationComponents/BP_IlluminationProbe.ProbeIllumination` (`self.BP_IlluminationProbe`)) (`self.LightEffectTriggerValue`))
    (`self.Close`)
    (else
      (`self.Open`))))

(fn `UserConstructionScript`)