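; Carnivorous plant hazard that attacks pawns with its tongue and sleeps with its jaws shut when the illumination probe reads below a threshold.
; A detect sphere sets the target and runs a looping timer that eases tongue yaw toward it.
; An attack sphere starts a self-rescheduling bite that applies delayed damage.
; Sleep blocks attacks and cuts incoming damage to a token amount, and death clears both timers and disables collision.
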(event `self.ReceiveBeginPlay`
  (`parent.ReceiveBeginPlay`))

(event `Close`
  (set `self.Asleep` true)
  (`SkeletalMeshComponent.PlayAnimation` (`self.SM_Carnivorous_Tongue`) "/Game/Environment/Plants/Carnivorous/Anim_Carnivorous_Tongue_Retract.Anim_Carnivorous_Tongue_Retract" false)
  (bind (_direction _float) (`Timeline|Close_Anim` :!via `PlayFromStart` :!label _label)
    (:`Update`
      (`SceneComponent.K2_SetRelativeRotation` (`self.JawSmall`) (`KismetMathLibrary.MakeRotator` 0.0 (* _float -20.0) 180.0) false false)
      (`SceneComponent.K2_SetRelativeRotation` (`self.JawBig`) (`KismetMathLibrary.MakeRotator` 0.0 (* _float -10.0)) false false)
      (`SceneComponent.SetHiddenInGame` (`self.SM_Carnivorous_Tongue`) (select `ETimelineDirection` _direction :`Forward` true) false))))

(event `Open`
  (bind _sm_carnivorous_tongue (`self.SM_Carnivorous_Tongue`))
  (set `self.Asleep` false)
  (`SceneComponent.SetHiddenInGame` _sm_carnivorous_tongue false false)
  (`SkeletalMeshComponent.PlayAnimation` _sm_carnivorous_tongue "/Game/Environment/Plants/Carnivorous/Anim_Carnivorous_Tongue_Unfurl.Anim_Carnivorous_Tongue_Unfurl" false)
  (goto _label :!via `ReverseFromEnd`))

(event `TrackTarget`
  (bind _sm_carnivorous_tongue (`self.SM_Carnivorous_Tongue`))
  (bind (_returnvalue_roll _returnvalue_pitch _returnvalue_yaw) (`KismetMathLibrary.BreakRotator` (`SceneComponent.K2_GetComponentRotation` _sm_carnivorous_tongue)))
  (bind (_returnvalue_roll_2 _returnvalue_pitch_2) (`KismetMathLibrary.BreakRotator` (`SceneComponent.K2_GetComponentRotation` _sm_carnivorous_tongue)))
  (bind (_returnvalue_roll_3 _returnvalue_pitch_3 _returnvalue_yaw_2) (`KismetMathLibrary.BreakRotator` (`KismetMathLibrary.FindLookAtRotation` (`SceneComponent.K2_GetComponentLocation` _sm_carnivorous_tongue) (`self.K2_GetActorLocation` (`self.OurTarget`)))))
  (`SceneComponent.K2_SetWorldRotation` _sm_carnivorous_tongue (`KismetMathLibrary.MakeRotator` _returnvalue_roll_2 _returnvalue_pitch_2 (`KismetMathLibrary.Lerp` _returnvalue_yaw (+ _returnvalue_yaw_2 -90.0) 0.12)) false false))

(event `Attack`
  (if (and (`KismetSystemLibrary.IsValid` (`self.OurTarget`)) (not (`self.Asleep`)) (not (`self.Dead`)))
    (`SkeletalMeshComponent.PlayAnimation` (`self.SM_Carnivorous_Tongue`) "/Game/Environment/Plants/Carnivorous/Anim_Carnivorous_Tongue_Attack.Anim_Carnivorous_Tongue_Attack" false)
    (`KismetSystemLibrary.Delay` 0.8)
    (`GameplayStatics.ApplyDamage` (`self.OurTarget`) 33.400002)
    (bind _returnvalue (`KismetSystemLibrary.K2_SetTimerDelegate` (delegate `Attack`) 1.5))
    (set `self.AttackTimer` _returnvalue)
    (else
      (`SkeletalMeshComponent.PlayAnimation` (`self.SM_Carnivorous_Tongue`) "/Game/Environment/Plants/Carnivorous/SM_Carnivorous_Tongue_Idle_Armature_Attack.SM_Carnivorous_Tongue_Idle_Armature_Attack" true))))

(event `self.AttackSphere.OnComponentBeginOverlap`
  (params (OverlappedComponent :type "PrimitiveComponent Object Reference") (OtherActor :type "Actor Object Reference") (OtherComp :type "PrimitiveComponent Object Reference") (OtherBodyIndex :type Integer) (bFromSweep :type Boolean) (SweepResult :type "HitResult Structure (by ref)"))
  (`self.Attack`))

(event `self.AttackSphere.OnComponentEndOverlap`
  (params (OverlappedComponent :type "PrimitiveComponent Object Reference") (OtherActor :type "Actor Object Reference") (OtherComp :type "PrimitiveComponent Object Reference") (OtherBodyIndex :type Integer))
  (`KismetSystemLibrary.K2_ClearAndInvalidateTimerHandle` (`self.AttackTimer`)))

(event `self.DetectSphere.OnComponentBeginOverlap`
  (params (OverlappedComponent :type "PrimitiveComponent Object Reference") (OtherActor :type "Actor Object Reference") (OtherComp :type "PrimitiveComponent Object Reference") (OtherBodyIndex :type Integer) (bFromSweep :type Boolean) (SweepResult :type "HitResult Structure (by ref)"))
  (bind _aspawn (cast `Pawn` OtherActor))
  (set `self.OurTarget` _aspawn)
  (bind _returnvalue (`KismetSystemLibrary.K2_SetTimerDelegate` (delegate `TrackTarget`) 0.03 true))
  (set `self.TrackingTimer` _returnvalue))

(event `self.DetectSphere.OnComponentEndOverlap`
  (params (OverlappedComponent :type "PrimitiveComponent Object Reference") (OtherActor :type "Actor Object Reference") (OtherComp :type "PrimitiveComponent Object Reference") (OtherBodyIndex :type Integer))
  (if (== OtherActor (`self.OurTarget`))
    (set `self.OurTarget` null)
    (`KismetSystemLibrary.K2_ClearAndInvalidateTimerHandle` (`self.TrackingTimer`))))

(event `self.ReceiveTick`
  (params (DeltaSeconds :type "Float (single-precision)"))
  (`parent.ReceiveTick` DeltaSeconds))

(event `PlayDeadAnim`)

(event `self.ReceiveAnyDamage`
  (params (Damage :type "Float (single-precision)") (DamageType :type "DamageType Object Reference") (InstigatedBy :type "Controller Object Reference") (DamageCauser :type "Actor Object Reference"))
  (set `self.Damage` Damage)
  (if (`self.Asleep`)
    (set `self.Damage` 0.1))
  (`parent.ReceiveAnyDamage` (`self.Damage`) DamageType InstigatedBy DamageCauser)
  (`GameplayStatics.SpawnEmitterAttached` null (`self.BloodEmissionPoint`)))

(event `self.DeathEffects`
  (`parent.DeathEffects`)
  (`KismetSystemLibrary.K2_ClearAndInvalidateTimerHandle` (`self.TrackingTimer`))
  (`KismetSystemLibrary.K2_ClearAndInvalidateTimerHandle` (`self.AttackTimer`))
  (`PrimitiveComponent.SetCollisionEnabled` (`self.AttackSphere`) "NoCollision")
  (`PrimitiveComponent.SetCollisionEnabled` (`self.DamageSphere`) "NoCollision")
  (`PrimitiveComponent.SetCollisionEnabled` (`self.JawBig`) "NoCollision")
  (`PrimitiveComponent.SetCollisionEnabled` (`self.JawSmall`) "NoCollision"))

(fn `PlayerDied`
  (`self.DeathEffects`))

(fn `UpdateLighting`
  (`KismetSystemLibrary.PrintString` "Update Lighting")
  (if (< (`/Game/IlluminationDetection/Blueprints/IlluminationComponents/BP_IlluminationProbe.ProbeIllumination` (`self.BP_IlluminationProbe`)) (`self.LightEffectTriggerValue`))
    (if (not (`self.Asleep`))
      (`self.Close`))
    (elif (`self.Asleep`)
      (`self.Open`))))

(fn `UserConstructionScript`
  (bind _returnvalue (`KismetMaterialLibrary.CreateDynamicMaterialInstance` "/Game/Environment/Plants/Carnivorous/MI_Carnivorous.MI_Carnivorous"))
  (`KismetArrayLibrary.Array_Add` (`self.Material`) _returnvalue)
  (`PrimitiveComponent.SetMaterial` (`self.JawBig`) 0 _returnvalue)
  (`PrimitiveComponent.SetMaterial` (`self.JawSmall`) 0 _returnvalue)
  (`PrimitiveComponent.SetMaterial` (`self.SM_Carnivorous_Tongue`) 0 _returnvalue))