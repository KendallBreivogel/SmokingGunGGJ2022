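; BP_Plant_LightOrb is a light orb plant that pops once when it takes any damage.
; Construction gives the mesh a dynamic M_LightOrb material, which a randomized-speed timeline drives to grow and disintegrate.
; A timeline event spawns scaled particles, disables collision, plays a size-pitched sound and subtracts LightAmount from a referenced PointLight's intensity.
; The sound's location is fed the actor's scale instead of its position.
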(event `self.ReceiveAnyDamage`
  (params (Damage :type "Float (single-precision)") (DamageType :type "DamageType Object Reference") (InstigatedBy :type "Controller Object Reference") (DamageCauser :type "Actor Object Reference"))
  (if (not (`self.Popped`))
    (set `self.Popped` true)
    (`self.Pop`)))

(event `Pop`
  (bind (_returnvalue_x _returnvalue_y _returnvalue_z) (`KismetMathLibrary.BreakVector` (`self.K2_GetActorLocation`)))
  (bind (_returnvalue_x_2 _returnvalue_y_2 _returnvalue_z_2) (`KismetMathLibrary.BreakVector` (`self.GetActorScale3D`)))
  (bind _pointlight (`self.PointLight`))
  (bind _material (`self.Material`))
  (bind _returnvalue (`KismetMathLibrary.MakeVector` _returnvalue_x_2 _returnvalue_y_2 _returnvalue_z_2))
  (bind _lightcomponent (`Light.LightComponent` _pointlight))
  (`TimelineComponent.SetPlayRate` (`self.PopAnim`) (`KismetMathLibrary.RandomFloatInRange` 1.0 5.0))
  (set `self.PopAmount` (`KismetMathLibrary.RandomFloatInRange` 2.0 5.0))
  (bind (_direction _pop _disintigrate) (`Timeline|PopAnim` :!via `PlayFromStart`)
    (:`Update`
      (`MaterialInstanceDynamic.SetScalarParameterValue` _material "Grow" (* _pop (`self.PopAmount`)))
      (`MaterialInstanceDynamic.SetScalarParameterValue` _material "Disintigration_Amount" _disintigrate))
    (:`EmitParticles`
      (`GameplayStatics.SpawnEmitterAtLocation` "/Game/Environment/Plants/LightOrb/P_LightOrb_Pop.P_LightOrb_Pop" (`KismetMathLibrary.MakeVector` _returnvalue_x _returnvalue_y (+ _returnvalue_z (* _returnvalue_x_2 25.0))) (struct) _returnvalue)
      (`PrimitiveComponent.SetCollisionEnabled` (`self.SM_LightOrb_1`) "NoCollision")
      (`GameplayStatics.PlaySoundAtLocation` "/Game/Environment/Plants/LightOrb/WAV_Pop.WAV_Pop" _returnvalue (struct) 1.0 (/ 1.0 (/ _returnvalue_x_2 2.0)) 0.0 null null null)
      (if (`KismetSystemLibrary.IsValid` _pointlight)
        (`LightComponent.SetIntensity` _lightcomponent (- (`LightComponentBase.Intensity` _lightcomponent) (`self.LightAmount`)))))))

(fn `UserConstructionScript`
  (bind _returnvalue (`KismetMaterialLibrary.CreateDynamicMaterialInstance` "/Game/Environment/Plants/LightOrb/M_LightOrb.M_LightOrb"))
  (bind _output_get (set `self.Material` _returnvalue))
  (`PrimitiveComponent.SetMaterial` (`self.SM_LightOrb_1`) 1 _output_get))