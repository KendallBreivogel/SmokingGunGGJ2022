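; Non-attacking plant actor that can be scanned and shows an indicator widget until it has been scanned.
; Shortly after BeginPlay it checks the player's MultiTool Scanned collection for its own class, hiding the ScannableUI component if found, otherwise caching the InteractableUi widget.
; ToggleScannableUI updates the scanned flag and drives the cached indicator's visibility, which stays hidden once scanned.
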(event `self.ReceiveBeginPlay`
  (`KismetSystemLibrary.Delay` 1.0)
  (`self.ConstructIndicatorUI`))

(event `/Game/Blueprints/BPI_Scannable.ToggleScannableUI`
  (params (HasBeenScanned :type Boolean))
  (bind _output_get (set `self.HasBeenScanned` HasBeenScanned))
  (`self.SetIndicatorUIVisisble` (not _output_get)))

(fn `ConstructIndicatorUI`
  (bind _scannableui (`self.ScannableUI`))
  (bind _asinteractable_ui (cast `/Game/UI/InteractableUi` (`WidgetComponent.GetUserWidgetObject` (`self.ScannableUI`))))
  (set `/Game/UI/InteractableUi.Owner` (`self.ScannableUI`) _asinteractable_ui)
  (bind _asfirst_person_character (cast `/Game/ExtraContent/FirstPersonBP/Blueprints/FirstPersonCharacter` (`GameplayStatics.GetPlayerPawn` 0)))
  (if (`KismetArrayLibrary.Array_Contains` (`/Game/Blueprints/Tools/BP_MultiTool.Scanned` (`/Game/ExtraContent/FirstPersonBP/Blueprints/FirstPersonCharacter.MultiTool` _asfirst_person_character)) (`GameplayStatics.GetObjectClass` self))
    (`SceneComponent.SetHiddenInGame` (`self.ScannableUI`) true false)
    (set `self.HasBeenScanned` true)
    (elif (not (`self.HasBeenScanned`))
      (`/Engine/EditorBlueprintResources/StandardMacros.IsValid` _scannableui
        (:`Is Valid`
          (bind _asinteractable_ui_2 (cast `/Game/UI/InteractableUi` (`WidgetComponent.GetWidget` _scannableui)))
          (set `self.IndicatorUI` _asinteractable_ui_2))))))

(fn `SetIndicatorUIVisisble`
  (params (IsVisible :type Boolean))
  (locals (visible :type Boolean))
  (bind _indicatorui (`self.IndicatorUI`))
  (set `local.visible` IsVisible)
  (if (`self.HasBeenScanned`)
    (set `local.visible` false))
  (`/Engine/EditorBlueprintResources/StandardMacros.IsValid` _indicatorui
    (:`Is Valid`
      (`Widget.SetVisibility` _indicatorui (select `bool` (`local.visible`) :`false` "Hidden" :`true` "Visible" :!type "ESlateVisibility Enum")))))

(fn `UserConstructionScript`)