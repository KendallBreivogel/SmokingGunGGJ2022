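; Illumination probe component that estimates, every tick, how lit its location is as a relative 0-1 value.
; Line traces test point/spot volumes (with distance falloff and cone checks) and directional lights; skylights count untraced, and tagged actors supply nested directional/sky components.
; It sums illumination from each light's BP_LightIlluminationProperties and optionally averages a color mix.
; Value changes fire an update dispatcher and debug display, with an OnRep notify for replication.
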(event `self.ReceiveTick`
  (params (DeltaSeconds :type "Float (single-precision)"))
  ;[1 1 1] Runs trace checks against any currently overlapped Illumination Volumes, optionally directional lights & skylights and returns an overall relative illumination value for the given probe. Stress testing revealed a 70K trace per second threshold before frame times were affected on an i5-4670K in a scene running at 150fps, normal lighting practices in conjunction with this system should provide no issue with running this function on tick.
  (`self.DetectLightVis`))

(fn `CheckForNestedDirectionalLight`
  (params (Actor :type "Actor Object Reference") (DirectionalLightComponent :type "DirectionalLightComponent Object Reference"))
  (returns (ReturnValue :type Boolean) (DirectionalLightComp :type "DirectionalLightComponent Object Reference") (FoundIllumProp :type "/Game/IlluminationDetection/Blueprints/IlluminationComponents/BP_LightIlluminationProperties Object Reference"))
  (locals (FoundReference :type Boolean) (FoundDirectionalLightComponent :type "DirectionalLightComponent Object Reference") (FoundIlluminationProperties :type "/Game/IlluminationDetection/Blueprints/IlluminationComponents/BP_LightIlluminationProperties Object Reference"))
  (for _array_element (`Actor.K2_GetComponentsByClass` Actor "/Game/IlluminationDetection/Blueprints/IlluminationComponents/BP_LightIlluminationProperties.BP_LightIlluminationProperties_C")
    (bind _directionallightcomponent (`/Game/IlluminationDetection/Blueprints/IlluminationComponents/BP_LightIlluminationProperties.DirectionalLightComponent` _array_element))
    (if (== _directionallightcomponent DirectionalLightComponent)
      (set `local.FoundDirectionalLightComponent` _directionallightcomponent)
      (set `local.FoundIlluminationProperties` _array_element)
      (set `local.FoundReference` true)
      (break)))
  (if (`local.FoundReference`)
    (return true (`local.FoundDirectionalLightComponent`) (`local.FoundIlluminationProperties`))
    (else
      (return false null null))))

(fn `CheckForNestedSkyLight`
  (params (Actor :type "Actor Object Reference") (SkyLightComponent :type "SkyLightComponent Object Reference"))
  (returns (ReturnValue :type Boolean) (FoundIllumProp :type "/Game/IlluminationDetection/Blueprints/IlluminationComponents/BP_LightIlluminationProperties Object Reference"))
  (locals (FoundReference :type Boolean) (FoundSkyLightComponent :type "SkyLightComponent Object Reference") (FoundIlluminationProperties :type "/Game/IlluminationDetection/Blueprints/IlluminationComponents/BP_LightIlluminationProperties Object Reference"))
  (for _array_element (`Actor.K2_GetComponentsByClass` Actor "/Game/IlluminationDetection/Blueprints/IlluminationComponents/BP_LightIlluminationProperties.BP_LightIlluminationProperties_C")
    (bind _skylightcomponent (`/Game/IlluminationDetection/Blueprints/IlluminationComponents/BP_LightIlluminationProperties.SkylightComponent` _array_element))
    (if (== _skylightcomponent SkyLightComponent)
      (set `local.FoundSkyLightComponent` _skylightcomponent)
      (set `local.FoundIlluminationProperties` _array_element)
      (set `local.FoundReference` true)
      (break)))
  (if (`local.FoundReference`)
    (return true (`local.FoundIlluminationProperties`))
    (else
      (return false null))))

(fn `DebugProbeInfo`
  (params (bDebugValues :type Boolean))
  ;[1 1 1] Reads off probe name, how many lights it's illuminated by, and the overall relative illumination of the given probe.
  (if bDebugValues
    (`KismetSystemLibrary.PrintString` (`KismetStringLibrary.Concat_StrStr` (`KismetSystemLibrary.GetObjectName` self) " is currently being illuminated by " (`KismetStringLibrary.Conv_IntToString` (`self.LightVisCount`)) " lights, for a relative illumination value of " (`KismetStringLibrary.Conv_DoubleToString` (`self.ProbeIllumination`)) "/1") true false (`KismetMathLibrary.SelectColor` (`self.ColorMix`) (struct :`G` 0.658824 :`B` 1.0 :`A` 1.0) (`self.CheckColorMix?`)) 0.0)
    (`KismetSystemLibrary.DrawDebugString` (`self.K2_GetComponentLocation`) (`KismetStringLibrary.Concat_StrStr` (`KismetStringLibrary.Conv_DoubleToString` (`self.ProbeIllumination`)) "/1") null (`KismetMathLibrary.SelectColor` (`self.ColorMix`) (struct :`G` 0.658824 :`B` 1.0 :`A` 1.0) (`self.CheckColorMix?`)))))

(fn `DetectLightVis`
  (locals (TempVisCount :type Integer) (TempIlluminationVal :type "Float (double-precision)") (TempColors :type "Array of LinearColor Structure"))
  (bind _returnvalue (`KismetMathLibrary.FClamp` (`local.TempIlluminationVal`)))
  ;[1 0.4745 0.1369] Initialize/Reset Temp Vals
  (set `local.TempVisCount` 0)
  (set `local.TempIlluminationVal` 0.0)
  (`KismetArrayLibrary.Array_Clear` (`local.TempColors`))
  ;[1 1 0.1] Optionally disable probe, could be used for flow control when checking illumination is/isn't necessary
  (if (`self.ProbeActive?`)
    ;[1 0.2471 0.749] Boundary Volume Probe Check
    (if (`self.CheckPoint/Spotlights?`)
      (for _array_element (`self.ArrayMV`)
        (if (`/Game/IlluminationDetection/Blueprints/IlluminationVolumes/BP_IlluminationVolumeMaster.IsSpotLight?` _array_element)
          (if (`self.IsProbeWithinConeAngle?` _array_element)
            (bind _returnvalue_2 (`/Game/IlluminationDetection/Blueprints/IlluminationVolumes/BP_IlluminationVolumeMaster.GetWorldspaceSourceLocation` _array_element))
            (bind _tracestart (`self.GetProbeTraceLocation` _returnvalue_2 :!label _label))
            (bind _outhit (`KismetSystemLibrary.LineTraceSingle` :`Start` _tracestart :`End` _returnvalue_2 :`TraceChannel` "TraceTypeQuery1" :`DrawDebugType` (`self.DebugTraceLine`) :`TraceColor` (struct :`R` 1.0 :`G` 0.247059 :`B` 0.74902 :`A` 1.0)))
            (bind (_bblockinghit _binitialoverlap _time _distance _location _impactpoint _normal _impactnormal _physmat _hitactor _hitcomponent _hitbonename _hititem _faceindex _tracestart_2 _traceend) (`GameplayStatics.BreakHitResult` _outhit))
            (if (not _bblockinghit)
              (`/Engine/EditorBlueprintResources/StandardMacros.IncrementInt` (`local.TempVisCount`)
                (:`  `
                  (bind _returnvalue_3 (* (`KismetMathLibrary.FClamp` (- 1.0 (/ (`KismetMathLibrary.VSize` (- _tracestart_2 _traceend)) (`/Game/IlluminationDetection/Blueprints/IlluminationVolumes/BP_IlluminationVolumeMaster.AttenuationDistance` _array_element)))) (`/Game/IlluminationDetection/Blueprints/IlluminationComponents/BP_LightIlluminationProperties.MaxIllumination` (`/Game/IlluminationDetection/Blueprints/IlluminationVolumes/BP_IlluminationVolumeMaster.BP_LightIlluminationProperties` _array_element))))
                  (set `local.TempIlluminationVal` (+ (`local.TempIlluminationVal`) _returnvalue_3))
                  (if (`self.CheckColorMix?`)
                    (`KismetArrayLibrary.Array_Add` (`local.TempColors`) (* (`/Game/IlluminationDetection/Blueprints/IlluminationComponents/BP_LightIlluminationProperties.LightSourceColor` (`/Game/IlluminationDetection/Blueprints/IlluminationVolumes/BP_IlluminationVolumeMaster.BP_LightIlluminationProperties` _array_element)) _returnvalue_3)))))))
          (else
            (goto _label)))))
    ;[0.2016 1 1] Directional Light Probe Check
    (if (`self.CheckDirectionalLights?`)
      (bind _outactors (`GameplayStatics.GetAllActorsOfClass` "/Script/Engine.DirectionalLight"))
      (for _array_element_2 _outactors
        (bind _lightcomponent (`Light.LightComponent` _array_element_2))
        (bind _returnvalue_4 (+ (`self.K2_GetComponentLocation` _lightcomponent) (* (`self.GetForwardVector` _lightcomponent) (* (`self.DirectionalLightTraceDistance`) -1.0))))
        (bind _tracestart_3 (`self.GetProbeTraceLocation` _returnvalue_4))
        (bind _outhit_2 (`KismetSystemLibrary.LineTraceSingle` :`Start` _tracestart_3 :`End` _returnvalue_4 :`TraceChannel` "TraceTypeQuery1" :`DrawDebugType` (`self.DebugTraceLine`) :`TraceColor` (struct :`R` 0.2 :`G` 1.0 :`B` 1.0 :`A` 1.0) :`DrawTime` 0.0))
        (bind _returnvalue_5 (`Actor.K2_GetComponentsByClass` _array_element_2 "/Game/IlluminationDetection/Blueprints/IlluminationComponents/BP_LightIlluminationProperties.BP_LightIlluminationProperties_C"))
        (if (and (not (`GameplayStatics.BreakHitResult` _outhit_2)) (> (`KismetArrayLibrary.Array_Length` _returnvalue_5) 0))
          (`/Engine/EditorBlueprintResources/StandardMacros.IncrementInt` (`local.TempVisCount`)
            (:`  `
              (bind _output (`|GetArrayItem` _returnvalue_5))
              (bind _maxillumination (`/Game/IlluminationDetection/Blueprints/IlluminationComponents/BP_LightIlluminationProperties.MaxIllumination` _output))
              (set `local.TempIlluminationVal` (+ (`local.TempIlluminationVal`) _maxillumination))
              (if (`self.CheckColorMix?`)
                (`KismetArrayLibrary.Array_Add` (`local.TempColors`) (* (`/Game/IlluminationDetection/Blueprints/IlluminationComponents/BP_LightIlluminationProperties.LightSourceColor` _output) _maxillumination))))))))
    ;[0.0317 0.1963 1] Skylight Probe Check
    (if (`self.CheckSkyLights?`)
      (bind _outactors_2 (`GameplayStatics.GetAllActorsOfClass` "/Script/Engine.SkyLight"))
      (for _array_element_3 _outactors_2
        (`/Engine/EditorBlueprintResources/StandardMacros.IncrementInt` (`local.TempVisCount`)
          (:`  `
            (bind _returnvalue_6 (`Actor.K2_GetComponentsByClass` _array_element_3 "/Game/IlluminationDetection/Blueprints/IlluminationComponents/BP_LightIlluminationProperties.BP_LightIlluminationProperties_C"))
            (if (> (`KismetArrayLibrary.Array_Length` _returnvalue_6) 0)
              (bind _output_2 (`|GetArrayItem` _returnvalue_6))
              (bind _maxillumination_2 (`/Game/IlluminationDetection/Blueprints/IlluminationComponents/BP_LightIlluminationProperties.MaxIllumination` _output_2))
              (set `local.TempIlluminationVal` (+ (`local.TempIlluminationVal`) _maxillumination_2))
              (if (`self.CheckColorMix?`)
                (`KismetArrayLibrary.Array_Add` (`local.TempColors`) (* (`/Game/IlluminationDetection/Blueprints/IlluminationComponents/BP_LightIlluminationProperties.LightSourceColor` _output_2) _maxillumination_2))))))))
    ;[0.5847 0.2889 1] Nested Directional Light Component Check
    (if (`self.CheckDirectionalLightComponentsNestedInActors?`)
      (bind _outactors_3 (`GameplayStatics.GetAllActorsWithTag` (`self.CustomLightActorTag`)))
      (for _array_element_4 _outactors_3
        (bind _returnvalue_7 (`Actor.K2_GetComponentsByClass` _array_element_4 "/Script/Engine.DirectionalLightComponent"))
        (if (and (> (`KismetArrayLibrary.Array_Length` _returnvalue_7) 0) (> (`KismetArrayLibrary.Array_Length` (`Actor.K2_GetComponentsByClass` _array_element_4 "/Game/IlluminationDetection/Blueprints/IlluminationComponents/BP_LightIlluminationProperties.BP_LightIlluminationProperties_C")) 0))
          (for _array_element_5 _returnvalue_7
            (bind (_returnvalue_8 _directionallightcomp _foundillumprop) (`self.CheckForNestedDirectionalLight` _array_element_4 _array_element_5))
            (if _returnvalue_8
              (bind _returnvalue_9 (+ (`self.K2_GetComponentLocation` _directionallightcomp) (* (`self.GetForwardVector` _directionallightcomp) (* (`self.DirectionalLightTraceDistance`) -1.0))))
              (bind _tracestart_4 (`self.GetProbeTraceLocation` _returnvalue_9))
              (bind _outhit_3 (`KismetSystemLibrary.LineTraceSingle` :`Start` _tracestart_4 :`End` _returnvalue_9 :`TraceChannel` "TraceTypeQuery1" :`DrawDebugType` (`self.DebugTraceLine`) :`TraceColor` (struct :`R` 0.2 :`G` 1.0 :`B` 1.0 :`A` 1.0) :`DrawTime` 0.0))
              (if (not (`GameplayStatics.BreakHitResult` _outhit_3))
                (`/Engine/EditorBlueprintResources/StandardMacros.IncrementInt` (`local.TempVisCount`)
                  (:`  `
                    (bind _maxillumination_3 (`/Game/IlluminationDetection/Blueprints/IlluminationComponents/BP_LightIlluminationProperties.MaxIllumination` _foundillumprop))
                    (set `local.TempIlluminationVal` (+ (`local.TempIlluminationVal`) _maxillumination_3))
                    (if (`self.CheckColorMix?`)
                      (`KismetArrayLibrary.Array_Add` (`local.TempColors`) (* (`/Game/IlluminationDetection/Blueprints/IlluminationComponents/BP_LightIlluminationProperties.LightSourceColor` _foundillumprop) _maxillumination_3)))))))))))
    ;[0.2384 1 0.4922] Nested Sky Light Component Check
    (if (`self.CheckSkyLightComponentsNestedInActors?`)
      (bind _outactors_4 (`GameplayStatics.GetAllActorsWithTag` (`self.CustomLightActorTag`)))
      (for _array_element_6 _outactors_4
        (bind _returnvalue_10 (`Actor.K2_GetComponentsByClass` _array_element_6 "/Script/Engine.SkyLightComponent"))
        (if (and (> (`KismetArrayLibrary.Array_Length` _returnvalue_10) 0) (> (`KismetArrayLibrary.Array_Length` (`Actor.K2_GetComponentsByClass` _array_element_6 "/Game/IlluminationDetection/Blueprints/IlluminationComponents/BP_LightIlluminationProperties.BP_LightIlluminationProperties_C")) 0))
          (for _array_element_7 _returnvalue_10
            (bind (_returnvalue_11 _foundillumprop_2) (`self.CheckForNestedSkyLight` _array_element_6 _array_element_7))
            (if _returnvalue_11
              (`/Engine/EditorBlueprintResources/StandardMacros.IncrementInt` (`local.TempVisCount`)
                (:`  `
                  (bind _maxillumination_4 (`/Game/IlluminationDetection/Blueprints/IlluminationComponents/BP_LightIlluminationProperties.MaxIllumination` _foundillumprop_2))
                  (set `local.TempIlluminationVal` (+ (`local.TempIlluminationVal`) _maxillumination_4))
                  (if (`self.CheckColorMix?`)
                    (`KismetArrayLibrary.Array_Add` (`local.TempColors`) (* (`/Game/IlluminationDetection/Blueprints/IlluminationComponents/BP_LightIlluminationProperties.LightSourceColor` _foundillumprop_2) _maxillumination_4))))))))))
    ;[0.5636 1 0.1869] Account Stats & Call Update Dispatcher
    (set `self.LightVisCount` (`local.TempVisCount`))
    (if (!= _returnvalue (`self.ProbeIllumination`))
      (set `self.ProbeIllumination` _returnvalue)
      (if (> (`KismetArrayLibrary.Array_Length` (`local.TempColors`)) 0)
        (`self.DetermineColorMixAtTraceHitPoint` (`local.TempColors`)))
      (if (not (`|EnumEquality` (`self.DebugTraceLine`)))
        (`KismetSystemLibrary.DrawDebugSphere` (`self.K2_GetComponentLocation`) (`self.ProbeRadius`) 12 (`KismetMathLibrary.LinearColorLerp` (struct) (`KismetMathLibrary.SelectColor` (`self.ColorMix`) (struct :`R` 1.0 :`G` 1.0 :`B` 0.247059 :`A` 1.0) (`self.CheckColorMix?`)) (`self.ProbeIllumination`)) 0.0 0.25))
      (`self.DebugProbeInfo` (`self.DebugProbeStats`))
      (`self.UpdateLightRangeStatus`)
      (return))
    (else
      (return))))

(fn `DetermineColorMixAtTraceHitPoint`
  (params (ColorArrayIn :type "Array of LinearColor Structure"))
  (returns (OutputColor :type "LinearColor Structure"))
  (locals (TempR :type "Float (double-precision)") (TempG :type "Float (double-precision)") (TempB :type "Float (double-precision)") (IllumArray :type "Array of Float (double-precision)") (ColorArray :type "Array of LinearColor Structure"))
  (bind _returnvalue (`KismetMathLibrary.Conv_IntToDouble` (`KismetArrayLibrary.Array_Length` (`local.ColorArray`))))
  ;[1 1 1] RestTempValues
  (set `local.ColorArray` ColorArrayIn)
  (set `local.TempR` 0.0)
  (set `local.TempG` 0.0)
  (set `local.TempB` 0.0)
  ;[1 1 1] Get total RGB
  (for _array_element (`local.ColorArray`)
    (bind (_r _g _b) (break `LinearColor` _array_element))
    (set `local.TempR` (+ _r (`local.TempR`)))
    (set `local.TempG` (+ _g (`local.TempG`)))
    (set `local.TempB` (+ _b (`local.TempB`))))
  ;[1 1 1] Sample RGB/number of colors sampled
  (set `local.TempR` (`KismetMathLibrary.FClamp` (/ (`local.TempR`) _returnvalue)))
  (set `local.TempG` (`KismetMathLibrary.FClamp` (/ (`local.TempG`) _returnvalue)))
  (set `local.TempB` (`KismetMathLibrary.FClamp` (/ (`local.TempB`) _returnvalue)))
  ;[1 1 1] Store result to ColorMix
  (bind _output_get (set `self.ColorMix` (make `LinearColor` (`local.TempR`) (`local.TempG`) (`local.TempB`) 1.0)))
  (return _output_get))

(fn `GetProbeTraceLocation`
  (params (TraceEndLocatoin :type "Vector Structure"))
  (returns (TraceStart :type "Vector Structure"))
  (bind _returnvalue (`self.K2_GetComponentLocation`))
  ;[1 1 1] Assigns probe trace start location based on ProbeRadius value
  (if (> (`self.ProbeRadius`) 0.0)
    (return (+ _returnvalue (* (`KismetMathLibrary.Conv_RotatorToVector` (`KismetMathLibrary.FindLookAtRotation` _returnvalue TraceEndLocatoin)) (`self.ProbeRadius`))))
    (else
      (return _returnvalue))))

(fn `IsProbeWithinConeAngle?`
  (params (IlluminationSphereRef :type "/Game/IlluminationDetection/Blueprints/IlluminationVolumes/BP_IlluminationVolumeMaster Object Reference"))
  (returns (ReturnValue :type Boolean))
  (bind _sl_ref (`/Game/IlluminationDetection/Blueprints/IlluminationVolumes/BP_IlluminationVolumeMaster.SL_Ref` IlluminationSphereRef))
  ;[1 1 1] Gets forward vector from look-at rotation from the overlap bounds source location to the probe location, compares the dot product of it and the overlap bounds forward vector against a 0-1 scaled cone angle (between 0 and 180 degrees) to determine if probe is within the spotlight's outer cone angle, & thus able to be illuminated.
  (return (>= (`KismetMathLibrary.Dot_VectorVector` (`self.GetForwardVector` _sl_ref) (`KismetMathLibrary.Conv_RotatorToVector` (`KismetMathLibrary.FindLookAtRotation` (`self.K2_GetComponentLocation` _sl_ref) (`self.K2_GetComponentLocation`)))) (- 1.0 (/ (`SpotLightComponent.OuterConeAngle` _sl_ref) 180.0)))))

(fn `OnRep_ProbeIllumination`
  (`self.ProbeIlluminationUpdated`))