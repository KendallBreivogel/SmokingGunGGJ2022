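; Manager actor that controls the background ambiance on two referenced sound actors, Ambiance1 and Ambiance2.
; On BeginPlay it reads the first-person character's current zone and assigns the desert or cave sound to both audio components.
; The NewAmbiance event changes the sound at runtime by fading both out, waiting for the fade, swapping in the given sound and fading back in.
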(event `self.ReceiveBeginPlay`
  (bind _audiocomponent (`AmbientSound.AudioComponent` (`self.Ambiance_1`)))
  (bind _asfirst_person_character (cast `/Game/ExtraContent/FirstPersonBP/Blueprints/FirstPersonCharacter` (`GameplayStatics.GetPlayerPawn` 0)))
  (switch `string` (`/Game/ExtraContent/FirstPersonBP/Blueprints/FirstPersonCharacter.CurrentZone` _asfirst_person_character)
    (:`Desert`
      (`AudioComponent.SetSound` _audiocomponent "/Game/Audio/WAV_Ambiance_Desert.WAV_Ambiance_Desert")
      (`AudioComponent.SetSound` (`AmbientSound.AudioComponent` (`self.Ambiance_2`)) "/Game/Audio/WAV_Ambiance_Desert.WAV_Ambiance_Desert"))
    (:`Cave_1`
      (`AudioComponent.SetSound` _audiocomponent "/Game/Audio/WAV_Ambiance_Cave.WAV_Ambiance_Cave")
      (`AudioComponent.SetSound` (`AmbientSound.AudioComponent` (`self.Ambiance_2`)) "/Game/Audio/WAV_Ambiance_Cave.WAV_Ambiance_Cave"))))

(event `NewAmbiance`
  (params (Ambiance :type "SoundWave Object Reference"))
  (bind _audiocomponent (`AmbientSound.AudioComponent` (`self.Ambiance_1`)))
  (`AudioComponent.FadeOut` _audiocomponent 1.0 0.0 "Linear")
  (`AudioComponent.FadeOut` (`AmbientSound.AudioComponent` (`self.Ambiance_2`)) 1.0 0.0 "Linear")
  (`KismetSystemLibrary.Delay` 1.0)
  (`AudioComponent.SetSound` _audiocomponent Ambiance)
  (`AudioComponent.SetSound` (`AmbientSound.AudioComponent` (`self.Ambiance_2`)) Ambiance)
  (`AudioComponent.FadeIn` _audiocomponent 1.0 1.0 0.0 "Linear")
  (`AudioComponent.FadeIn` (`AmbientSound.AudioComponent` (`self.Ambiance_2`)) 1.0 1.0 0.0 "Linear"))

(fn `UserConstructionScript`)