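; BP_SwimVolume is an underwater trigger volume that manages audio and breath for the FirstPersonCharacter while it is inside the Box.
; Entering plays a dive sound, fades in underwater ambience, pushes a sound mix and starts a looping timer that drains Breath.
; Once Breath hits zero, each timer tick applies damage.
; Exiting plays a surface sound, reverses the audio changes, refills Breath and clears the timer.
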(event `self.Box.OnComponentBeginOverlap`
  (params (OverlappedComponent :type "PrimitiveComponent Object Reference") (OtherActor :type "Actor Object Reference") (OtherComp :type "PrimitiveComponent Object Reference") (OtherBodyIndex :type Integer) (bFromSweep :type Boolean) (SweepResult :type "HitResult Structure (by ref)"))
  (bind _asfirst_person_character (cast `/Game/ExtraContent/FirstPersonBP/Blueprints/FirstPersonCharacter` OtherActor))
  (set `self.Character` _asfirst_person_character)
  (`GameplayStatics.PlaySound2D` "/Game/Blueprints/Character/Audio/WAV_Dive.WAV_Dive" 1.0 1.0 0.0 null null)
  (`AudioComponent.FadeIn` (`self.WAV_Ambiance_Underwater`) 1.0 1.0 0.0 "Linear")
  (bind _returnvalue (`KismetSystemLibrary.K2_SetTimerDelegate` (delegate `DepleteBreath`) 0.03 true))
  (set `self.Timer` _returnvalue)
  (`GameplayStatics.PushSoundMixModifier` "/Game/Audio/Mixes/Underwater.Underwater"))

(event `self.Box.OnComponentEndOverlap`
  (params (OverlappedComponent :type "PrimitiveComponent Object Reference") (OtherActor :type "Actor Object Reference") (OtherComp :type "PrimitiveComponent Object Reference") (OtherBodyIndex :type Integer))
  (cast `/Game/ExtraContent/FirstPersonBP/Blueprints/FirstPersonCharacter` OtherActor)
  (`GameplayStatics.PlaySound2D` "/Game/Blueprints/Character/Audio/WAV_Surface.WAV_Surface" 1.0 1.0 0.0 null null)
  (`AudioComponent.FadeOut` (`self.WAV_Ambiance_Underwater`) 0.5 0.0 "Linear")
  (set `/Game/ExtraContent/FirstPersonBP/Blueprints/FirstPersonCharacter.Breath` 1.0 (`self.Character`))
  (`KismetSystemLibrary.K2_ClearAndInvalidateTimerHandle` (`self.Timer`))
  (`GameplayStatics.PopSoundMixModifier` "/Game/Audio/Mixes/Underwater.Underwater"))

(event `DepleteBreath`
  (bind _character (`self.Character`))
  (bind _output_get (set `/Game/ExtraContent/FirstPersonBP/Blueprints/FirstPersonCharacter.Breath` (`KismetMathLibrary.FClamp` (- (`/Game/ExtraContent/FirstPersonBP/Blueprints/FirstPersonCharacter.Breath` _character) 0.001)) _character))
  (if (== _output_get 0.0)
    (`GameplayStatics.ApplyDamage` (`self.Character`) 1.0)))

(fn `UserConstructionScript`)