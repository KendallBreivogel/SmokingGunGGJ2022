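; BP_SaveLoadManager is a level actor that restores the player's progress from the "Autosave" save slot.
; BeginPlay caches the level's single MusicMangerBP reference.
; LoadAutosave reads a SaveSlot1 object, sets the current room number, moves the first-person character to the saved spawn location and restores the MultiTool's modes, canisters and scanned data.
; It then switches the music and returns whether a save was found.
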(event `self.ReceiveBeginPlay`
  ;[1 1 1 1 12] Gets and stores a reference to the MusicMangerBP. There should only be 1 MusicMangerBP per level so it will be index 0.
  (bind _outactors (`GameplayStatics.GetAllActorsOfClass` "/Game/Audio/Music/MusicChanging/MusicMangerBP.MusicMangerBP_C"))
  (set `self.MusicMangerRef` (`|GetArrayItem` _outactors)))

(fn `LoadAutosave`
  (returns (Success :type Boolean))
  (bind _returnvalue (`GameplayStatics.LoadGameFromSlot` "Autosave"))
  (if (`KismetSystemLibrary.IsValid` _returnvalue)
    (bind _assave_slot_1 (cast `/Game/Blueprints/SaveSlot1` _returnvalue))
    (set `self.CurrentRoomNum` (`/Game/Blueprints/SaveSlot1.RoomNum` _assave_slot_1))
    (bind _asfirst_person_character (cast `/Game/ExtraContent/FirstPersonBP/Blueprints/FirstPersonCharacter` (`GameplayStatics.GetPlayerPawn` 0)))
    (`self.K2_SetActorLocation` _asfirst_person_character (`/Game/Blueprints/SaveSlot1.SpawnLocation` _assave_slot_1) false false)
    (bind _multitool (`/Game/ExtraContent/FirstPersonBP/Blueprints/FirstPersonCharacter.MultiTool` _asfirst_person_character))
    (set `/Game/Blueprints/Tools/BP_MultiTool.AvailableModes` (`/Game/Blueprints/SaveSlot1.CollectedTools` _assave_slot_1) _multitool)
    (`/Game/Blueprints/Tools/BP_MultiTool.InitCannisters` _multitool)
    (set `/Game/Blueprints/Tools/BP_MultiTool.Scanned` (`/Game/Blueprints/SaveSlot1.Scanned` _assave_slot_1) _multitool)
    (`/Game/Audio/Music/MusicChanging/MusicMangerBP.Change Music From To` (`self.MusicMangerRef`) 2)
    (return true)
    (else
      (return false))))

(fn `UserConstructionScript`)