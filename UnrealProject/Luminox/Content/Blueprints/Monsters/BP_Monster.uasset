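; Base AI monster that wakes via its Blackboard, pounces along a timeline arc and damages listed enemy pawn classes, with cooldowns on both attacks.
; Damage drains health and updates a widget bar shown when hurt and in line of sight; death plays a material disintegration.
; A scan indicator follows the player's MultiTool scan record.
; A timer displays detected light level, but the light-weakness multiplier currently always evaluates to zero.
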(event `self.ReceiveBeginPlay`
  (bind _asfirst_person_character (cast `/Game/ExtraContent/FirstPersonBP/Blueprints/FirstPersonCharacter` (`GameplayStatics.GetPlayerCharacter` 0)))
  (set `self.Player` _asfirst_person_character)
  (`self.ConstructHealthUI`)
  (`KismetSystemLibrary.Delay` 1.0)
  (`self.ConstructIndicatorUI`)
  (bind _returnvalue (`KismetSystemLibrary.K2_SetTimer` self "UpdateLighting" (`self.UpdateLightTime`) true))
  (set `self.UpdateLightTimer` _returnvalue)
  (if (`self.StartActive`)
    (`self.WakeUp`)))

(event `self.ReceiveTick`
  (params (DeltaSeconds :type "Float (single-precision)"))
  (`self.CheckVisibility`)
  (`self.SetWeaknessScalar`))

(event `self.ReceiveAnyDamage`
  (params (Damage :type "Float (single-precision)") (DamageType :type "DamageType Object Reference") (InstigatedBy :type "Controller Object Reference") (DamageCauser :type "Actor Object Reference"))
  (bind _heathui (`self.HeathUI`))
  (if (not (`self.Dead`))
    (`KismetSystemLibrary.PrintString` (`KismetStringLibrary.Concat_StrStr` (`KismetSystemLibrary.GetDisplayName` self) ": Was Damaged"))
    (bind _output_get (set `self.Health` (- (`self.Health`) (* (+ (`self.WeaknessScalar`) 1.0) Damage))))
    (`/Engine/EditorBlueprintResources/StandardMacros.IsValid` _heathui
      (:`Is Valid`
        (`/Game/UI/MonsterHealth.SetHealth` _heathui (/ _output_get 100.0)))
      (:`Is Not Valid`
        _))
    (`KismetSystemLibrary.PrintString` (`KismetStringLibrary.Concat_StrStr` "Health: " (`KismetStringLibrary.Conv_DoubleToString` _output_get)))
    (if (<= (`self.Health`) 0.0)
      (set `self.Dead` true)
      (`self.PlayerDied`))))

(event `self.ReceiveDestroyed`
  (`KismetSystemLibrary.PrintString` "Destroyed"))

(event `DeathEffects`
  (bind (_direction _amount) (`Timeline|Distintigration` :!via `PlayFromStart`)
    (:`Update`
      (for _array_element (`self.Material`)
        (`MaterialInstanceDynamic.SetScalarParameterValue` _array_element "Disintigration_Amount" _amount)))
    (:`Finished`
      (`self.DeathCleanup`))))

(event `DeathCleanup`)

(event `WakeUp`
  (bind _returnvalue (`AIBlueprintHelperLibrary.GetBlackboard` (`AIBlueprintHelperLibrary.GetAIController` self)))
  (set `self.State` "NewEnumerator6")
  (`KismetSystemLibrary.Delay` (`self.TimeToWake`))
  (set `self.State` "NewEnumerator0")
  (if (`KismetSystemLibrary.IsValid` _returnvalue)
    (`BlackboardComponent.SetValueAsBool` _returnvalue "Awake" true)
    (`BlackboardComponent.SetValueAsBool` _returnvalue "AnimationInterrupt" false)
    (set `CharacterMovementComponent.GravityScale` 1.0 (`self.CharacterMovement`))
    (`KismetSystemLibrary.PrintString` (`KismetStringLibrary.Concat_StrStr` (`KismetSystemLibrary.GetDisplayName` self) " is Awake") true true (struct :`G` 0.66 :`B` 1.0 :`A` 1.0) 10.0)))

(event `Pounce`
  (params (Location :type "Vector Structure"))
  (bind _returnvalue (`AIBlueprintHelperLibrary.GetAIController` self))
  (`KismetSystemLibrary.PrintString` "POUNCE!" true true (struct :`G` 0.66 :`B` 1.0 :`A` 1.0) 20.0)
  (set `self.State` "NewEnumerator4")
  (set `self.pounceStartLocation` (`self.K2_GetActorLocation`))
  (set `self.canPounce` false)
  (`Controller.StopMovement` _returnvalue)
  (bind (_direction _movement _height) (`Timeline|PounceAnim` :!via `PlayFromStart`)
    (:`Update`
      (`self.K2_SetActorLocation` (+ (`KismetMathLibrary.VLerp` (`self.pounceStartLocation`) Location _movement) (`KismetMathLibrary.MakeVector` 0.0 0.0 (* _height 100.0)))))
    (:`Finished`
      (`BlackboardComponent.SetValueAsBool` (`AIBlueprintHelperLibrary.GetBlackboard` _returnvalue) "Pouncing" false)
      (`KismetSystemLibrary.K2_SetTimerDelegate` (delegate `ResetCanPounce`) (`self.pounceCoolDown`))
      (set `self.State` "NewEnumerator1"))))

(event `ResetCanPounce`
  (set `self.canPounce` true))

(event `DamageActor`
  (params (Actor :type "Actor Object Reference"))
  (if (`self.CanDamage`)
    (bind _aspawn (cast `Pawn` Actor))
    (if (`KismetArrayLibrary.Array_Contains` (`self.EnemyTypes`) (`GameplayStatics.GetObjectClass` _aspawn))
      (`GameplayStatics.ApplyDamage` _aspawn (`self.Damage`) (`AIBlueprintHelperLibrary.GetAIController` self) self)
      (set `self.CanDamage` false)
      (`KismetSystemLibrary.K2_SetTimerDelegate` (delegate `ResetCanDamage`) (`self.DamageCooldown`)))))

(event `ResetCanDamage`
  (set `self.CanDamage` true))

(event `/Game/Blueprints/BPI_Scannable.ToggleScannableUI`
  (params (HasBeenScanned :type Boolean))
  (bind _output_get (set `self.HasBeenScanned` HasBeenScanned))
  (`self.SetIndicatorUIVisisble` (not _output_get))
  (`KismetArrayLibrary.Array_Add` (`self.Tags`) "Scanned"))

(fn `CheckVisibility`
  (bind _outhit (`KismetSystemLibrary.LineTraceSingle` (`self.K2_GetActorLocation`) (`self.K2_GetActorLocation` (`GameplayStatics.GetPlayerPawn` 0)) "TraceTypeQuery2"))
  (`self.SetHealthUIVisible` (== (`.HitActor` (`GameplayStatics.BreakHitResult` _outhit)) (`GameplayStatics.GetPlayerPawn` 0))))

(fn `ConstructHealthUI`
  (bind _healthbar (`self.HealthBar`))
  (if (`self.CanBeHurt`)
    (`/Engine/EditorBlueprintResources/StandardMacros.IsValid` _healthbar
      (:`Is Valid`
        (bind _asmonster_health (cast `/Game/UI/MonsterHealth` (`WidgetComponent.GetWidget` _healthbar)))
        (set `self.HeathUI` _asmonster_health)))
    (else
      (`ActorComponent.K2_DestroyComponent` (`self.HealthBar`)))))

(fn `ConstructIndicatorUI`
  (bind _interactindicator (`self.InteractIndicator`))
  (bind _asinteractable_ui (cast `/Game/UI/InteractableUi` (`WidgetComponent.GetUserWidgetObject` (`self.InteractIndicator`))))
  (set `/Game/UI/InteractableUi.Owner` (`self.InteractIndicator`) _asinteractable_ui)
  (bind _asfirst_person_character (cast `/Game/ExtraContent/FirstPersonBP/Blueprints/FirstPersonCharacter` (`GameplayStatics.GetPlayerPawn` 0)))
  (if (`KismetArrayLibrary.Array_Contains` (`/Game/Blueprints/Tools/BP_MultiTool.Scanned` (`/Game/ExtraContent/FirstPersonBP/Blueprints/FirstPersonCharacter.MultiTool` _asfirst_person_character)) (`GameplayStatics.GetObjectClass` self))
    (`SceneComponent.SetHiddenInGame` (`self.InteractIndicator`) true false)
    (set `self.HasBeenScanned` true)
    (`KismetArrayLibrary.Array_Add` (`self.Tags`) "Scanned")
    (elif (not (`self.HasBeenScanned`))
      (`/Engine/EditorBlueprintResources/StandardMacros.IsValid` _interactindicator
        (:`Is Valid`
          (bind _asinteractable_ui_2 (cast `/Game/UI/InteractableUi` (`WidgetComponent.GetWidget` _interactindicator)))
          (set `self.IndicatorUI` _asinteractable_ui_2)
          (bind _asfirst_person_character_2 (cast `/Game/ExtraContent/FirstPersonBP/Blueprints/FirstPersonCharacter` (`GameplayStatics.GetPlayerPawn` 0)))
          (bind _hud (`/Game/ExtraContent/FirstPersonBP/Blueprints/FirstPersonCharacter.HUD` _asfirst_person_character_2))
          (if (`Widget.IsVisible` _hud)
            (`/Game/UI/Menu.SetScanIndicatorVisibility` _hud true)))))))

(fn `PlayerDied`
  (`KismetSystemLibrary.K2_ClearAndInvalidateTimerHandle` (`self.UpdateLightTimer`))
  (`self.DeathEffects`)
  (`/Engine/EditorBlueprintResources/StandardMacros.IsValid` (`self.HealthBar`)
    (:`Is Valid`
      (`self.SetHealthUIVisible` false))))

(fn `PlayerRecievesDamage`)

(fn `SetHealthUIVisible`
  (params (bNewVisibility :type Boolean))
  (locals (IsVisible :type Boolean))
  (bind _heathui (`self.HeathUI`))
  (set `local.IsVisible` bNewVisibility)
  (if (== (`self.Health`) 100.0)
    (set `local.IsVisible` false))
  (`/Engine/EditorBlueprintResources/StandardMacros.IsValid` _heathui
    (:`Is Valid`
      (`Widget.SetVisibility` _heathui (select `bool` (`local.IsVisible`) :`false` "Hidden" :`true` "Visible" :!type "ESlateVisibility Enum")))))

(fn `SetIndicatorUIVisisble`
  (params (IsVisible :type Boolean))
  (locals (visible :type Boolean))
  (bind _indicatorui (`self.IndicatorUI`))
  (set `local.visible` IsVisible)
  (if (`self.HasBeenScanned`)
    (set `local.visible` false))
  (`/Engine/EditorBlueprintResources/StandardMacros.IsValid` _indicatorui
    (:`Is Valid`
      (`Widget.SetVisibility` _indicatorui (select `bool` (`local.visible`) :`false` "Hidden" :`true` "Visible" :!type "ESlateVisibility Enum")))))

(fn `SetWeaknessScalar`
  (if (`self.bIsLightSensitive`)
    (set `self.WeaknessScalar` 0.0)
    (else
      (set `self.WeaknessScalar` (- 1.0 1.0)))))

(fn `UpdateLighting`
  (bind _lightlevel (`/Game/Blueprints/LightDetection/SceneComp_LightDetector.GetTotalLightLevel` (`self.SceneComp_LightDetector`)))
  (`TextRenderComponent.K2_SetText` (`self.TextRender`) (`KismetTextLibrary.Conv_DoubleToText` _lightlevel "HalfToEven")))

(fn `UpdateSpeed`
  (params (NewSpeed :type "Float (double-precision)"))
  (set `CharacterMovementComponent.MaxWalkSpeed` NewSpeed (`self.CharacterMovement`)))

(fn `UserConstructionScript`
  (`SceneComponent.SetHiddenInGame` (`self.TextRender`) (not (`self.ShowLightAmount`)) false))