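; Lizard monster child Blueprint that wakes when lit, pounces, and damages enemy pawns overlapping its sphere.
; Waking restores gravity and levels roll and pitch via a timeline; pounces temporarily double the sphere's radius.
; Light above a threshold sets the Blackboard flee flag and disables sphere collision.
; An integer parameter switches Lizard audio per behavior, walk animation rate follows speed and scale, and construction creates dynamic body and eye materials.
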(event `self.ReceiveBeginPlay`
  (`parent.ReceiveBeginPlay`))

(event `self.ReceiveTick`
  (params (DeltaSeconds :type "Float (single-precision)"))
  (`parent.ReceiveTick` DeltaSeconds))

(event `self.DeathEffects`
  (bind _lizard (`self.lizard`))
  (`parent.DeathEffects`)
  (`AudioComponent.SetIntParameter` _lizard "lizard_switch" 3)
  (`AudioComponent.FadeIn` _lizard 0.1 1.0 0.0 "Linear"))

(event `self.DeathCleanup`
  (`self.K2_DestroyActor`))

(event `self.Pounce`
  (params (Location :type "Vector Structure"))
  (bind _sphere (`self.Sphere`))
  (bind _lizard (`self.lizard`))
  (bind _sphere_2 (`self.Sphere`))
  (`parent.Pounce` Location)
  (`SphereComponent.SetSphereRadius` _sphere_2 (* (`SphereComponent.SphereRadius` _sphere_2) 2.0) true)
  (`AudioComponent.SetIntParameter` _lizard "lizard_switch" 2)
  (`AudioComponent.FadeIn` _lizard 0.1 1.0 0.0 "Linear")
  (`KismetSystemLibrary.Delay` 1.0)
  (`AudioComponent.SetIntParameter` _lizard "lizard_switch" 1)
  (`AudioComponent.FadeIn` _lizard 0.1 1.0 0.0 "Linear")
  (`SphereComponent.SetSphereRadius` _sphere (* (`SphereComponent.SphereRadius` _sphere) 0.5) true))

(event `self.WakeUp`
  (bind (_returnvalue_roll _returnvalue_pitch _returnvalue_yaw) (`KismetMathLibrary.BreakRotator` (`self.K2_GetActorRotation`)))
  (bind _lizard (`self.lizard`))
  (bind _lizard_2 (`self.lizard`))
  (`parent.WakeUp`)
  (`KismetSystemLibrary.Delay` 2.0)
  (`AudioComponent.SetIntParameter` _lizard "lizard_switch" 0)
  (`AudioComponent.FadeIn` _lizard 0.1 1.0 0.0 "Linear")
  (set `CharacterMovementComponent.GravityScale` 1.0 (`self.CharacterMovement`))
  (bind (_direction _alpha) (`Timeline|CorrectRotation` :!via `PlayFromStart`)
    (:`Update`
      (`self.K2_SetActorRotation` (`KismetMathLibrary.MakeRotator` (`KismetMathLibrary.Lerp` _returnvalue_roll 0.0 _alpha) (`KismetMathLibrary.Lerp` _returnvalue_pitch 0.0 _alpha) _returnvalue_yaw))
      (`AudioComponent.SetIntParameter` _lizard_2 "lizard_switch" 1)
      (`AudioComponent.FadeIn` _lizard_2 0.1 1.0 0.0 "Linear"))))

(event `self.Sphere.OnComponentBeginOverlap`
  (params (OverlappedComponent :type "PrimitiveComponent Object Reference") (OtherActor :type "Actor Object Reference") (OtherComp :type "PrimitiveComponent Object Reference") (OtherBodyIndex :type Integer) (bFromSweep :type Boolean) (SweepResult :type "HitResult Structure (by ref)"))
  (bind _aspawn (cast `Pawn` OtherActor))
  (if (`KismetArrayLibrary.Array_Contains` (`self.EnemyTypes`) (`GameplayStatics.GetObjectClass` _aspawn))
    (`self.DamageActor` OtherActor)))

(fn `UpdateLighting`
  (bind _state (`self.State`))
  (bind _lightlevel (`/Game/Blueprints/LightDetection/SceneComp_LightDetector.LightLevel` (`self.SceneComp_LightDetector`)))
  (bind _returnvalue (> _lightlevel (`self.LightEffectTriggerValue`)))
  (`parent.UpdateLighting`)
  (if (and (> _lightlevel 0.0) (`|EnumEquality` _state "NewEnumerator5"))
    (`self.WakeUp`)
    (elif (not (`|EnumEquality` _state "NewEnumerator6"))
      (`BlackboardComponent.SetValueAsBool` (`AIBlueprintHelperLibrary.GetBlackboard` (`AIBlueprintHelperLibrary.GetAIController` self)) "IsFleeing" _returnvalue)
      (`PrimitiveComponent.SetCollisionEnabled` (`self.Sphere`) (select `bool` _returnvalue :`false` "QueryOnly" :`true` "NoCollision" :!type "ECollisionEnabled Enum")))))

(fn `UpdateSpeed`
  (params (NewSpeed :type "Float (double-precision)"))
  (bind _returnvalue_x (`KismetMathLibrary.BreakVector` (`self.GetActorScale3D`)))
  (`parent.UpdateSpeed` NewSpeed)
  (set `self.WalkAnimSpeed` (/ (/ NewSpeed 78.0) _returnvalue_x)))

(fn `UserConstructionScript`
  (bind _returnvalue (`KismetMaterialLibrary.CreateDynamicMaterialInstance` "/Game/Blueprints/Monsters/LizardMonster/Mesh/MI_lizardMonster.MI_LizardMonster"))
  (`KismetArrayLibrary.Array_Add` (`self.Material`) _returnvalue)
  (`PrimitiveComponent.SetMaterial` (`self.Mesh`) 1 _returnvalue)
  (bind _returnvalue_2 (`KismetMaterialLibrary.CreateDynamicMaterialInstance` "/Game/Blueprints/Monsters/LizardMonster/Mesh/M_Eyes.M_Eyes"))
  (`KismetArrayLibrary.Array_Add` (`self.Material`) _returnvalue_2)
  (`PrimitiveComponent.SetMaterial` (`self.Mesh`) 0 _returnvalue_2))