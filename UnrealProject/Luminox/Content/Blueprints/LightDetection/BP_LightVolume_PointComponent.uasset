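; Point-light volume for the light detection system that reports how much a linked light component contributes at a given location.
; The construction script sizes its sphere from Radius.
; GetLightContribution optionally line traces from the actor, returning zero when blocked.
; Otherwise it scales intensity by linear falloff over attenuation radius and a multiplier, clamps it non-negative, and flags OutOfRange when the pre-clamp value is well below zero.
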(fn `GetLightContribution`
  (params (Location :type "Vector Structure") (ActorsToIgnore :type "Array of Actor Object Reference (by ref)"))
  (returns (LightContribution :type "Float (double-precision)") (OutOfRange :type Boolean))
  (bind _lightcomponent (`self.LightComponent`))
  (bind _intensity (`LightComponentBase.Intensity` _lightcomponent))
  (bind _attenuationradius (`LocalLightComponent.AttenuationRadius` _lightcomponent))
  (bind _returnvalue (`KismetMathLibrary.FClamp` (* (* _intensity (- 1.0 (/ (`KismetMathLibrary.Vector_Distance` Location (`self.K2_GetActorLocation`)) (`KismetMathLibrary.FClamp` _attenuationradius 0.001 _attenuationradius)))) (`self.ContributionMulitplier`)) -100.0 _intensity))
  (if (`self.Raycast`)
    (bind (_outhit _returnvalue_2) (`KismetSystemLibrary.LineTraceSingle` (`self.K2_GetActorLocation`) (`local.Location`) "TraceTypeQuery5" false (`local.ActorsToIgnore`)))
    (if _returnvalue_2
      (return 0.0 false)
      (else
        _)))
  (return (`KismetMathLibrary.FClamp` _returnvalue 0.0 _intensity) (< _returnvalue -50.0)))

(fn `UserConstructionScript`
  (`SphereComponent.SetSphereRadius` (`self.Sphere`) (`self.Radius`) true))