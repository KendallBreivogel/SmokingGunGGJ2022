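; Light detection volume that reports how much a referenced point or spot light contributes at a location.
; Its sphere registers it with overlapping actors' SceneComp_LightDetector, starting at zero radius and expanding after a short BeginPlay delay.
; GetLightContribution scales intensity by linear distance falloff and a multiplier, gating spot lights by outer cone angle.
; An optional line trace zeroes blocked light, and strongly negative values flag out-of-range.
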(event `self.ReceiveBeginPlay`
  (bind _sphere (`self.Sphere`))
  (`SphereComponent.SetSphereRadius` _sphere 0.0 true)
  (`KismetSystemLibrary.Delay` 0.2)
  (`SphereComponent.SetSphereRadius` _sphere (`self.Radius`) true))

(event `self.Sphere.OnComponentBeginOverlap`
  (params (OverlappedComponent :type "PrimitiveComponent Object Reference") (OtherActor :type "Actor Object Reference") (OtherComp :type "PrimitiveComponent Object Reference") (OtherBodyIndex :type Integer) (bFromSweep :type Boolean) (SweepResult :type "HitResult Structure (by ref)"))
  (bind _returnvalue (`self.GetComponentByClass` OtherActor "/Game/Blueprints/LightDetection/SceneComp_LightDetector.SceneComp_LightDetector_C"))
  (bind _lightvolumes (`/Game/Blueprints/LightDetection/SceneComp_LightDetector.LightVolumes` _returnvalue))
  (if (`KismetSystemLibrary.IsValid` _returnvalue)
    (if (not (`KismetArrayLibrary.Array_Contains` _lightvolumes self))
      (`KismetArrayLibrary.Array_Add` _lightvolumes self))))

(fn `GetLightContribution`
  (params (Location :type "Vector Structure") (ActorsToIgnore :type "Array of Actor Object Reference"))
  (returns (LightContribution :type "Float (double-precision)") (OutOfRange :type Boolean))
  (bind _light (`self.Light`))
  (bind _returnvalue (`KismetMathLibrary.Vector_Distance` Location (`self.K2_GetActorLocation`)))
  (bind _returnvalue_2 (`KismetMathLibrary.Normal` (- (`self.K2_GetActorLocation`) (`local.Location`))))
  (if (`self.Raycast`)
    (bind (_outhit _returnvalue_3) (`KismetSystemLibrary.LineTraceSingle` (`self.K2_GetActorLocation`) (`local.Location`) "TraceTypeQuery5" false (`local.ActorsToIgnore`)))
    (if _returnvalue_3
      (return 0.0 false)
      (else
        _)))
  (bind _aspoint_light (cast `PointLight` _light)
    (:`then`
      (bind _intensity (`LightComponentBase.Intensity` (`PointLight.PointLightComponent` _aspoint_light)))
      (bind _returnvalue_4 (`KismetMathLibrary.FClamp` (* (* _intensity (- 1.0 (/ _returnvalue (`self.Radius`)))) (`self.ContributionMulitplier`)) -100.0 _intensity))
      (return (`KismetMathLibrary.FClamp` _returnvalue_4 0.0 _intensity) (< _returnvalue_4 -50.0)))
    (:`CastFailed`
      (bind _asspot_light (cast `SpotLight` _light))
      (bind _spotlightcomponent (`SpotLight.SpotLightComponent` _asspot_light))
      (bind _returnvalue_5 (`KismetMathLibrary.Normal` (* (`self.GetActorForwardVector` _asspot_light) -1.0)))
      (bind (_returnvalue_x _returnvalue_y _returnvalue_z) (`KismetMathLibrary.BreakVector` (`KismetMathLibrary.Cross_VectorVector` _returnvalue_5 _returnvalue_2)))
      (bind _returnvalue_6 (* (`LightComponentBase.Intensity` _spotlightcomponent) (`KismetMathLibrary.SelectFloat` 1.0 0.0 (<= (`KismetMathLibrary.Abs` (* (`KismetMathLibrary.DegAcos` (`KismetMathLibrary.Dot_VectorVector` _returnvalue_5 _returnvalue_2)) (`KismetMathLibrary.SelectFloat` 1.0 -1.0 (> _returnvalue_z 0.0)))) (`SpotLightComponent.OuterConeAngle` _spotlightcomponent)))))
      (bind _returnvalue_7 (`KismetMathLibrary.FClamp` (* (* _returnvalue_6 (- 1.0 (/ _returnvalue (`self.Radius`)))) (`self.ContributionMulitplier`)) -100.0 _returnvalue_6))
      (return (`KismetMathLibrary.FClamp` _returnvalue_7 0.0 _returnvalue_6) (< _returnvalue_7 -50.0)))))

(fn `Set New Radius`
  (params (Radius :type "Float (double-precision)"))
  (bind _output_get (set `self.Radius` Radius))
  (`SphereComponent.SetSphereRadius` (`self.Sphere`) _output_get true))

(fn `UserConstructionScript`)