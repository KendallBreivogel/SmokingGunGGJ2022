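; BP_Plant_LightOrbGroup is a plant actor that groups three BP_Plant_LightOrb child actors around a single PointLight.
; Its construction script casts each child actor in turn and assigns the group's PointLight to that orb's PointLight variable, so all three reference the same light.
; A failed cast stops the chain, and the event graph holds only disabled placeholder events.
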(fn `UserConstructionScript`
  (bind _pointlight (`self.PointLight`))
  (bind _asbp_plant_light_orb (cast `/Game/Blueprints/Plants/BP_Plant_LightOrb` (`ChildActorComponent.ChildActor` (`self.BP_Plant_LightOrb`))))
  (set `/Game/Blueprints/Plants/BP_Plant_LightOrb.PointLight` _pointlight _asbp_plant_light_orb)
  (bind _asbp_plant_light_orb_2 (cast `/Game/Blueprints/Plants/BP_Plant_LightOrb` (`ChildActorComponent.ChildActor` (`self.BP_Plant_LightOrb1`))))
  (set `/Game/Blueprints/Plants/BP_Plant_LightOrb.PointLight` _pointlight _asbp_plant_light_orb_2)
  (bind _asbp_plant_light_orb_3 (cast `/Game/Blueprints/Plants/BP_Plant_LightOrb` (`ChildActorComponent.ChildActor` (`self.BP_Plant_LightOrb2`))))
  (set `/Game/Blueprints/Plants/BP_Plant_LightOrb.PointLight` _pointlight _asbp_plant_light_orb_3))