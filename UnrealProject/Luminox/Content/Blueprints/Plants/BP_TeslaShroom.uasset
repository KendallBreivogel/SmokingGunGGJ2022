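; BP_TeslaShroom is a plant that charges the player's multi-tool while damaging the player who stands within its sphere.
; Sphere overlap by the first-person character starts the multi-tool charging state and a fast looping timer.
; Each tick of the timer applies slight damage to the player and calls DepleteBattery with a negative amount to refill the battery.
; Leaving the sphere clears the timer and ends charging.
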(event `self.Sphere.OnComponentBeginOverlap`
  (params (OverlappedComponent :type "PrimitiveComponent Object Reference") (OtherActor :type "Actor Object Reference") (OtherComp :type "PrimitiveComponent Object Reference") (OtherBodyIndex :type Integer) (bFromSweep :type Boolean) (SweepResult :type "HitResult Structure (by ref)"))
  (bind _asfirst_person_character (cast `/Game/ExtraContent/FirstPersonBP/Blueprints/FirstPersonCharacter` OtherActor))
  (set `self.Player` _asfirst_person_character)
  (bind _returnvalue (`KismetSystemLibrary.K2_SetTimerDelegate` (delegate `ChargeTool`) 0.03 true))
  (set `self.ChargeTimer` _returnvalue)
  (`/Game/Blueprints/Tools/BP_MultiTool.Begin Charging` (`/Game/ExtraContent/FirstPersonBP/Blueprints/FirstPersonCharacter.MultiTool` (`self.Player`))))

(event `self.Sphere.OnComponentEndOverlap`
  (params (OverlappedComponent :type "PrimitiveComponent Object Reference") (OtherActor :type "Actor Object Reference") (OtherComp :type "PrimitiveComponent Object Reference") (OtherBodyIndex :type Integer))
  (cast `/Game/ExtraContent/FirstPersonBP/Blueprints/FirstPersonCharacter` OtherActor)
  (`KismetSystemLibrary.K2_ClearAndInvalidateTimerHandle` (`self.ChargeTimer`))
  (`/Game/Blueprints/Tools/BP_MultiTool.End Charging` (`/Game/ExtraContent/FirstPersonBP/Blueprints/FirstPersonCharacter.MultiTool` (`self.Player`))))

(event `ChargeTool`
  (bind _player (`self.Player`))
  (`GameplayStatics.ApplyDamage` _player 0.1)
  (`/Game/Blueprints/Tools/BP_MultiTool.DepleteBattery` (`/Game/ExtraContent/FirstPersonBP/Blueprints/FirstPersonCharacter.MultiTool` _player) -0.004))

(fn `UserConstructionScript`)