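; Thorny vine that grows along a spline and retracts when the light at its sensor rises above a threshold, regrowing when it falls.
; Construction script builds spline mesh sections sharing a dynamic material and positions the light detector.
; A looping timer polls the detector, using paired DoOnce gates to trigger growth or retraction once per change.
; A timeline animates the material's Radius parameter, toggling each section's collision to match.
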(event `self.ReceiveBeginPlay`
  (`parent.ReceiveBeginPlay`)
  (`KismetSystemLibrary.K2_SetTimerDelegate` (delegate `UpdateLighting`) 0.5 true)
  (`self.Grow` false))

(event `UpdateLighting`
  (bind _lightlevel (`/Game/Blueprints/LightDetection/SceneComp_LightDetector.GetTotalLightLevel` (`self.SceneComp_LightDetector`)))
  (if (> _lightlevel (`self.LightLevelThreshold`))
    (`|ExecutionSequence`
      (:`then_0`
        (`/Engine/EditorBlueprintResources/StandardMacros.DoOnce` false :!label _label
          (:`Completed`
            (`self.Grow` true))))
      (:`then_1`
        (goto _label_2 :!via `Reset`)))
    (else
      (`|ExecutionSequence`
        (:`then_0`
          (`/Engine/EditorBlueprintResources/StandardMacros.DoOnce` true :!label _label_2
            (:`Completed`
              (`self.Grow` false))))
        (:`then_1`
          (goto _label :!via `Reset`))))))

(event `Grow`
  (params (IsRetracting :type Boolean))
  (bind _output (`|GetArrayItem` (`self.SplineMeshes`) (- (`self.CurrentSplineIndex`) 1)))
  (bind _returnvalue (* (/ 1.0 (`KismetMathLibrary.Conv_IntToDouble` (`KismetArrayLibrary.Array_Length` (`self.SplineMeshes`)))) (`KismetMathLibrary.Conv_IntToDouble` (`self.CurrentSplineIndex`))))
  (`TimelineComponent.SetPlayRate` (`self.GrowAnim`) (/ 1.0 (`self.GrowSpeed`)))
  (set `self.CurrentSplineIndex` (select `bool` IsRetracting :`false` 1 :`true` (`KismetArrayLibrary.Array_Length` (`self.SplineMeshes`))))
  (if IsRetracting
    (bind (_direction _alpha) (`Timeline|GrowAnim` :!via `Reverse` :!label _label_3)
      (:`Update`
        (`MaterialInstanceDynamic.SetScalarParameterValue` (`self.Material_Vine`) "Radius" (`KismetMathLibrary.Lerp` (`self.StartingVineLength`) (+ (`SplineComponent.GetSplineLength` (`self.Spline`)) 1000.0) _alpha))
        (if IsRetracting
          (if (< _alpha _returnvalue)
            (`PrimitiveComponent.SetCollisionEnabled` _output "NoCollision")
            (`/Engine/EditorBlueprintResources/StandardMacros.DecrementInt` (`self.CurrentSplineIndex`)))
          (elif (> _alpha _returnvalue)
            (`PrimitiveComponent.SetCollisionEnabled` _output "QueryAndPhysics")
            (`/Engine/EditorBlueprintResources/StandardMacros.IncrementInt` (`self.CurrentSplineIndex`)))))
      (:`Finished`
        (`PrimitiveComponent.SetCollisionEnabled` (`|GetArrayItem` (`self.SplineMeshes`)) "QueryAndPhysics")))
    (else
      (goto _label_3))))

(fn `UserConstructionScript`
  (bind _vinesectionsize (`self.VineSectionSize`))
  (bind _spline (`self.Spline`))
  (`parent.UserConstructionScript`)
  (bind _returnvalue (`KismetMaterialLibrary.CreateDynamicMaterialInstance` "/Game/Environment/Plants/Vines/MI_Vine_Thorns.MI_Vine_Thorns"))
  (set `self.Material_Vine` _returnvalue)
  (`MaterialInstanceDynamic.SetScalarParameterValue` (`self.Material_Vine`) "Radius" (`self.StartingVineLength`))
  (`KismetArrayLibrary.Array_Clear` (`self.SplineMeshes`))
  (bind _output_get (set `self.SplineMeshes` (`self.K2_GetComponentsByClass` "/Script/Engine.SplineMeshComponent")))
  (for _array_element _output_get
    (`ActorComponent.K2_DestroyComponent` _array_element))
  (for _index (range (+ (`KismetMathLibrary.FTrunc` (/ (`SplineComponent.GetSplineLength` (`self.Spline`)) (`self.VineSectionSize`))) 1))
    (bind _returnvalue_2 (`AddComponent|NODE_AddSplineMeshComponent-3`))
    (bind _returnvalue_3 (* _vinesectionsize (`KismetMathLibrary.Conv_IntToDouble` _index)))
    (bind _returnvalue_4 (* _vinesectionsize (`KismetMathLibrary.Conv_IntToDouble` (+ _index 1))))
    (`SplineMeshComponent.SetStartAndEnd` _returnvalue_2 (`SplineComponent.GetLocationAtDistanceAlongSpline` _spline _returnvalue_3 "Local") (`SplineComponent.GetTangentAtDistanceAlongSpline` _spline _returnvalue_3 "Local") (`SplineComponent.GetLocationAtDistanceAlongSpline` _spline _returnvalue_4 "Local") (`SplineComponent.GetTangentAtDistanceAlongSpline` _spline _returnvalue_4 "Local") true)
    (`PrimitiveComponent.SetMaterial` _returnvalue_2 0 (`self.Material_Vine`))
    (`PrimitiveComponent.SetCollisionEnabled` _returnvalue_2 (select `bool` (== _index 0) :`false` "NoCollision" :`true` "QueryAndPhysics" :!type "ECollisionEnabled Enum"))
    (`KismetArrayLibrary.Array_Add` (`self.SplineMeshes`) _returnvalue_2))
  (`SceneComponent.K2_SetRelativeLocation` (`self.SceneComp_LightDetector`) (`self.LightSensorLocation`) false false))