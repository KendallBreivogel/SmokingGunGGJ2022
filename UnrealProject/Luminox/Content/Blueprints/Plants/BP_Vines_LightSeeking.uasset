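; Light-seeking vine plant that grows along a spline when a bright enough light is near its tip, and retracts when that light is gone.
; The construction script builds spline mesh sections with dynamic vine and leaf materials, placing an acceptance sphere at the spline's end.
; A looping timer polls the light detector, triggering a timeline through DoOnce gates.
; The timeline animates the materials' Radius to reveal the vine while toggling each section's collision in step.
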(event `self.ReceiveBeginPlay`
  (`parent.ReceiveBeginPlay`)
  (`KismetSystemLibrary.K2_SetTimerDelegate` (delegate `UpdateLighting`) 0.5 true))

(event `UpdateLighting`
  (set `self.FoundValidLight` false)
  (bind (_lightlevel _lightvolume) (`/Game/Blueprints/LightDetection/SceneComp_LightDetector.GetAllLightsInVicinity` (`self.SceneComp_LightDetector`)))
  (for (_array_element _array_index) _lightvolume
    (if (> (`|GetArrayItem` _lightlevel _array_index) (`self.LightLevelThreshold`))
      (if (<= (`KismetMathLibrary.Vector_Distance` (`self.K2_GetActorLocation` _array_element) (`SceneComponent.K2_GetComponentLocation` (`self.AcceptanceSphere`))) (`self.AcceptanceRadius`))
        (set `self.FoundValidLight` true)
        (`|ExecutionSequence`
          (:`then_0`
            (`/Engine/EditorBlueprintResources/StandardMacros.DoOnce` false :!label _label
              (:`Completed`
                (`self.Grow` false)
                (`AudioComponent.FadeIn` (`self.foliage`) 0.0 1.0 0.0 "Linear" :!label _label_2))))
          (:`then_1`
            (goto _label_3 :!via `Reset`))))))
  (if (not (`self.FoundValidLight`))
    (`|ExecutionSequence`
      (:`then_0`
        (`/Engine/EditorBlueprintResources/StandardMacros.DoOnce` true :!label _label_3
          (:`Completed`
            (`self.Grow` true)
            (goto _label_2))))
      (:`then_1`
        (goto _label :!via `Reset`)))))

(event `Grow`
  (params (IsRetracting :type Boolean))
  (bind _output (`|GetArrayItem` (`self.SplineMeshes`) (- (`self.CurrentSplineIndex`) 1)))
  (bind _returnvalue (* (/ 1.0 (`KismetMathLibrary.Conv_IntToDouble` (`KismetArrayLibrary.Array_Length` (`self.SplineMeshes`)))) (`KismetMathLibrary.Conv_IntToDouble` (`self.CurrentSplineIndex`))))
  (`TimelineComponent.SetPlayRate` (`self.GrowAnim`) (/ 1.0 (`self.GrowSpeed`)))
  (set `self.CurrentSplineIndex` (select `bool` IsRetracting :`false` 1 :`true` (`KismetArrayLibrary.Array_Length` (`self.SplineMeshes`))))
  (if IsRetracting
    (bind (_direction _alpha) (`Timeline|GrowAnim` :!via `Reverse` :!label _label_4)
      (:`Update`
        (`MaterialInstanceDynamic.SetScalarParameterValue` (`self.Material_Vine`) "Radius" (`KismetMathLibrary.Lerp` (`self.StartingVineLength`) (+ (`SplineComponent.GetSplineLength` (`self.Spline`)) 1000.0) _alpha))
        (`MaterialInstanceDynamic.SetScalarParameterValue` (`self.Material_Leaves`) "Radius" (`KismetMathLibrary.Lerp` (`self.StartingVineLength`) (+ (`SplineComponent.GetSplineLength` (`self.Spline`)) 1000.0) _alpha))
        (if IsRetracting
          (if (< _alpha _returnvalue)
            (`PrimitiveComponent.SetCollisionEnabled` _output "NoCollision")
            (`/Engine/EditorBlueprintResources/StandardMacros.DecrementInt` (`self.CurrentSplineIndex`)))
          (elif (> _alpha _returnvalue)
            (`PrimitiveComponent.SetCollisionEnabled` _output "QueryAndPhysics")
            (`/Engine/EditorBlueprintResources/StandardMacros.IncrementInt` (`self.CurrentSplineIndex`)))))
      (:`Finished`
        (`PrimitiveComponent.SetCollisionEnabled` (`|GetArrayItem` (`self.SplineMeshes`)) "QueryAndPhysics")
        (`AudioComponent.FadeOut` (`self.foliage`) 0.0 0.0 "Linear")))
    (else
      (goto _label_4))))

(fn `UserConstructionScript`
  (bind _spline (`self.Spline`))
  (bind _vinesectionsize (`self.VineSectionSize`))
  (bind _spline_2 (`self.Spline`))
  (`parent.UserConstructionScript`)
  (bind _returnvalue (`KismetMaterialLibrary.CreateDynamicMaterialInstance` "/Game/Environment/Plants/Vines/M_Vine_Master.M_Vine_Master"))
  (set `self.Material_Vine` _returnvalue)
  (bind _returnvalue_2 (`KismetMaterialLibrary.CreateDynamicMaterialInstance` "/Game/Environment/Plants/Vines/M_Vine_Leaves.M_Vine_Leaves"))
  (set `self.Material_Leaves` _returnvalue_2)
  (`MaterialInstanceDynamic.SetScalarParameterValue` (`self.Material_Vine`) "Radius" (`self.StartingVineLength`))
  (`MaterialInstanceDynamic.SetScalarParameterValue` (`self.Material_Leaves`) "Radius" (`self.StartingVineLength`))
  (`KismetArrayLibrary.Array_Clear` (`self.SplineMeshes`))
  (bind _output_get (set `self.SplineMeshes` (`self.K2_GetComponentsByClass` "/Script/Engine.SplineMeshComponent")))
  (for _array_element _output_get
    (`ActorComponent.K2_DestroyComponent` _array_element))
  (for _index (range (+ (`KismetMathLibrary.FTrunc` (/ (`SplineComponent.GetSplineLength` (`self.Spline`)) (`self.VineSectionSize`))) 1))
    (bind _returnvalue_3 (`AddComponent|NODE_AddSplineMeshComponent-3`))
    (bind _returnvalue_4 (* _vinesectionsize (`KismetMathLibrary.Conv_IntToDouble` _index)))
    (bind _returnvalue_5 (* _vinesectionsize (`KismetMathLibrary.Conv_IntToDouble` (+ _index 1))))
    (`SplineMeshComponent.SetStartAndEnd` _returnvalue_3 (`SplineComponent.GetLocationAtDistanceAlongSpline` _spline_2 _returnvalue_4 "Local") (`SplineComponent.GetTangentAtDistanceAlongSpline` _spline_2 _returnvalue_4 "Local") (`SplineComponent.GetLocationAtDistanceAlongSpline` _spline_2 _returnvalue_5 "Local") (`SplineComponent.GetTangentAtDistanceAlongSpline` _spline_2 _returnvalue_5 "Local") true)
    (`PrimitiveComponent.SetMaterial` _returnvalue_3 0 (`self.Material_Vine`))
    (`PrimitiveComponent.SetMaterial` _returnvalue_3 1 (`self.Material_Leaves`))
    (`PrimitiveComponent.SetCollisionEnabled` _returnvalue_3 (select `bool` (== _index 0) :`false` "NoCollision" :`true` "QueryAndPhysics" :!type "ECollisionEnabled Enum"))
    (`KismetArrayLibrary.Array_Add` (`self.SplineMeshes`) _returnvalue_3))
  (`SceneComponent.K2_SetRelativeLocation` (`self.SceneComp_LightDetector`) (`self.LightSensorLocation`) false false)
  (`SceneComponent.K2_SetRelativeLocation` (`self.AcceptanceSphere`) (`SplineComponent.GetLocationAtDistanceAlongSpline` _spline (`SplineComponent.GetSplineLength` _spline) "Local") false false)
  (`SphereComponent.SetSphereRadius` (`self.AcceptanceSphere`) (`self.AcceptanceRadius`) true))