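; Canister prop actor whose colored material can be lit or dimmed at runtime.
; On BeginPlay or an InitializeCanisterMaterial call it creates a dynamic instance of M_Cannister_Simple on the mesh's second material slot, applies the stored CanisterColor and sets full brightness.
; ToggleCanister switches the Brightness parameter on or off, while SetCanisterColor only stores the color until the next initialization or explicit material color change.
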(event `self.ReceiveBeginPlay`
  (`self.InitializeCanister`))

(event `/Game/Blueprints/Interfaces/BPI_Canister.InitializeCanisterMaterial`
  (`self.InitializeCanister`))

(event `/Game/Blueprints/Interfaces/BPI_Canister.ToggleCanister`
  (params (ToggleCanisterOn :type Boolean))
  (`self.SetMaterialBrightness` (`KismetMathLibrary.SelectFloat` 1.0 0.0 ToggleCanisterOn)))

(fn `ChangeMaterialColor`
  (params (NewMaterialColor :type "LinearColor Structure"))
  (`MaterialInstanceDynamic.SetVectorParameterValue` (`self.DynamicMaterial`) "Color" NewMaterialColor))

(fn `CreateDynamicMaterial`
  (bind _returnvalue (`KismetMaterialLibrary.CreateDynamicMaterialInstance` "/Game/Blueprints/Tools/Mesh/M_Cannister_Simple.M_Cannister_Simple"))
  (`self.SetDynamicMaterial` _returnvalue)
  (`PrimitiveComponent.SetMaterial` (`self.SM_Canister`) 1 (`self.DynamicMaterial`)))

(fn `GetCanisterColor`
  (returns (Color :type "LinearColor Structure"))
  (return (`self.CanisterColor`)))

(fn `InitializeCanister`
  (`self.CreateDynamicMaterial`)
  (`self.ChangeMaterialColor` (`self.CanisterColor`))
  (`self.SetMaterialBrightness` 1.0))

(fn `SetCanisterColor`
  (params (NewCanisterColor :type "LinearColor Structure"))
  (set `self.CanisterColor` NewCanisterColor))

(fn `SetDynamicMaterial`
  (params (DynamicMaterial :type "MaterialInstanceDynamic Object Reference"))
  (set `self.DynamicMaterial` DynamicMaterial))

(fn `SetMaterialBrightness`
  (params (Brightness :type "Float (double-precision)"))
  (`MaterialInstanceDynamic.SetScalarParameterValue` (`self.DynamicMaterial`) "Brightness" Brightness))

(fn `UserConstructionScript`)