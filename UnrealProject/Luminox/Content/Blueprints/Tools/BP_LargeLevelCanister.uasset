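; BP_LargeLevelCanister is a level pickup that unlocks a MultiTool mode: Scanner, Laser, Plasma Flare or Grapple.
; EnumToolMode sets the mesh color through a dynamic material in the construction script and at BeginPlay.
; A scannable widget above it serves as an indicator, hidden once scanned.
; Interact adds the mode to the player's MultiTool, passes it matching audio and text, refreshes canisters and destroys the actor.
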(event `self.ReceiveBeginPlay`
  (bind _asfirst_person_character (cast `/Game/ExtraContent/FirstPersonBP/Blueprints/FirstPersonCharacter` (`GameplayStatics.GetPlayerCharacter` 0)))
  (set `self.PlayerRef` _asfirst_person_character)
  (`self.Set New Canister Color`)
  (`self.ConstructIndicatorUI`))

(event `self.ReceiveHit`
  (params (MyComp :type "PrimitiveComponent Object Reference") (Other :type "Actor Object Reference") (OtherComp :type "PrimitiveComponent Object Reference") (bSelfMoved :type Boolean) (HitLocation :type "Vector Structure") (HitNormal :type "Vector Structure") (NormalImpulse :type "Vector Structure") (Hit :type "HitResult Structure (by ref)")))

(fn `ConstructIndicatorUI`
  (bind _scannableui (`self.ScannableUI`))
  (bind _asinteractable_ui (cast `/Game/UI/InteractableUi` (`WidgetComponent.GetUserWidgetObject` (`self.ScannableUI`))))
  (set `/Game/UI/InteractableUi.Owner` (`self.ScannableUI`) _asinteractable_ui)
  (if (not (`self.HasBeenScanned`))
    (`/Engine/EditorBlueprintResources/StandardMacros.IsValid` _scannableui
      (:`Is Valid`
        (bind _asinteractable_ui_2 (cast `/Game/UI/InteractableUi` (`WidgetComponent.GetWidget` _scannableui)))
        (set `self.IndicatorUI` _asinteractable_ui_2)))))

(fn `Interact`
  (returns (Success :type Boolean))
  (bind _enumtoolmode (`self.EnumToolMode`))
  (bind _returnvalue (select `/Game/Blueprints/Tools/Enum_ToolModes` _enumtoolmode :`NewEnumerator3` "/Game/Audio/Voiceover/av_na_scanner_mod.av_na_scanner_mod" :`NewEnumerator0` "/Game/Audio/Voiceover/av_na_laser_mod.av_na_laser_mod" :`NewEnumerator2` "/Game/Audio/Voiceover/av_na_flare_mod.av_na_flare_mod" :`NewEnumerator1` "/Game/Audio/Voiceover/av_na_grapple_mod.av_na_grapple_mod" :!type "SoundBase Object Reference"))
  (bind _multitool (`/Game/ExtraContent/FirstPersonBP/Blueprints/FirstPersonCharacter.MultiTool` (`self.PlayerRef`)))
  (`KismetArrayLibrary.Array_Add` (`/Game/Blueprints/Tools/BP_MultiTool.AvailableModes` _multitool) _enumtoolmode)
  (`/Engine/EditorBlueprintResources/StandardMacros.IsValid` _returnvalue
    (:`Is Valid`
      (`/Game/Blueprints/Tools/BP_MultiTool.CannisterAdded` (`/Game/ExtraContent/FirstPersonBP/Blueprints/FirstPersonCharacter.MultiTool` (`self.PlayerRef`)) _returnvalue (select `/Game/Blueprints/Tools/Enum_ToolModes` _enumtoolmode :`NewEnumerator3` "Loaded: Scanner Module" :`NewEnumerator0` "Loaded: Laser Module" :`NewEnumerator2` "Loaded: Flare Module" :`NewEnumerator1` "Loaded: Grapple Module") (select `/Game/Blueprints/Tools/Enum_ToolModes` _enumtoolmode :`NewEnumerator3` "Loaded: Scanner Module" :`NewEnumerator0` "Aim multitool and initiate firing to emit a powerful beam. United Terraforming assumes no responsibility for any death or injury that may occur while using this module." :`NewEnumerator2` "Aim multitool and fire to launch a plasma flare. Average flare lifespan is around 15 seconds." :`NewEnumerator1` "Aim multitool at any valid grapple target and fire to pull user towards destination location. Use with extreme caution.")))
    (:`Is Not Valid`
      _))
  (`/Game/Blueprints/Tools/BP_MultiTool.InitCannisters` _multitool)
  (`self.K2_DestroyActor`)
  (return false))

(fn `Set New Canister Color`
  (bind _returnvalue (`KismetMaterialLibrary.CreateDynamicMaterialInstance` "/Game/Blueprints/Tools/Mesh/M_Cannister_Simple.M_Cannister_Simple"))
  (bind _output_get (set `self.MaterialRef` _returnvalue))
  (`PrimitiveComponent.SetMaterial` (`self.SM_Canister`) 1 _output_get)
  (switch `/Game/Blueprints/Tools/Enum_ToolModes` (`self.EnumToolMode`)
    (:`NewEnumerator3`
      (set `self.CanisterColor_0` (struct :`G` 0.904661 :`B` 0.012983 :`A` 1.0)))
    (:`NewEnumerator0`
      (set `self.CanisterColor_0` (struct :`R` 1.0 :`G` 0.47932 :`A` 1.0)))
    (:`NewEnumerator2`
      (set `self.CanisterColor_0` (struct :`R` 1.0 :`A` 1.0)))
    (:`NewEnumerator1`
      (set `self.CanisterColor_0` (struct :`G` 1.0 :`B` 0.991102 :`A` 1.0))))
  (`MaterialInstanceDynamic.SetVectorParameterValue` (`self.MaterialRef`) "Color" (`self.CanisterColor_0`))
  (`MaterialInstanceDynamic.SetScalarParameterValue` (`self.MaterialRef`) "Brightness" 1.0))

(fn `SetIndicatorUIVisisble`
  (params (IsVisible :type Boolean))
  (locals (visible :type Boolean))
  (bind _indicatorui (`self.IndicatorUI`))
  (set `local.visible` IsVisible)
  (if (`self.HasBeenScanned`)
    (set `local.visible` false))
  (`/Engine/EditorBlueprintResources/StandardMacros.IsValid` _indicatorui
    (:`Is Valid`
      (`Widget.SetVisibility` _indicatorui (select `bool` (`local.visible`) :`false` "Hidden" :`true` "Visible" :!type "ESlateVisibility Enum")))))

(fn `UserConstructionScript`
  (bind (_returnvalue_x _returnvalue_y _returnvalue_z) (`KismetMathLibrary.BreakVector` (`self.K2_GetActorLocation`)))
  (`self.Set New Canister Color`)
  (`SceneComponent.K2_SetWorldLocation` (`self.ScannableUI`) (`KismetMathLibrary.MakeVector` _returnvalue_x _returnvalue_y (+ _returnvalue_z 50.0)) false false))