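; Player multitool with battery-powered scanner, laser, plasma flare and grapple modes, plus a flashlight.
; Scrolling cycles available modes, animating colored canisters; the main canister material displays mode color and battery fill, and empty power stops laser and flashlight.
; Timers drive laser traces, which damage actors or show reflections off some monsters, and grapple pulls toward grapple points.
; Scanning finds BPI_Scannable actors, plays their info audio and updates the HUD.
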(event `FireGrappleLine`
  (bind _returnvalue (`GameplayStatics.GetPlayerCameraManager` 0))
  (bind _cable (`self.Cable`))
  (bind _cable_2 (`self.Cable`))
  (bind _returnvalue_2 (`PlayerCameraManager.GetCameraLocation` _returnvalue))
  (if (`self.Grappled`)
    (`KismetSystemLibrary.K2_ClearAndInvalidateTimerHandle` (`self.GrappleTimer`))
    (`SceneComponent.SetHiddenInGame` _cable_2 true false)
    (set `CableComponent.EndLocation` (50.0 0.0 0.0) _cable_2)
    (set `self.CanFireGrapple` true)
    (set `self.Grappled` false)
    (set `CharacterMovementComponent.GravityScale` 1.0 (`Character.CharacterMovement` (`self.Player`)))
    (set `self.PullVelocity` 5.0)
    (elif (`self.CanFireGrapple`)
      (bind (_outhit _returnvalue_3) (`KismetSystemLibrary.LineTraceSingleForObjects` _returnvalue_2 (+ _returnvalue_2 (* (`self.GetActorForwardVector` _returnvalue) 15000.0)) (`|MakeArray` "ObjectTypeQuery1" :!type "EObjectTypeQuery Enum")))
      (if _returnvalue_3
        (bind (_bblockinghit _binitialoverlap _time _distance _location _impactpoint _normal _impactnormal _physmat _hitactor) (`GameplayStatics.BreakHitResult` _outhit))
        (cast `/Game/Blueprints/Tools/BP_GrapplePoint` _hitactor)
        (set `self.CanFireGrapple` false)
        (`/Game/ExtraContent/FirstPersonBP/Blueprints/FirstPersonCharacter.FireKickback` (`self.Player`))
        (`AudioComponent.Play` (`self.Flare`) 0.0)
        (set `self.InitialGrappleLocation` (`self.K2_GetActorLocation` (`self.Player`)))
        (set `self.GrappleLocation` _location)
        (`SceneComponent.SetHiddenInGame` (`self.Cable`) false false)
        (`self.DepleteBattery` 0.1)
        (bind (_direction _alpha) (`Timeline|CastGrappleLine` :!via `PlayFromStart`)
          (:`Update`
            (set `CableComponent.EndLocation` (`KismetMathLibrary.VLerp` (`CableComponent.EndLocation` _cable) (`KismetMathLibrary.InverseTransformLocation` (`self.GetTransform`) (`self.GrappleLocation`)) _alpha) _cable))
          (:`Finished`
            (bind _returnvalue_4 (`KismetSystemLibrary.K2_SetTimerDelegate` (delegate `PullPlayerToGrapple`) 0.03 true))
            (set `self.GrappleTimer` _returnvalue_4)))))))

(event `PullPlayerToGrapple`
  (bind _grapplelocation (`self.GrappleLocation`))
  (bind _returnvalue (`self.K2_GetActorLocation` (`self.Player`)))
  (bind _charactermovement (`Character.CharacterMovement` (`self.Player`)))
  (set `CableComponent.EndLocation` (`KismetMathLibrary.InverseTransformLocation` (`self.GetTransform`) (`self.GrappleLocation`)) (`self.Cable`))
  (`Character.LaunchCharacter` (`self.Player`) (* (- _grapplelocation _returnvalue) (`self.PullVelocity`)) true true)
  (if (<= (`KismetMathLibrary.Vector_Distance` _grapplelocation _returnvalue) 300.0)
    (set `self.Grappled` true)
    (set `self.PullVelocity` 0.0)
    (set `CharacterMovementComponent.GravityScale` 0.0 _charactermovement)
    (set `MovementComponent.Velocity` (0.0 0.0 0.0) _charactermovement)))

(event `self.ReceiveBeginPlay`
  (`self.ScrollEquipped` false)
  (`self.InitCannisters`)
  (`self.SearchForUnscannedSubjects`))

(event `BeginFiring`
  (bind _hasbatterypower (`self.CheckHasPower`))
  (if _hasbatterypower
    (switch `/Game/Blueprints/Tools/Enum_ToolModes` (`self.Mode`)
      (:`NewEnumerator3`
        (`self.Scan`))
      (:`NewEnumerator0`
        (`self.StartLaser`))
      (:`NewEnumerator2`
        (`self.FireFlare`))
      (:`NewEnumerator1`
        (`self.FireGrappleLine`)))))

(event `StopFiring`
  (`self.StopLaser`))

(event `FireFlare`
  (`self.LaunchFlare`)
  (`self.DepleteBattery` 0.25)
  (`KismetSystemLibrary.Delay` (`self.FlareCooldownTime`))
  (set `self.CanFireFlare` true))

(event `StartLaser`
  (bind _returnvalue (`KismetSystemLibrary.K2_SetTimerDelegate` (delegate `Laser`) 0.03 true))
  (set `self.LaserTimer` _returnvalue)
  (`SceneComponent.SetHiddenInGame` (`self.FBX_LaserPlane`) false false)
  (`ActorComponent.SetActive` (`self.P_Sparks_Laser`) true false)
  (`LocalLightComponent.SetAttenuationRadius` (`self.PointLight`) 100.0)
  (`AudioComponent.FadeIn` (`self.Laser1`) 0.0 1.0 0.0 "Linear"))

(event `Laser`
  (bind _fbx_laserplane (`self.FBX_LaserPlane`))
  (bind _returnvalue (`SceneComponent.K2_GetComponentLocation` _fbx_laserplane))
  (bind (_outhit _wasahit) (`self.LineTraceFromActorForward` (`GameplayStatics.GetPlayerCameraManager` 0) 5000.0 (`|MakeArray` null :!type "Actor Object Reference")))
  (if _wasahit
    (`SceneComponent.K2_SetWorldRotation` (`self.FBX_LaserPlane`) (`KismetMathLibrary.FindLookAtRotation` (`SceneComponent.K2_GetComponentLocation` (`self.FBX_LaserPlane`)) (`.Location` (`GameplayStatics.BreakHitResult` _outhit))) false false))
  (bind (_outhit_2 _returnvalue_2) (`KismetSystemLibrary.LineTraceSingle` _returnvalue (+ _returnvalue (* (`SceneComponent.GetForwardVector` _fbx_laserplane) 5000.0)) "TraceTypeQuery1" false (`|MakeArray` (`self.Player`) :!type "Actor Object Reference") "None" true (struct :`R` 1.0 :`A` 1.0) (struct :`G` 1.0 :`A` 1.0) 0.1))
  (if _returnvalue_2
    (bind (_bblockinghit _binitialoverlap _time _distance _location _impactpoint _normal _impactnormal _physmat _hitactor) (`GameplayStatics.BreakHitResult` _outhit_2))
    (bind _asbp_monster (cast `/Game/Blueprints/Monsters/BP_Monster` _hitactor)
      (:`then`
        (bind _reflectlaser (`/Game/Blueprints/Monsters/BP_Monster.ReflectLaser` _asbp_monster))
        (`SceneComponent.SetHiddenInGame` (`self.FBX_LaserPlane_Refleced`) (not _reflectlaser) false)
        (if _reflectlaser
          (`SceneComponent.K2_SetWorldLocation` (`self.FBX_LaserPlane_Refleced`) _location false false)
          (`SceneComponent.K2_SetWorldRotation` (`self.FBX_LaserPlane_Refleced`) (`KismetMathLibrary.Conv_VectorToRotator` _normal) false false)
          (else
            (`GameplayStatics.ApplyDamage` _hitactor (`self.LaserDamage`) :!label _label))))
      (:`CastFailed`
        (`SceneComponent.SetHiddenInGame` (`self.FBX_LaserPlane_Refleced`) true false)
        (goto _label)))
    (`SceneComponent.SetRelativeScale3D` (`self.FBX_LaserPlane`) (`KismetMathLibrary.MakeVector` _distance 0.1 0.1))
    (`SceneComponent.K2_SetWorldLocation` (`self.P_Sparks_Laser`) _location false false)
    (`SceneComponent.K2_SetWorldLocation` (`self.PointLight`) (+ _location (* _normal 25.0)) false false)
    (`LocalLightComponent.SetAttenuationRadius` (`self.PointLight`) (`KismetMathLibrary.RandomFloatInRange` 0.0 100.0))
    (`/Game/Blueprints/BL_Senses.ActorNoise` (`GameplayStatics.GetPlayerPawn` 0) 1.0)
    (else
      (`SceneComponent.K2_SetWorldLocation` (`self.P_Sparks_Laser`) (0.0 0.0 20000.0) false false)))
  (`self.DepleteBattery` 0.001))

(event `StopLaser`
  (`KismetSystemLibrary.K2_ClearAndInvalidateTimerHandle` (`self.LaserTimer`))
  (`SceneComponent.SetHiddenInGame` (`self.FBX_LaserPlane`) true false)
  (`SceneComponent.SetHiddenInGame` (`self.FBX_LaserPlane_Refleced`) true false)
  (`ActorComponent.SetActive` (`self.P_Sparks_Laser`) false false)
  (`LocalLightComponent.SetAttenuationRadius` (`self.PointLight`) 0.0)
  (`AudioComponent.FadeOut` (`self.Laser1`) 0.1 0.0 "Linear"))

(event `ToggleFlashlight`
  (`GameplayStatics.PlaySound2D` "/Game/Blueprints/Character/Audio/WAV_Click.WAV_Click" 1.0 1.0 0.0 null null)
  (bind _hasbatterypower (`self.CheckHasPower`))
  (if _hasbatterypower
    (bind _output_get (set `self.FlashlightOn` (not (`self.FlashlightOn`))))
    (if _output_get
      (`self.UpdateFlashlightLighting` 6000.0 2000.0)
      (bind _returnvalue (`KismetSystemLibrary.K2_SetTimerDelegate` (delegate `FlashlightBatteryDrain`) 1.0 true))
      (set `self.FlashlightTimer` _returnvalue)
      (else
        (`self.KillFlashlight`)))))

(event `FlashlightBatteryDrain`
  (`self.DepleteBattery` 0.0)
  (if (== (`KismetMathLibrary.RandomIntegerInRange` 0 55) 0)
    (`self.FlashlightFlicker`)))

(event `FlashlightFlicker`
  (bind (_direction _power) (`Timeline|Flicker`)
    (:`Update`
      (`self.UpdateFlashlightLighting` (* _power 6000.0) (* _power 2000.0)))))

(event `KillFlashlight`
  (set `self.FlashlightOn` false)
  (`self.UpdateFlashlightLighting` 0.0)
  (`KismetSystemLibrary.K2_ClearAndInvalidateTimerHandle` (`self.FlashlightTimer`)))

(event `ScrollEquipped`
  (params (Dir :type Boolean) (Skip :type Boolean))
  (bind _mode (`self.Mode`))
  (bind _asmaterial_instance_dynamic (cast `MaterialInstanceDynamic` (`PrimitiveComponent.GetMaterial` (`self.CurrentModeCan`) 1) :!pure true))
  (bind _asmaterial_instance_dynamic_2 (cast `MaterialInstanceDynamic` (`PrimitiveComponent.GetMaterial` (`self.PreviousModeCan`) 1) :!pure true))
  (if (`self.isSwitchingMode`)
    (`|ExecutionSequence`
      (:`then_0`
        (`MaterialInstanceDynamic.SetScalarParameterValue` (cast `MaterialInstanceDynamic` (`PrimitiveComponent.GetMaterial` (`self.PreviousModeCan`) 1) :!pure true) "Brightness" 0.0))
      (:`then_1`
        (if (not Skip) :!label _label_2
          (set `self.PreviousModeCan` (select `/Game/Blueprints/Tools/Enum_ToolModes` _mode :`NewEnumerator3` (`self.ScannerCan`) :`NewEnumerator0` (`self.LaserCan`) :`NewEnumerator2` (`self.FlareCan`) :`NewEnumerator1` (`self.GrappleCan`))))
        (bind _output_get (set `self.Mode` (select `bool` Dir :`false` (select `/Game/Blueprints/Tools/Enum_ToolModes` _mode :`NewEnumerator3` "NewEnumerator0" :`NewEnumerator0` "NewEnumerator2" :`NewEnumerator2` "NewEnumerator1" :`NewEnumerator1` "NewEnumerator3" :!type "/Game/Blueprints/Tools/Enum_ToolModes Enum") :`true` (select `/Game/Blueprints/Tools/Enum_ToolModes` _mode :`NewEnumerator3` "NewEnumerator1" :`NewEnumerator0` "NewEnumerator3" :`NewEnumerator2` "NewEnumerator0" :`NewEnumerator1` "NewEnumerator2" :!type "/Game/Blueprints/Tools/Enum_ToolModes Enum"))))
        (if (`KismetArrayLibrary.Array_Contains` (`self.AvailableModes`) _output_get)
          (set `self.CurrentModeCan` (select `/Game/Blueprints/Tools/Enum_ToolModes` (`self.Mode`) :`NewEnumerator3` (`self.ScannerCan`) :`NewEnumerator0` (`self.LaserCan`) :`NewEnumerator2` (`self.FlareCan`) :`NewEnumerator1` (`self.GrappleCan`)))
          (set `self.isSwitchingMode` true)
          (bind (_direction _jut) (`Timeline|SwitchCan` :!via `PlayFromStart`)
            (:`Update`
              (bind _returnvalue (- 1.0 _jut))
              (`SceneComponent.K2_SetRelativeLocation` (`self.PreviousModeCan`) (`KismetMathLibrary.MakeVector` (* _returnvalue 2.0)) false false)
              (`SceneComponent.K2_SetRelativeLocation` (`self.CurrentModeCan`) (`KismetMathLibrary.MakeVector` (* _jut 2.0)) false false)
              (`MaterialInstanceDynamic.SetScalarParameterValue` _asmaterial_instance_dynamic_2 "Brightness" _returnvalue)
              (`MaterialInstanceDynamic.SetScalarParameterValue` _asmaterial_instance_dynamic "Brightness" _jut)
              (bind _returnvalue_2 (`MaterialInstanceDynamic.K2_GetVectorParameterValue` _asmaterial_instance_dynamic "Color"))
              (bind _returnvalue_3 (`MaterialInstanceDynamic.K2_GetVectorParameterValue` _asmaterial_instance_dynamic_2 "Color"))
              (`MaterialInstanceDynamic.SetVectorParameterValue` (`self.MainCannisterMat`) "Color" (`KismetMathLibrary.LinearColorLerp` _returnvalue_3 _returnvalue_2 _jut)))
            (:`Finished`
              (set `self.isSwitchingMode` false)))
          (else
            (`self.ScrollEquipped` Dir true)))))
    (else
      (goto _label_2))))

(event `Scan`
  (bind _scanobject (`self.scanObject`))
  (if (not (`self.isScanning`))
    (set `self.isScanning` true)
    (set `self.scanObject` null)
    (`SceneComponent.SetHiddenInGame` (`self.SM_ScanPlanes`) false false)
    (bind (_direction _movement) (`Timeline|ScanAnim` :!via `PlayFromStart`)
      (:`Update`
        (`SceneComponent.K2_SetRelativeRotation` (`self.SM_ScanPlanes`) (`KismetMathLibrary.MakeRotator` (+ (* _movement 25.0) 90.0)) false false)
        (bind (_outhit _wasahit) (`self.LineTraceFromActorForward` (`GameplayStatics.GetPlayerCameraManager` 0) 5000.0 (`|MakeArray` null :!type "Actor Object Reference")))
        (if _wasahit
          (bind (_bblockinghit _binitialoverlap _time _distance _location _impactpoint _normal _impactnormal _physmat _hitactor) (`GameplayStatics.BreakHitResult` _outhit))
          (`SceneComponent.SetWorldScale3D` (`self.SM_ScanPlanes`) (`KismetMathLibrary.MakeVector` 2.0 (/ (+ _distance 1000.0) 100.0) 5.0))
          (if (not (`KismetSystemLibrary.IsValid` (`self.scanObject`)))
            (if (`KismetSystemLibrary.DoesImplementInterface` _hitactor "/Game/Blueprints/Interfaces/BPI_Scannable.BPI_Scannable_C")
              (set `self.scanObject` _hitactor)))))
      (:`Finished`
        (set `self.isScanning` false)
        (`SceneComponent.SetHiddenInGame` (`self.SM_ScanPlanes`) true false)
        (if (`KismetSystemLibrary.IsValid` _scanobject)
          (`self.GetScanInfo` _scanobject))))))

(event `CannisterAdded`
  (params (CanisterAudio :type "SoundBase Object Reference") (CanisterTitle :type String) (CanisterTextBody :type String))
  (`AudioComponent.SetSound` (`self.Audio`) CanisterAudio)
  (`GameplayStatics.PlaySound2D` CanisterAudio 1.0 1.0 0.0 null null)
  (`/Game/UI/Menu.PrintScanInfo` (`/Game/ExtraContent/FirstPersonBP/Blueprints/FirstPersonCharacter.HUD` (`self.Player`)) CanisterTextBody CanisterTitle))

(fn `CheckHasPower`
  (returns (HasBatteryPower :type Boolean))
  (return (> (`self.Battery`) 0.0)))

(fn `DepleteBattery`
  (params (PowerUsage :type "Float (double-precision)"))
  (bind _output_get (set `self.Battery` (`KismetMathLibrary.FClamp` (- (`self.Battery`) PowerUsage))))
  (`MaterialInstanceDynamic.SetScalarParameterValue` (`self.MainCannisterMat`) "Fill" _output_get)
  (if (== _output_get 0.0)
    (`self.StopFiring`)
    (`self.KillFlashlight`)))

(fn `GetScanInfo`
  (params (ScannedActor :type "Actor Object Reference"))
  (locals (IsUnscannedPresent :type Boolean))
  (bind _returnvalue (`GameplayStatics.GetObjectClass` ScannedActor))
  (if (not (`AudioComponent.IsPlaying` (`self.Audio`)))
    (for _array_element (`self.scanInfo`)
      (bind (_actor _name _infobite _infotexttitle _infotextbody) (break `/Game/Blueprints/Tools/Struct_ScanInfo` _array_element))
      (if (== _actor _returnvalue)
        (`KismetArrayLibrary.Array_Add` (`self.Scanned`) _returnvalue)
        (bind _outactors (`GameplayStatics.GetAllActorsOfClass` _returnvalue))
        (for _array_element_2 _outactors
          (message `/Game/Blueprints/Interfaces/BPI_Scannable.ToggleScannableUI` _array_element_2 true))
        (`self.SearchForUnscannedSubjects`)
        (setmembers `/Game/Blueprints/Tools/Struct_ScanInfo` :`StructRef` _array_element :`HasBeenScanned` true)
        (`AudioComponent.SetSound` (`self.Audio`) _infobite)
        (`AudioComponent.Play` (`self.Audio`) 0.0)
        (`/Game/UI/Menu.PrintScanInfo` (`/Game/ExtraContent/FirstPersonBP/Blueprints/FirstPersonCharacter.HUD` (`self.Player`)) _infotextbody _infotexttitle)
        (`KismetSystemLibrary.PrintString` _name true true (struct :`G` 0.66 :`B` 1.0 :`A` 1.0) 10.0)))))

(fn `InitCannisters`
  (`KismetSystemLibrary.PrintString` "Initcanister")
  (for _array_element (`self.AvailableModes`)
    (`SceneComponent.SetHiddenInGame` (select `/Game/Blueprints/Tools/Enum_ToolModes` _array_element :`NewEnumerator3` (`self.ScannerCanRoot`) :`NewEnumerator0` (`self.LaserCanRoot`) :`NewEnumerator2` (`self.FlareCanRoot`) :`NewEnumerator1` (`self.GrappleCanRoot`)) false true)))

(fn `LaunchFlare`
  (bind (_returnvalue_location _returnvalue_rotation) (`KismetMathLibrary.BreakTransform` (`SceneComponent.K2_GetComponentToWorld` (`self.FireLocation`))))
  (if (`self.CanFireFlare`)
    (set `self.CanFireFlare` false)
    (`|SpawnActorFromClass` "/Game/Blueprints/Tools/BP_PlasmaFlare.BP_PlasmaFlare_C" (`KismetMathLibrary.MakeTransform` _returnvalue_location _returnvalue_rotation) "Undefined" "OverrideRootScale" null null)
    (`/Game/ExtraContent/FirstPersonBP/Blueprints/FirstPersonCharacter.FireKickback` (`self.Player`))
    (`AudioComponent.Play` (`self.Flare`) 0.0)
    (`/Game/Blueprints/BL_Senses.ActorNoise` (`GameplayStatics.GetPlayerPawn` 0) 3.0)))

(fn `LineTraceFromActorForward`
  (params (Actor :type "Actor Object Reference") (LineTraceDistance :type "Float (double-precision)") (ActorsToIgnore :type "Array of Actor Object Reference"))
  (returns (OutHit :type "HitResult Structure") (WasAHit :type Boolean))
  (bind _returnvalue (`self.K2_GetActorLocation` Actor))
  (bind (_outhit _returnvalue_2) (`KismetSystemLibrary.LineTraceSingle` _returnvalue (+ _returnvalue (* (`self.GetActorForwardVector` Actor) LineTraceDistance)) "TraceTypeQuery1" false ActorsToIgnore))
  (return _outhit _returnvalue_2))

(fn `SearchForUnscannedSubjects`
  (locals (IsUnscannedPresent :type Boolean))
  (bind _hud (`/Game/ExtraContent/FirstPersonBP/Blueprints/FirstPersonCharacter.HUD` (`self.Player`)))
  (bind _outactors (`GameplayStatics.GetAllActorsWithTag` "Scannable"))
  (for _array_element _outactors
    (if (not (`KismetArrayLibrary.Array_Contains` (`Actor.Tags` _array_element) "Scanned"))
      (set `local.IsUnscannedPresent` true)))
  (if (`KismetSystemLibrary.IsValid` _hud)
    (`/Game/UI/Menu.SetScanIndicatorVisibility` _hud (`local.IsUnscannedPresent`))))

(fn `UpdateFlashlightLighting`
  (params (NewRadius :type "Float (double-precision)") (Radius :type "Float (double-precision)"))
  (`LocalLightComponent.SetAttenuationRadius` (`self.Flashlight`) (`local.NewRadius`))
  (`LocalLightComponent.SetAttenuationRadius` (`self.Flashlight`) (`local.NewRadius`))
  (`/Game/Blueprints/LightDetection/BP_LightVolume.Set New Radius` (`self.FlashlightLightVol`) (`local.Radius`)))

(fn `UserConstructionScript`
  (`|ExecutionSequence`
    (:`then_0`
      (bind _returnvalue (`KismetMaterialLibrary.CreateDynamicMaterialInstance` "/Game/Blueprints/Tools/Mesh/M_Cannister.M_Cannister"))
      (bind _output_get (set `self.MainCannisterMat` _returnvalue))
      (`PrimitiveComponent.SetMaterial` (`self.SM_MultiTool`) 1 _output_get))
    (:`then_1`
      (bind _returnvalue_2 (`KismetMaterialLibrary.CreateDynamicMaterialInstance` "/Game/Blueprints/Tools/Mesh/M_Cannister_Simple.M_Cannister_Simple"))
      (bind _output_get_2 (set `self.LaserCanMat` _returnvalue_2))
      (`PrimitiveComponent.SetMaterial` (`self.LaserCan`) 1 _output_get_2)
      (`MaterialInstanceDynamic.SetVectorParameterValue` (`self.LaserCanMat`) "Color" (struct :`R` 1.0 :`G` 0.47932 :`A` 1.0)))
    (:`then_2`
      (bind _returnvalue_3 (`KismetMaterialLibrary.CreateDynamicMaterialInstance` "/Game/Blueprints/Tools/Mesh/M_Cannister_Simple.M_Cannister_Simple"))
      (bind _output_get_3 (set `self.FlareCanMat` _returnvalue_3))
      (`PrimitiveComponent.SetMaterial` (`self.FlareCan`) 1 _output_get_3)
      (`MaterialInstanceDynamic.SetVectorParameterValue` (`self.FlareCanMat`) "Color" (struct :`R` 1.0 :`A` 1.0)))
    (:`then_3`
      (bind _returnvalue_4 (`KismetMaterialLibrary.CreateDynamicMaterialInstance` "/Game/Blueprints/Tools/Mesh/M_Cannister_Simple.M_Cannister_Simple"))
      (bind _output_get_4 (set `self.GrappleCanMat` _returnvalue_4))
      (`PrimitiveComponent.SetMaterial` (`self.GrappleCan`) 1 _output_get_4)
      (`MaterialInstanceDynamic.SetVectorParameterValue` (`self.GrappleCanMat`) "Color" (struct :`G` 1.0 :`B` 0.984843 :`A` 1.0)))
    (:`then_4`
      (bind _returnvalue_5 (`KismetMaterialLibrary.CreateDynamicMaterialInstance` "/Game/Blueprints/Tools/Mesh/M_Cannister_Simple.M_Cannister_Simple"))
      (bind _output_get_5 (set `self.ScannerCanMat` _returnvalue_5))
      (`PrimitiveComponent.SetMaterial` (`self.ScannerCan`) 1 _output_get_5)
      (`MaterialInstanceDynamic.SetVectorParameterValue` (`self.ScannerCanMat`) "Color" (struct :`G` 1.0 :`B` 0.013883 :`A` 1.0)))))