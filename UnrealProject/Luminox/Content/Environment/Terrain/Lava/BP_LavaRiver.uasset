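; BP_LavaRiver is a terrain actor that builds a river, presumably of lava, along an editable spline.
; The construction script clears an array of components, then adds spline mesh components that follow the spline points' local positions and tangents.
; Each segment takes the Material variable, scales its width and height by RiverWidth, and casts no shadow.
; It has no runtime logic, and SectionSize is unused.
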(fn `UserConstructionScript`
  (bind _riverwidth (`self.RiverWidth`))
  (bind _spline (`self.Spline`))
  (for _array_element _
    (`ActorComponent.K2_DestroyComponent` _array_element))
  (for _index (range 1 (+ (`SplineComponent.GetNumberOfSplinePoints` (`self.Spline`)) 1))
    (bind _returnvalue (`AddComponent|NODE_AddSplineMeshComponent-0`))
    (bind (_location _tangent) (`SplineComponent.GetLocationAndTangentAtSplinePoint` _spline (+ _index -1) "Local"))
    (bind (_location_2 _tangent_2) (`SplineComponent.GetLocationAndTangentAtSplinePoint` _spline _index "Local"))
    (`SplineMeshComponent.SetStartAndEnd` _returnvalue _location _tangent _location_2 _tangent_2 true)
    (`SceneComponent.SetRelativeScale3D` _returnvalue (`KismetMathLibrary.MakeVector` 1.0 _riverwidth _riverwidth))
    (`PrimitiveComponent.SetMaterial` _returnvalue 0 (`self.Material`))
    (`PrimitiveComponent.SetCastShadow` _returnvalue false)))